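; Actor component that keeps its owning actor in the world only if a linked level is recorded in the game data's codex, apparently as completed.
; On BeginPlay it looks up LevelThatLoadsMe in the codex level and world block entries from the GameInstance, and destroys the owner if neither contains it.
; The actor is removed after load rather than spawned on demand, and stays when no level is set.
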(event EventBeginPlay
  (bind _level_that_loads_me (Variables|Default|GetLevel%20That%20Loads%20Me))
  ;[1 1 1] Spawns the Actor if the Level has been Completed - Ryan
  (Utilities|IsValid (Variables|Default|GetLevel%20That%20Loads%20Me)
    (:Is%20Valid
      (bind _savegamedata (Class|BPISaveGameInterface|GetGameData(Message) (Game|GetGameInstance)))
      (if (not (or (Utilities|Array|ContainsItem (Variables|/Game/Blueprints/Saving/BP_SaveGame.BP_SaveGame_C|GetCodexEntries%20-%20Levels _savegamedata) _level_that_loads_me) (Utilities|Array|ContainsItem (Variables|/Game/Blueprints/Saving/BP_SaveGame.BP_SaveGame_C|GetCodexEntries%20-%20WorldBlocks _savegamedata) _level_that_loads_me)))
        (Actor|DestroyActor (Components|GetOwner))))))