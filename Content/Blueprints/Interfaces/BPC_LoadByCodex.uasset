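; Actor component that keeps its owning actor in the level only if the asset set in CodexThatLoadsMe is recorded in the game data.
; On BeginPlay it casts that asset to a codex entry, challenge area or time trial and checks the matching GameInstance collections.
; It destroys the owner when the asset is missing or of another type, and does nothing when none is set.
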(event EventBeginPlay
  (bind _codex_that_loads_me (Variables|Default|GetCodex%20That%20Loads%20Me))
  ;[1 1 1] Spawns the Actor if the Level has been Completed - Ryan
  (Utilities|IsValid (Variables|Default|GetCodex%20That%20Loads%20Me)
    (:Is%20Valid
      (bind _savegamedata (Class|BPISaveGameInterface|GetGameData(Message) (Game|GetGameInstance)))
      (bind _asbp_codex_entry (Utilities|Casting|CastToBP_CodexEntry _codex_that_loads_me)
        (:then
          (if (not (Math|Boolean|ORBoolean (Utilities|Array|ContainsItem (Variables|/Game/Blueprints/Saving/BP_SaveGame.BP_SaveGame_C|GetCodexEntries%20-%20Levels _savegamedata) _asbp_codex_entry) (Utilities|Array|ContainsItem (Variables|/Game/Blueprints/Saving/BP_SaveGame.BP_SaveGame_C|GetCodexEntries%20-%20WorldBlocks _savegamedata) _asbp_codex_entry) (Utilities|Array|ContainsItem (Variables|/Game/Blueprints/Saving/BP_SaveGame.BP_SaveGame_C|GetCodexEntries%20-%20Pages _savegamedata) _asbp_codex_entry) (Utilities|Array|ContainsItem (Variables|/Game/Blueprints/Saving/BP_SaveGame.BP_SaveGame_C|GetCodexEntries%20-%20Tutorials _savegamedata) _asbp_codex_entry) (Utilities|Array|ContainsItem (Variables|/Game/Blueprints/Saving/BP_SaveGame.BP_SaveGame_C|GetCodexEntries%20-%20Cates _savegamedata) _asbp_codex_entry)))
            (Actor|DestroyActor (Components|GetOwner) :!label _label)))
        (:CastFailed
          (bind _asbp_challenge_area_asset (Utilities|Casting|CastToBP_ChallengeAreaAsset _codex_that_loads_me)
            (:then
              (if (not (Utilities|Array|ContainsItem (Variables|/Game/Blueprints/Saving/BP_SaveGame.BP_SaveGame_C|GetChallenge%20Area%20Collectibles _savegamedata) _asbp_challenge_area_asset))
                (goto _label)))
            (:CastFailed
              (bind _asbp_time_trial_asset (Utilities|Casting|CastToBP_TimeTrialAsset _codex_that_loads_me)
                (:then
                  (if (not (Utilities|Array|ContainsItem (Variables|/Game/Blueprints/Saving/BP_SaveGame.BP_SaveGame_C|GetTime%20Trial%20Collectibles _savegamedata) _asbp_time_trial_asset))
                    (goto _label)))
                (:CastFailed
                  (goto _label))))))))))