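; Level manager that resets a list of area actors whenever the player dies, via the player's death event bound on BeginPlay.
; BeginPlay records the list indices of goo plants, goo areas, time pickups and gold fly collectibles as exceptions.
; On respawn, those exceptions get their own reset function through casts, while every other valid actor receives a generic ReplaceResetMessage call.
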(event Custom|Respawned
  (for (_array_element _array_index) (Variables|Default|GetActorsToReset)
    (if (not (Utilities|Array|ContainsItem (Variables|Default|GetFuckedUpActors) _array_index))
      (Utilities|IsValid _array_element
        (:Is%20Valid
          (Class|ResetEnviro|ReplaceReset(Message) _array_element)))
      (else
        (bind _asbp_goo_plant (Utilities|Casting|CastToBP_GooPlant _array_element)
          (:then
            (Default|FuckReset _asbp_goo_plant))
          (:CastFailed
            (bind _asgoo_area (Utilities|Casting|CastToGooArea _array_element)
              (:then
                (Default|FuckReset _asgoo_area))
              (:CastFailed
                (bind _asbp_time_pick_up (Utilities|Casting|CastToBP_TimePickUp _array_element)
                  (:then
                    (Default|FuckReset _asbp_time_pick_up))
                  (:CastFailed
                    (bind _asbp_gold_fly_collectible (Utilities|Casting|CastToBP_GoldFlyCollectible _array_element))
                    (Default|FuckReset _asbp_gold_fly_collectible)))))))))))

(event EventBeginPlay
  (bind _asbp_player (Utilities|Casting|CastToBP_Player (Game|Player|GetPlayerPawn 0)))
  (EventDispatchers|BindEventtoPlayerDied _asbp_player (delegate Custom|Respawned))
  (for (_array_element _array_index) (Variables|Default|GetActorsToReset)
    (Utilities|Casting|CastToBP_GooPlant _array_element
      (:then
        _)
      (:CastFailed
        (Utilities|Casting|CastToGooArea _array_element
          (:then
            _)
          (:CastFailed
            (Utilities|Casting|CastToBP_TimePickUp _array_element
              (:then
                _)
              (:CastFailed
                (Utilities|Casting|CastToBP_GoldFlyCollectible _array_element)))))))
    (Utilities|Array|AddUnique (Variables|Default|GetFuckedUpActors) _array_index)))

(fn ConstructionScript)