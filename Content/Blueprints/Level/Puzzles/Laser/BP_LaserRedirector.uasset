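; Laser puzzle redirector that, while active, fires a beam forward and relays power to other BP_LaserInterface actors.
; Tick line-traces from the arrow, moving the cable's end and stretching the collision to the hit, with DoOnce gates limiting Activate/Deactivate calls as targets change.
; Deactivate ignores calls from the actor it is hitting.
; Interact turns it 90 degrees via timeline; a sphere overlap shows the player a widget.
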(event OnComponentBeginOverlap(Sphere)
  (params (OverlappedComponent :type Primitive%20Component%20Object%20Reference) (OtherActor :type Actor%20Object%20Reference) (OtherComp :type Primitive%20Component%20Object%20Reference) (OtherBodyIndex :type Integer) (bFromSweep :type Boolean) (SweepResult :type Hit%20Result%20Structure%20%28by%20ref%29))
  (if (== OtherActor (Game|Player|GetPlayerPawn 0))
    (Rendering|SetVisibility (Variables|Default|GetWidget) true false)))

(event OnComponentEndOverlap(Sphere)
  (params (OverlappedComponent :type Primitive%20Component%20Object%20Reference) (OtherActor :type Actor%20Object%20Reference) (OtherComp :type Primitive%20Component%20Object%20Reference) (OtherBodyIndex :type Integer))
  (if (== OtherActor (Game|Player|GetPlayerPawn 0))
    (Rendering|SetVisibility (Variables|Default|GetWidget) false true)))

(event Custom|ActivateLaser
  (Variables|Default|SetIsActive true))

(event Custom|DeactivateLaser
  (Variables|Default|SetIsActive false)
  (Transformation|SetWorldLocation (Variables|Default|GetLaserEnd) (Transformation|GetWorldLocation (Variables|Default|GetArrow)) false true))

(event EventBeginPlay
  (Class|CableComponent|SetAttachEndtoComponent (Variables|Default|GetCable) (Variables|Default|GetLaserEnd) "None")
  (Rendering|SetVisibility (Variables|Default|GetLaserCollision) false false)
  (Rendering|SetVisibility (Variables|Default|GetWidget) false false))

(event Collision|EventActorBeginOverlap
  (params (OtherActor :type Actor%20Object%20Reference)))

(event EventTick
  (params (DeltaSeconds :type Float%20%28single-precision%29))
  (bind _lasercollision (Variables|Default|GetLaserCollision))
  (bind _arrow (Variables|Default|GetArrow))
  (bind _returnvalue (Transformation|GetWorldLocation _arrow))
  (bind _relativescale3d (Variables|/Script/Engine.SceneComponent|GetRelativeScale3D _lasercollision))
  ;[1 1 1] Ew
  (if (Variables|Default|GetIsActive)
    (Utilities|FlowControl|Sequence
      (:then_0
        ;[1 1 1] If just turned active, turn on hum
        (Utilities|FlowControl|DoOnce false :!label _label
          (:Completed
            (Audio|PlaySoundatLocation "/Game/Sounds/SFX/Laser/LaserStart.LaserStart" (Transformation|GetActorLocation) "0, 0, 0" 1.0 1.0 0.0 0 0 0 0)
            (Utilities|FlowControl|Delay 2.457)
            (Audio|Components|Audio|Play (Variables|Default|GetLaserHum) 0.0))))
      (:then_1
        (Utilities|FlowControl|Sequence
          (:then_0
            (goto _label_5 Reset))
          (:then_1
            ;[1 1 1] If active in general
            ;;[1 1 1] Line trace forward
            (bind (_outhit _returnvalue_2) (Collision|LineTraceByChannel _returnvalue (+ _returnvalue (* (Math|Vector|GetForwardVector _arrow) (Variables|Default|GetLaser%20Check%20Distance))) "TraceTypeQuery1" false 0 "None"))
            ;;[1 1 1] Move Laser end to end of trace
            (Transformation|SetWorldLocation (Variables|Default|GetLaserEnd) (select _returnvalue_2 (.ImpactPoint (Collision|BreakHitResult _outhit)) (.TraceEnd (Collision|BreakHitResult _outhit))) false true)
            ;;[1 1 1] Set laser collision to point
            (Transformation|SetRelativeScale3D _lasercollision (Math|Vector|MakeVector (.x _relativescale3d) (.y _relativescale3d) (/ (Math|Vector|VectorLength (- (.TraceStart (Collision|BreakHitResult _outhit)) (select _returnvalue_2 (.ImpactPoint (Collision|BreakHitResult _outhit)) (.TraceEnd (Collision|BreakHitResult _outhit))))) 1e+02)))
            (if _returnvalue_2
              (if (Utilities|DoesObjectImplementInterface (.HitActor (Collision|BreakHitResult _outhit)) "/Game/Blueprints/Level/Puzzles/Laser/BP_LaserInterface.BP_LaserInterface_C")
                ;;[1 1 1] If hit actor is a laser, active (reciever)
                (Utilities|FlowControl|Sequence
                  (:then_0
                    (Utilities|FlowControl|DoOnce false :!label _label_2
                      (:Completed
                        (bind _output_get (Variables|Default|SetLaser%20Hit%20Actor (.HitActor (Collision|BreakHitResult _outhit))))
                        (bind _asbp_laser_interface (Utilities|Casting|CastToBP_LaserInterface _output_get))
                        (Default|Activate _asbp_laser_interface self))))
                  (:then_1
                    ;;[1 1 1] If hit actor is not laser, deactivate previous reciever
                    (if (!= (.HitActor (Collision|BreakHitResult _outhit)) (Variables|Default|GetLaser%20Hit%20Actor)) :!label _label_3
                      (Utilities|FlowControl|DoOnce false :!label _label_4
                        (:Completed
                          (bind _asbp_laser_interface_2 (Utilities|Casting|CastToBP_LaserInterface (Variables|Default|GetLaser%20Hit%20Actor)))
                          (Default|Deactivate _asbp_laser_interface_2 self)
                          (Variables|Default|SetLaser%20Hit%20Actor (.HitActor (Collision|BreakHitResult _outhit)))
                          (goto _label_2 Reset)))
                      (else
                        (goto _label_4 Reset)))))
                (else
                  (goto _label_3))))))))
    (else
      (Utilities|FlowControl|Sequence
        (:then_0
          ;;[1 1 1] If just turned off, stop noise and open gate
          (Audio|Components|Audio|Stop (Variables|Default|GetLaserHum))
          (goto _label Reset))
        (:then_1
          ;[1 1 1] Then if just turned off or just made active, disable actor it was hitting
          (Utilities|FlowControl|DoOnce false :!label _label_5
            (:Completed
              (bind _asbp_laser_interface_3 (Utilities|Casting|CastToBP_LaserInterface (Variables|Default|GetLaser%20Hit%20Actor)))
              (Default|Deactivate _asbp_laser_interface_3 self)
              (Variables|Default|SetLaser%20Hit%20Actor 0)
              (Variables|Default|SetSource 0)
              (Utilities|FlowControl|Sequence
                (:then_0
                  (goto _label_2 Reset))
                (:then_1
                  (goto _label_4 Reset))))))))))

(event EventActivate
  (params (Source :type Actor%20Object%20Reference))
  (Variables|Default|SetIsActive true)
  (Variables|Default|SetSource Source))

(event EventDeactivate
  (params (Source :type Actor%20Object%20Reference))
  (if (not (== Source (Variables|Default|GetLaser%20Hit%20Actor)))
    (Variables|Default|SetIsActive false)
    (Variables|Default|SetSource 0)
    (Transformation|SetWorldLocation (Variables|Default|GetLaserEnd) (Transformation|GetWorldLocation (Variables|Default|GetArrow)) false true)))

(event EventRotate
  (if (Variables|Default|GetRotationFinished)
    (Audio|PlaySoundatLocation "/Game/Sounds/SFX/Laser/Redirector/RedirectorTurn.RedirectorTurn" (Transformation|GetActorLocation) "0, 0, 0" 1.0 0.5 0.5 0 0 0 0)
    (Variables|Default|SetInitialRotation (Transformation|GetActorRotation))
    (bind _newtrack_0 (Timeline|Timeline PlayFromStart)
      (:Update
        (Variables|Default|SetRotationFinished false)
        (Transformation|SetActorRotation (Math|Rotator|MakeRotator (.roll (Variables|Default|GetInitialRotation)) (.pitch (Variables|Default|GetInitialRotation)) (+ (* _newtrack_0 9e+01) (.yaw (Variables|Default|GetInitialRotation))))))
      (:Finished
        (Variables|Default|SetInitialRotation (Transformation|GetActorRotation))
        (Variables|Default|SetRotationFinished true)))))

(event EventFlipVisible
  (Utilities|FlowControl|FlipFlop
    (:A
      (Rendering|SetVisibility (Variables|Default|GetLaserCollision) true false))
    (:B
      (Rendering|SetVisibility (Variables|Default|GetLaserCollision) false false))))

(fn ConstructionScript)

(fn Interact
  (CallFunction|Rotate)
  (return false))

(fn Ping
  (return (Variables|Default|GetIsActive) false))