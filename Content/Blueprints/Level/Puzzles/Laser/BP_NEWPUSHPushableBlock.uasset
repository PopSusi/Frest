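; Pushable laser puzzle block that emits a beam and moves through a series of Sequences when pushed by the player.
; Tick traces from the Arrow to place the cable's end, scale the laser collision, and message BP_LaserInterface actors on hit changes.
; Player overlap starts a shake timeline and tolerance-check timer, then plays the next sequence, but WithinTolerance always returns false, so pushes never proceed.
; Reset restores the starting transform and sequence index.
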(event OnComponentBeginOverlap(Box)
  (params (OverlappedComponent :type Primitive%20Component%20Object%20Reference) (OtherActor :type Actor%20Object%20Reference) (OtherComp :type Primitive%20Component%20Object%20Reference) (OtherBodyIndex :type Integer) (bFromSweep :type Boolean) (SweepResult :type Hit%20Result%20Structure%20%28by%20ref%29))
  (bind _returnvalue (Game|Player|GetPlayerPawn 0))
  (if (== OtherActor _returnvalue)
    (Utilities|IsValid (Variables|Default|GetAs%20BP%20Player)
      (:Is%20Valid
        _)
      (:Is%20Not%20Valid
        (bind _asbp_player (Utilities|Casting|CastToBP_Player _returnvalue))
        (bind _output_get (Variables|Default|SetAs%20BP%20Player _asbp_player))))
    (bind _within_tolerance (CallFunction|WithinTolerance))
    (if _within_tolerance
      (bind _returnvalue_2 (Utilities|Time|SetTimerbyEvent (delegate Custom|Check) 0.1 true))
      (Variables|Default|SetCheckLoop _returnvalue_2)
      (Utilities|FlowControl|Sequence
        (:then_0
          (Utilities|FlowControl|Gate true) ; enters at Open
        )
        (:then_1
          (bind _shaky (Timeline|Timeline_0 PlayFromStart)
            (:Update
              (Transformation|SetRelativeLocation (Variables|Default|GetStaticMesh) (Math|Vector|MakeVector _shaky _shaky _shaky) false false))
            (:Finished
              (bind _within_tolerance_2 (CallFunction|WithinTolerance))
              (if (and (!= (Utilities|Array|Length (Variables|Default|GetSequences)) (Variables|Default|GetSequenceIndex)) _within_tolerance_2)
                (Sequencer|Player|Play (Variables|/Script/LevelSequence.LevelSequenceActor|GetSequencePlayer (Utilities|Array|Get(acopy) (Variables|Default|GetSequences) (Variables|Default|GetSequenceIndex))) :!class /Script/MovieScene.MovieSceneSequencePlayer)
                (Variables|Default|SetControlNegativeRotation (Math|Conversions|RotationFromXVector (Math|Vector|RotateVector (Math|Vector|MakeVector -1.8e+02 0.0 0.0) (Variables|Default|GetControlRotation))))
                (Variables|Default|SetControlRotation (Math|Conversions|RotationFromXVector (Math|Vector|RotateVector (Math|Vector|MakeVector 0.0 (Utilities|Array|Get(acopy) (Variables|Default|GetRotateSet) (Variables|Default|GetSequenceIndex)) 0.0) (Variables|Default|GetControlRotation))))
                (Math|Integer|IncrementInt (Variables|Default|GetSequenceIndex)
                  (:%20%20
                    (Default|ExitState (Variables|Default|GetAs%20BP%20Player) "NewEnumerator0" "NewEnumerator13"))))))))
      (else
        (Default|ExitState _output_get "NewEnumerator0" "NewEnumerator13")))))

(event OnComponentBeginOverlap(LazerEnd)
  (params (OverlappedComponent :type Primitive%20Component%20Object%20Reference) (OtherActor :type Actor%20Object%20Reference) (OtherComp :type Primitive%20Component%20Object%20Reference) (OtherBodyIndex :type Integer) (bFromSweep :type Boolean) (SweepResult :type Hit%20Result%20Structure%20%28by%20ref%29)))

(event OnComponentEndOverlap(LazerEnd)
  (params (OverlappedComponent :type Primitive%20Component%20Object%20Reference) (OtherActor :type Actor%20Object%20Reference) (OtherComp :type Primitive%20Component%20Object%20Reference) (OtherBodyIndex :type Integer)))

(event OnComponentEndOverlap(Box)
  (params (OverlappedComponent :type Primitive%20Component%20Object%20Reference) (OtherActor :type Actor%20Object%20Reference) (OtherComp :type Primitive%20Component%20Object%20Reference) (OtherBodyIndex :type Integer))
  (if (== OtherActor (Game|Player|GetPlayerPawn 0))
    (CallFunction|Cancel)))

(event Custom|Cancel
  (Utilities|Time|ClearandInvalidateTimerbyHandle (Variables|Default|GetCheckLoop))
  (Utilities|FlowControl|Sequence
    (:then_0
      (bind _shaky (Timeline|Timeline_0 Stop)
        (:Update
          (Transformation|SetRelativeLocation (Variables|Default|GetStaticMesh) (Math|Vector|MakeVector _shaky _shaky _shaky) false false))
        (:Finished
          (bind _within_tolerance (CallFunction|WithinTolerance))
          (if (and (!= (Utilities|Array|Length (Variables|Default|GetSequences)) (Variables|Default|GetSequenceIndex)) _within_tolerance)
            (Sequencer|Player|Play (Variables|/Script/LevelSequence.LevelSequenceActor|GetSequencePlayer (Utilities|Array|Get(acopy) (Variables|Default|GetSequences) (Variables|Default|GetSequenceIndex))) :!class /Script/MovieScene.MovieSceneSequencePlayer)
            (Variables|Default|SetControlNegativeRotation (Math|Conversions|RotationFromXVector (Math|Vector|RotateVector (Math|Vector|MakeVector -1.8e+02 0.0 0.0) (Variables|Default|GetControlRotation))))
            (Variables|Default|SetControlRotation (Math|Conversions|RotationFromXVector (Math|Vector|RotateVector (Math|Vector|MakeVector 0.0 (Utilities|Array|Get(acopy) (Variables|Default|GetRotateSet) (Variables|Default|GetSequenceIndex)) 0.0) (Variables|Default|GetControlRotation))))
            (Math|Integer|IncrementInt (Variables|Default|GetSequenceIndex)
              (:%20%20
                (Default|ExitState (Variables|Default|GetAs%20BP%20Player) "NewEnumerator0" "NewEnumerator13")))))))
    (:then_1
      (Utilities|FlowControl|Gate true) ; enters at Close
    )))

(event Custom|Check
  (bind _within_tolerance (CallFunction|WithinTolerance))
  (if (not _within_tolerance)
    (CallFunction|Cancel)))

(event EventBeginPlay
  (Class|CableComponent|SetAttachEndtoComponent (Variables|Default|GetCable) (Variables|Default|GetLazerEnd) "None")
  (Rendering|SetVisibility (Variables|Default|GetLaserCollision) false false)
  (CallFunction|SetDefaults))

(event EventReset
  (Transformation|SetActorTransform (Variables|Default|GetDefaultPosition))
  (Variables|Default|SetSequenceIndex 0))

(event EventSetDefaults
  (Variables|Default|SetDefaultPosition (Transformation|GetActorTransform)))

(event EventTick
  (params (DeltaSeconds :type Float%20%28single-precision%29))
  (bind _arrow (Variables|Default|GetArrow))
  (bind _lasercollision (Variables|Default|GetLaserCollision))
  (bind _returnvalue (Transformation|GetWorldLocation _arrow))
  (bind _returnvalue_2 (Transformation|GetWorldScale _lasercollision))
  (bind _returnvalue_3 (Math|Vector|GetForwardVector _arrow))
  (bind (_outhit _returnvalue_4) (Collision|LineTraceByChannel _returnvalue (+ _returnvalue (* _returnvalue_3 1e+04)) "TraceTypeQuery1" false 0 "None"))
  (Transformation|SetWorldLocation (Variables|Default|GetLazerEnd) (+ (select _returnvalue_4 (.ImpactPoint (Collision|BreakHitResult _outhit)) (.TraceEnd (Collision|BreakHitResult _outhit))) (* _returnvalue_3 2.0)) false false)
  (Transformation|SetWorldScale3D _lasercollision (Math|Vector|MakeVector (.x _returnvalue_2) (.y _returnvalue_2) (/ (Math|Vector|VectorLength (- (.ImpactPoint (Collision|BreakHitResult _outhit)) _returnvalue)) 1e+02)))
  (if (.bBlockingHit (Collision|BreakHitResult _outhit))
    (if (Utilities|DoesObjectImplementInterface (.HitActor (Collision|BreakHitResult _outhit)) "/Game/Blueprints/Level/Puzzles/Laser/BP_LaserInterface.BP_LaserInterface_C")
      (Utilities|FlowControl|Sequence
        (:then_0
          (Utilities|FlowControl|DoOnce false :!label _label
            (:Completed
              (bind _output_get (Variables|Default|SetLaserHitActor (.HitActor (Collision|BreakHitResult _outhit))))
              (Class|BPLaserInterface|Activate(Message) _output_get self))))
        (:then_1
          (if (!= (.HitActor (Collision|BreakHitResult _outhit)) (Variables|Default|GetLaserHitActor)) :!label _label_2
            (Utilities|FlowControl|DoOnce false :!label _label_3
              (:Completed
                (Class|BPLaserInterface|Deactivate(Message) (Variables|Default|GetLaserHitActor) self)
                (Variables|Default|SetLaserHitActor 0)
                (goto _label Reset)))
            (else
              (goto _label_3 Reset)))))
      (else
        (goto _label_2)))))

(event EventFlipVisible
  (Utilities|FlowControl|FlipFlop
    (:A
      (Rendering|SetVisibility (Variables|Default|GetLaserCollision) true false))
    (:B
      (Rendering|SetVisibility (Variables|Default|GetLaserCollision) false false))))

(fn ConstructionScript)

(fn WithinTolerance
  (return false))

(fn Ping
  (return true false))