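; Laser receiver puzzle actor that completes its puzzle when the laser source activating it overlaps it.
; Activate stores the source, waits briefly, then on finding it among overlapping actors calls PuzzleComplete, plays a sound and starts a looping QueryLaser timer.
; QueryLaser tests only the first overlapping actor, cancelling on mismatch or no overlap, but clears the timer only on mismatch.
; Deactivate calls PuzzleDeactivate directly.
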(event Custom|QueryLaser
  (bind _overlappingactors (Collision|GetOverlappingActors 0 :!class /Script/Engine.Actor))
  (if (Utilities|Array|IsNotEmpty _overlappingactors)
    (bind _array_element (Utilities|Array|ForEachLoopwithBreak _overlappingactors :!label _label)
      (:LoopBody
        (if (== _array_element (Variables|Default|GetActivator))
          (goto _label Break)
          (else
            (Utilities|Time|ClearandInvalidateTimerbyHandle (Variables|Default|GetLoopCheck)))))))
  (CallFunction|PuzzleCancelled)
  (goto _label Break))

(event EventBeginPlay)

(event Collision|EventActorBeginOverlap
  (params (OtherActor :type Actor%20Object%20Reference)))

(event EventTick
  (params (DeltaSeconds :type Float%20%28single-precision%29)))

(event EventActivate
  (params (Source :type Actor%20Object%20Reference))
  (Variables|Default|SetActivator Source)
  (Utilities|FlowControl|Delay 0.2)
  (bind _array_element (Utilities|Array|ForEachLoopwithBreak (Collision|GetOverlappingActors 0 :!class /Script/Engine.Actor) :!label _label)
    (:LoopBody
      (if (== _array_element (Variables|Default|GetActivator))
        (CallFunction|PuzzleComplete)
        (Audio|PlaySoundatLocation "/Game/Sounds/SFX/Gameplay/GoodJob.GoodJob" (Transformation|GetActorLocation) "0, 0, 0" 1.0 1.0 0.0 0 0 0 0)
        (bind _returnvalue (Utilities|Time|SetTimerbyEvent (delegate Custom|QueryLaser) 3.0 true))
        (Variables|Default|SetLoopCheck _returnvalue)
        (goto _label Break)))))

(event EventDeactivate
  (params (Source :type Actor%20Object%20Reference))
  (CallFunction|PuzzleDeactivate))

(fn ConstructionScript)