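; Puzzle block that casts a laser from its Arrow and switches hit actors implementing BP_LaserInterface on and off.
; Each Tick a line trace positions LazerEnd, which anchors the Cable beam, and sets LaserCollision's Z scale to the beam length.
; DoOnce gates limit Activate and Deactivate calls, with deactivation checked only when the trace hits something.
; The older overlap-based BP_LaserRedirector logic is disconnected, and no pushing logic appears here.
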(event OnComponentBeginOverlap(LazerEnd)
  (params (OverlappedComponent :type Primitive%20Component%20Object%20Reference) (OtherActor :type Actor%20Object%20Reference) (OtherComp :type Primitive%20Component%20Object%20Reference) (OtherBodyIndex :type Integer) (bFromSweep :type Boolean) (SweepResult :type Hit%20Result%20Structure%20%28by%20ref%29)))

(event OnComponentEndOverlap(LazerEnd)
  (params (OverlappedComponent :type Primitive%20Component%20Object%20Reference) (OtherActor :type Actor%20Object%20Reference) (OtherComp :type Primitive%20Component%20Object%20Reference) (OtherBodyIndex :type Integer)))

(event EventBeginPlay
  (Class|CableComponent|SetAttachEndtoComponent (Variables|Default|GetCable) (Variables|Default|GetLazerEnd) "None"))

(event Collision|EventActorBeginOverlap
  (params (OtherActor :type Actor%20Object%20Reference)))

(event EventTick
  (params (DeltaSeconds :type Float%20%28single-precision%29))
  (bind _arrow (Variables|Default|GetArrow))
  (bind _returnvalue (Transformation|GetWorldLocation _arrow))
  (bind (_outhit _returnvalue_2) (Collision|LineTraceByChannel _returnvalue (+ _returnvalue (* (Math|Vector|GetForwardVector _arrow) (Variables|Default|GetLaserCheckDistance))) "TraceTypeQuery1" false 0 "ForOneFrame"))
  (Transformation|SetWorldLocation (Variables|Default|GetLazerEnd) (select _returnvalue_2 (.ImpactPoint (Collision|BreakHitResult _outhit)) (.TraceEnd (Collision|BreakHitResult _outhit))) false false)
  (Transformation|SetRelativeScale3D (Variables|Default|GetLaserCollision) (Math|Vector|MakeVector 0.0 0.0 (Math|Vector|VectorLength (- _returnvalue (select _returnvalue_2 (.ImpactPoint (Collision|BreakHitResult _outhit)) (.TraceEnd (Collision|BreakHitResult _outhit)))))))
  (if _returnvalue_2
    (if (Utilities|DoesObjectImplementInterface (.HitActor (Collision|BreakHitResult _outhit)) "/Game/Blueprints/Level/Puzzles/BP_LaserInterface.BP_LaserInterface_C")
      (Utilities|FlowControl|Sequence
        (:then_0
          (Utilities|FlowControl|DoOnce false :!label _label
            (:Completed
              (Development|PrintString "act")
              (bind _output_get (Variables|Default|SetLaserHitActor (.HitActor (Collision|BreakHitResult _outhit))))
              (bind _asbp_laser_interface (Utilities|Casting|CastToBP_LaserInterface _output_get))
              (Default|Activate _asbp_laser_interface))))
        (:then_1
          (if (!= (.HitActor (Collision|BreakHitResult _outhit)) (Variables|Default|GetLaserHitActor)) :!label _label_2
            (Utilities|FlowControl|DoOnce false :!label _label_3
              (:Completed
                (bind _asbp_laser_interface_2 (Utilities|Casting|CastToBP_LaserInterface (Variables|Default|GetLaserHitActor)))
                (Default|Deactivate _asbp_laser_interface_2)
                (Variables|Default|SetLaserHitActor 0)
                (Development|PrintString "Deac")
                (goto _label Reset)))
            (else
              (goto _label_3 Reset)))))
      (else
        (goto _label_2)))))

(fn ConstructionScript)

(fn Ping
  (return true))