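; Checkpoint actor for a platforming game that saves the player's respawn point when touched.
; When BP_Player overlaps its Box, it writes the Capsule's world location and rotation, with unit scale, into the Checkpoints field of PlatformingGameMode's save object.
; It then saves that object to the game mode's SaveOne slot, printing debug messages for touch, success or a missing save.
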(event OnComponentBeginOverlap(Box)
  (params (OverlappedComponent :type Primitive%20Component%20Object%20Reference) (OtherActor :type Actor%20Object%20Reference) (OtherComp :type Primitive%20Component%20Object%20Reference) (OtherBodyIndex :type Integer) (bFromSweep :type Boolean) (SweepResult :type Hit%20Result%20Structure%20%28by%20ref%29))
  (bind _capsule (Variables|Default|GetCapsule))
  (bind _returnvalue (Transformation|GetWorldTransform _capsule))
  (Utilities|Casting|CastToBP_Player OtherActor)
  (Development|PrintText "Touched")
  (bind _asplatforming_game_mode (Utilities|Casting|CastToPlatformingGameMode (Game|GetGameMode)))
  (Utilities|IsValid (Variables|/Game/GameModes/PlatformingGameMode.PlatformingGameMode_C|GetSaveGameObject _asplatforming_game_mode)
    (:Is%20Valid
      (Variables|/Game/Blueprints/Player/Save.Save_C|SetCheckpoints (Variables|/Game/GameModes/PlatformingGameMode.PlatformingGameMode_C|GetSaveGameObject _asplatforming_game_mode) (Math|Transform|MakeTransform (.location _returnvalue) (.rotation _returnvalue) "1.000000,1.000000,1.000000"))
      (SaveGame|SaveGametoSlot (Variables|/Game/GameModes/PlatformingGameMode.PlatformingGameMode_C|GetSaveGameObject _asplatforming_game_mode) (Variables|/Game/GameModes/PlatformingGameMode.PlatformingGameMode_C|GetSaveOne _asplatforming_game_mode))
      (Development|PrintString "Saved"))
    (:Is%20Not%20Valid
      (Development|PrintString "Save is not there"))))

(fn ConstructionScript)