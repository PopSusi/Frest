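; Death trigger volume that sends a player who falls off the map back to the last checkpoint.
; On box overlap it fades the camera, waits briefly, then passes the Game Instance's saved data to the player's UpdatePlayerData.
; It then refreshes the HUD's Gold Fly count and re-enables collision and visibility on every Gold Fly collectible in the level.
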(event OnComponentBeginOverlap(Box)
  (params (OverlappedComponent :type Primitive%20Component%20Object%20Reference) (OtherActor :type Actor%20Object%20Reference) (OtherComp :type Primitive%20Component%20Object%20Reference) (OtherBodyIndex :type Integer) (bFromSweep :type Boolean) (SweepResult :type Hit%20Result%20Structure%20%28by%20ref%29))
  ;[1 1 1] If the player falls off of the map, they will respawn at the last checkpoint with the values they had at the time of entering the checkpoint. Also, any Gold Flies that were picked up will respawn - Ryan
  (bind _asbp_player (Utilities|Casting|CastToBP_Player OtherActor))
  (CameraFades|StartCameraFade :self (Game|GetPlayerCameraManager 0) :ToAlpha 2.0 :Duration 0.5)
  (Utilities|FlowControl|Delay 0.5)
  (bind _savegamedata (Class|BPISaveGameInterface|GetGameData(Message) (Game|GetGameInstance)))
  (Utilities|IsValid _savegamedata
    (:Is%20Valid
      (Default|UpdatePlayerData _asbp_player (Variables|/Game/Blueprints/Saving/BP_SaveGame.BP_SaveGame_C|GetPlayerData _savegamedata))
      (Variables|/Script/UMG.TextBlock|SetText (Variables|/Game/UI/Widgets/HUD/WB_HUD.WB_HUD_C|GetGoldFlyCount (Variables|/Game/Blueprints/Player/BP_Player.BP_Player_C|GetHUD _asbp_player)) (Utilities|Text|ToText(Integer) (Variables|/Game/Blueprints/Player/BP_Player.BP_Player_C|GetGoldFlies _asbp_player)))
      (bind _outactors (Actor|GetAllActorsOfClass "/Game/Blueprints/Collectibles/BP_GoldFlyCollectible.BP_GoldFlyCollectible_C"))
      (for _array_element _outactors
        (Collision|SetCollisionEnabled (Variables|/Game/Blueprints/Collectibles/BP_BaseCollectible.BP_BaseCollectible_C|GetSphere _array_element) "QueryAndPhysics")
        (Components|Activation|SetActive (Variables|/Game/Blueprints/Collectibles/BP_BaseCollectible.BP_BaseCollectible_C|GetMesh _array_element) true false)
        (Development|SetHiddeninGame (Variables|/Game/Blueprints/Collectibles/BP_BaseCollectible.BP_BaseCollectible_C|GetMesh _array_element) false false)))))

(event EventBeginPlay)

(event Collision|EventActorBeginOverlap
  (params (OtherActor :type Actor%20Object%20Reference)))

(event EventTick
  (params (DeltaSeconds :type Float%20%28single-precision%29)))

(fn ConstructionScript)