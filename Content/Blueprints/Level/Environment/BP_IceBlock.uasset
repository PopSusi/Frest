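; Ice block environment actor that steps along a chain of level sequences when the player holds against it.
; HoldCheck overlap starts a shake; on finish, dot products of player facing against two tracked directions choose playing the next sequence or reversing the previous.
; RotateSet turns those directions each step, with debug traces drawn on Tick.
; Overlap end or a looping timer check cancels the shake; separate events handle shrinking and temporary time-dilation slow.
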(event OnComponentBeginOverlap(HoldCheck)
  (params (OverlappedComponent :type Primitive%20Component%20Object%20Reference) (OtherActor :type Actor%20Object%20Reference) (OtherComp :type Primitive%20Component%20Object%20Reference) (OtherBodyIndex :type Integer) (bFromSweep :type Boolean) (SweepResult :type Hit%20Result%20Structure%20%28by%20ref%29))
  (bind _returnvalue (Game|Player|GetPlayerPawn 0))
  (if (== OtherActor _returnvalue)
    (Utilities|IsValid (Variables|Default|GetAs%20BP%20Player)
      (:Is%20Valid
        _)
      (:Is%20Not%20Valid
        (bind _asbp_player (Utilities|Casting|CastToBP_Player _returnvalue))
        (Variables|Default|SetAs%20BP%20Player _asbp_player)))
    (bind _returnvalue_2 (Utilities|Time|SetTimerbyEvent (delegate Custom|Check%20Loop) 1.1 true))
    (Variables|Default|SetCheckLoop _returnvalue_2)
    (bind _shaky (Timeline|Shaking PlayFromStart)
      (:Update
        (Transformation|SetRelativeLocation (Variables|Default|GetStaticMesh1) (Math|Vector|MakeVector _shaky _shaky _shaky) false false))
      (:Finished
        (if (and (!= (Utilities|Array|Length (Variables|Default|GetSequences)) (Variables|Default|GetSequenceIndex)) (>= (Math|Vector|DotProduct (Math|Vector|GetForwardVector (Variables|Default|GetControlRotation)) (Transformation|GetActorForwardVector (Variables|Default|GetAs%20BP%20Player))) 0.7))
          (Sequencer|Player|Play (Variables|/Script/LevelSequence.LevelSequenceActor|GetSequencePlayer (Utilities|Array|Get(acopy) (Variables|Default|GetSequences) (Variables|Default|GetSequenceIndex))) :!class /Script/MovieScene.MovieSceneSequencePlayer)
          (Variables|Default|SetControlNegativeRotation (Math|Conversions|RotationFromXVector (Math|Vector|RotateVector (Math|Vector|MakeVector -1.8e+02 0.0 0.0) (Variables|Default|GetControlRotation))))
          (Variables|Default|SetControlRotation (Math|Conversions|RotationFromXVector (Math|Vector|RotateVector (Math|Vector|MakeVector 0.0 (Utilities|Array|Get(acopy) (Variables|Default|GetRotateSet) (Variables|Default|GetSequenceIndex)) 0.0) (Variables|Default|GetControlRotation))))
          (Math|Integer|IncrementInt (Variables|Default|GetSequenceIndex)
            (:%20%20
              _))
          (elif (>= (Math|Vector|DotProduct (Math|Vector|GetForwardVector (Variables|Default|GetControlNegativeRotation)) (Transformation|GetActorForwardVector (Variables|Default|GetAs%20BP%20Player))) 0.7)
            (if (< (- (Variables|Default|GetSequenceIndex) 1) 0)
              _
              (else
                (Variables|Default|SetSequenceIndex (- (Variables|Default|GetSequenceIndex) 1))
                (Class|MovieSceneSequencePlayer|PlayReverse (Variables|/Script/LevelSequence.LevelSequenceActor|GetSequencePlayer (Utilities|Array|Get(acopy) (Variables|Default|GetSequences) (Variables|Default|GetSequenceIndex))))
                (bind _output_get (Variables|Default|SetControlRotation (Math|Conversions|RotationFromXVector (Math|Vector|RotateVector (Math|Vector|MakeVector 0.0 (* (Utilities|Array|Get(acopy) (Variables|Default|GetRotateSet) (Variables|Default|GetSequenceIndex)) -1.0) 0.0) (Variables|Default|GetControlRotation)))))
                (Variables|Default|SetControlNegativeRotation (Math|Conversions|RotationFromXVector (Math|Vector|RotateVector (Math|Vector|MakeVector -1.8e+02 0.0 0.0) _output_get)))))))
        (Development|PrintString "Hello")
        (Default|ExitState (Variables|Default|GetAs%20BP%20Player) "NewEnumerator0" "NewEnumerator13")))))

(event OnComponentEndOverlap(HoldCheck)
  (params (OverlappedComponent :type Primitive%20Component%20Object%20Reference) (OtherActor :type Actor%20Object%20Reference) (OtherComp :type Primitive%20Component%20Object%20Reference) (OtherBodyIndex :type Integer))
  (if (== OtherActor (Game|Player|GetPlayerPawn 0))
    (CallFunction|Cancel)))

(event Custom|Shrink
  (bind _shrinktimeline (Timeline|ShrinkCube PlayFromStart)
    (:Update
      (Transformation|SetRelativeScale3D (Variables|Default|GetStaticMesh) (Math|Conversions|ToVector(Float) _shrinktimeline))
      (Transformation|SetRelativeScale3D (Variables|Default|GetStaticMesh1) (Math|Conversions|ToVector(Float) _shrinktimeline)))))

(event Custom|Check%20Loop
  (if (Utilities|Array|IsNotEmpty (Collision|GetOverlappingActors (Variables|Default|GetHoldCheck) "/Game/Blueprints/Player/BP_Player.BP_Player_C" :!class /Script/Engine.PrimitiveComponent))
    (CallFunction|Cancel)))

(event Custom|Cancel
  (Utilities|Time|ClearandInvalidateTimerbyHandle (Variables|Default|GetCheckLoop))
  (bind _shaky (Timeline|Shaking Stop)
    (:Update
      (Transformation|SetRelativeLocation (Variables|Default|GetStaticMesh1) (Math|Vector|MakeVector _shaky _shaky _shaky) false false))
    (:Finished
      (if (and (!= (Utilities|Array|Length (Variables|Default|GetSequences)) (Variables|Default|GetSequenceIndex)) (>= (Math|Vector|DotProduct (Math|Vector|GetForwardVector (Variables|Default|GetControlRotation)) (Transformation|GetActorForwardVector (Variables|Default|GetAs%20BP%20Player))) 0.7))
        (Sequencer|Player|Play (Variables|/Script/LevelSequence.LevelSequenceActor|GetSequencePlayer (Utilities|Array|Get(acopy) (Variables|Default|GetSequences) (Variables|Default|GetSequenceIndex))) :!class /Script/MovieScene.MovieSceneSequencePlayer)
        (Variables|Default|SetControlNegativeRotation (Math|Conversions|RotationFromXVector (Math|Vector|RotateVector (Math|Vector|MakeVector -1.8e+02 0.0 0.0) (Variables|Default|GetControlRotation))))
        (Variables|Default|SetControlRotation (Math|Conversions|RotationFromXVector (Math|Vector|RotateVector (Math|Vector|MakeVector 0.0 (Utilities|Array|Get(acopy) (Variables|Default|GetRotateSet) (Variables|Default|GetSequenceIndex)) 0.0) (Variables|Default|GetControlRotation))))
        (Math|Integer|IncrementInt (Variables|Default|GetSequenceIndex)
          (:%20%20
            _))
        (elif (>= (Math|Vector|DotProduct (Math|Vector|GetForwardVector (Variables|Default|GetControlNegativeRotation)) (Transformation|GetActorForwardVector (Variables|Default|GetAs%20BP%20Player))) 0.7)
          (if (< (- (Variables|Default|GetSequenceIndex) 1) 0)
            _
            (else
              (Variables|Default|SetSequenceIndex (- (Variables|Default|GetSequenceIndex) 1))
              (Class|MovieSceneSequencePlayer|PlayReverse (Variables|/Script/LevelSequence.LevelSequenceActor|GetSequencePlayer (Utilities|Array|Get(acopy) (Variables|Default|GetSequences) (Variables|Default|GetSequenceIndex))))
              (bind _output_get (Variables|Default|SetControlRotation (Math|Conversions|RotationFromXVector (Math|Vector|RotateVector (Math|Vector|MakeVector 0.0 (* (Utilities|Array|Get(acopy) (Variables|Default|GetRotateSet) (Variables|Default|GetSequenceIndex)) -1.0) 0.0) (Variables|Default|GetControlRotation)))))
              (Variables|Default|SetControlNegativeRotation (Math|Conversions|RotationFromXVector (Math|Vector|RotateVector (Math|Vector|MakeVector -1.8e+02 0.0 0.0) _output_get)))))))
      (Development|PrintString "Hello")
      (Default|ExitState (Variables|Default|GetAs%20BP%20Player) "NewEnumerator0" "NewEnumerator13"))))

(event EventBeginPlay
  (Variables|Default|SetControlRotation (Transformation|GetActorRotation))
  (if (!= (- (Utilities|Array|Length (Variables|Default|GetSequences)) 1) (Utilities|Array|Length (Variables|Default|GetRotateSet)))
    (Class|AutomationBlueprintFunctionLibrary|AddExpectedLogError "ROTATOR SET NEEDS TO BE LENGTH OF SEQUENCER"))
  (Variables|Default|SetControlNegativeRotation (Math|Conversions|RotationFromXVector (Math|Vector|RotateVector (Math|Vector|MakeVector 1.8e+02 0.0 0.0) (Variables|Default|GetControlRotation)))))

(event Collision|EventActorBeginOverlap
  (params (OtherActor :type Actor%20Object%20Reference)))

(event EventTick
  (params (DeltaSeconds :type Float%20%28single-precision%29))
  (bind _returnvalue (Transformation|GetActorLocation))
  ;[1 1 1] Debug
  (Collision|LineTraceByChannel _returnvalue (+ _returnvalue (* (Math|Vector|GetForwardVector (Variables|Default|GetControlRotation)) 1e+03)) "TraceTypeQuery1" false 0 "ForOneFrame")
  (Collision|LineTraceByChannel _returnvalue (+ _returnvalue (* (Math|Vector|GetForwardVector (Variables|Default|GetControlNegativeRotation)) 1e+03)) "TraceTypeQuery1" false 0 "ForOneFrame" true "(R=0.000000,G=0.215603,B=1.000000,A=1.000000)")
  (Collision|LineTraceByChannel "0, 0, 0" "0, 0, 0" "TraceTypeQuery1" false 0 "ForOneFrame"))

(event EventStartSlow
  (Variables|Default|SetCustomTimeDilation 0.25)
  (Utilities|Time|SetTimerbyEvent (delegate EventBreakSlow) 3.0))

(event EventBreakSlow
  (Variables|Default|SetCustomTimeDilation 1.0))

(fn ConstructionScript)

(fn SlowStats
  (return 1e+03 3.0))