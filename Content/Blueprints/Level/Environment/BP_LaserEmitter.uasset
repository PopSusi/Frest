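; Laser emitter that activates actors its beam hits and reports whether the beam overlaps the player for damage.
; Each tick a forward line trace positions LazerEnd, which anchors the Cable, and stretches LaserCollision to the impact distance.
; DoOnce gates send activate and deactivate messages to BP_LaserInterface actors as the hit target changes.
; Ping returns the player overlap as DamagePing, and FlipVisible toggles visibility of the normally hidden collision mesh.
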(event EventTick
  (params (DeltaSeconds :type Float%20%28single-precision%29))
  (bind _arrow (Variables|Default|GetArrow))
  (bind _lasercollision (Variables|Default|GetLaserCollision))
  (bind _returnvalue (Transformation|GetWorldScale _lasercollision))
  (bind _returnvalue_2 (Math|Vector|GetForwardVector _arrow))
  (bind _returnvalue_3 (Transformation|GetWorldLocation _arrow))
  (|CallParentFunction DeltaSeconds)
  (bind (_outhit _returnvalue_4) (Collision|LineTraceByChannel _returnvalue_3 (+ _returnvalue_3 (* _returnvalue_2 1e+04)) "TraceTypeQuery1" false 0 "None"))
  (Transformation|SetWorldLocation (Variables|Default|GetLazerEnd) (+ (select _returnvalue_4 (.ImpactPoint (Collision|BreakHitResult _outhit)) (.TraceEnd (Collision|BreakHitResult _outhit))) (* _returnvalue_2 2.0)) false false)
  (Transformation|SetWorldScale3D _lasercollision (Math|Vector|MakeVector (.x _returnvalue) (.y _returnvalue) (/ (Math|Vector|VectorLength (- (.ImpactPoint (Collision|BreakHitResult _outhit)) _returnvalue_3)) 1e+02)))
  (if (.bBlockingHit (Collision|BreakHitResult _outhit))
    (if (Utilities|DoesObjectImplementInterface (.HitActor (Collision|BreakHitResult _outhit)) "/Game/Blueprints/Level/Puzzles/Laser/BP_LaserInterface.BP_LaserInterface_C")
      (Utilities|FlowControl|Sequence
        (:then_0
          (Utilities|FlowControl|DoOnce false :!label _label
            (:Completed
              (bind _output_get (Variables|Default|SetLaserHitActor (.HitActor (Collision|BreakHitResult _outhit))))
              (Class|BPLaserInterface|Activate(Message) _output_get self))))
        (:then_1
          (Utilities|IsValid (Variables|Default|GetLaserHitActor) :!label _label_2
            (:Is%20Valid
              (if (!= (.HitActor (Collision|BreakHitResult _outhit)) (Variables|Default|GetLaserHitActor))
                (Utilities|FlowControl|DoOnce false :!label _label_3
                  (:Completed
                    (Class|BPLaserInterface|Deactivate(Message) (Variables|Default|GetLaserHitActor) self)
                    (goto _label Reset)))
                (else
                  (goto _label_3 Reset)))))))
      (else
        (goto _label_2)))
    (else
      (goto _label_2))))

(event EventBeginPlay
  (|CallParentFunction)
  (Class|CableComponent|SetAttachEndtoComponent (Variables|Default|GetCable) (Variables|Default|GetLazerEnd) "None")
  (Rendering|SetVisibility (Variables|Default|GetLaserCollision) false false)
  (CallFunction|SetDefaults))

(event EventFlipVisible
  (Utilities|FlowControl|FlipFlop
    (:A
      (Rendering|SetVisibility (Variables|Default|GetLaserCollision) true false))
    (:B
      (Rendering|SetVisibility (Variables|Default|GetLaserCollision) false false))))

(fn ConstructionScript
  (|CallParentFunction))

(fn Ping
  (return (Collision|IsOverlappingActor (Variables|Default|GetLaserCollision) (Game|Player|GetPlayerPawn 0) :!class /Script/Engine.PrimitiveComponent) false))