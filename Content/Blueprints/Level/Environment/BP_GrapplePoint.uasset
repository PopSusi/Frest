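; A grapple point actor that shows a range indicator to the player and serves as an anchor for rope swinging.
; Once activated with a pawn, it shows a widget, turns it toward the camera each tick, and grows its fill as the pawn nears, tinting it green at full size.
; Rope swing events attach the pawn's capsule to the anchor through a physics constraint or break it.
; Deactivate is empty.
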(event Custom|StartRopeSwing
  (Class|PhysicsConstraintComponent|SetConstrainedComponents (Variables|Default|GetPhysicsConstraint) (Variables|Default|GetAnchor) "None" (Actor|GetComponentbyClass (Variables|Default|GetPawnRef) "/Script/Engine.CapsuleComponent") "None"))

(event Custom|EndRopeSwing
  (Class|PhysicsConstraintComponent|BreakConstraint (Variables|Default|GetPhysicsConstraint)))

(event EventBeginPlay
  (bind _asbpw_grapple_detection_node (Utilities|Casting|CastToBPW_GrappleDetectionNode (UserInterface|GetUserWidgetObject (Variables|Default|GetWidget)))
    (:then
      (Variables|Default|SetAs%20BPW%20Grapple%20Detection%20Node _asbpw_grapple_detection_node))
    (:CastFailed
      (Development|PrintString "CastFailed"))))

(event Collision|EventActorBeginOverlap
  (params (OtherActor :type Actor%20Object%20Reference)))

(event EventTick
  (params (DeltaSeconds :type Float%20%28single-precision%29))
  (bind _widget (Variables|Default|GetWidget))
  (if (Variables|Default|GetIsActive)
    (Transformation|SetWorldRotation _widget (Math|Rotator|FindLookatRotation (Transformation|GetWorldLocation _widget) (Transformation|GetWorldLocation (Variables|/Script/Engine.PlayerCameraManager|GetTransformComponent (Game|GetPlayerCameraManager 0)))) false false)
    (CallFunction|CheckDistancefromPlayer)))

(fn ConstructionScript)

(fn Activate
  (params (PawnRef :type BP%20Player%20Object%20Reference))
  (Variables|Default|SetIsActive true)
  (Rendering|SetVisibility (Variables|Default|GetWidget) true false)
  (Variables|Default|SetPawnRef PawnRef))

(fn Deactivate)

(fn CheckDistancefromPlayer
  (bind _returnvalue (Transformation|GetActorLocation))
  (bind _as_bpw_grapple_detection_node (Variables|Default|GetAs%20BPW%20Grapple%20Detection%20Node))
  (bind _pawnref (Variables|Default|GetPawnRef))
  (bind _returnvalue_2 (Transformation|GetActorLocation _pawnref))
  (bind _fill (Variables|/Game/UI/GameplayUI/GrappleUI/BPW_GrappleDetectionNode.BPW_GrappleDetectionNode_C|GetFill _as_bpw_grapple_detection_node))
  (bind _returnvalue_3 (- _returnvalue_2 _returnvalue))
  (bind _returnvalue_4 (Math|Vector|VectorLength _returnvalue_3))
  (bind _returnvalue_5 (Math|Float|MapRangeClamped _returnvalue_4 6e+02 1.2e+03 3e+02 1e+01))
  (Class|CanvasPanelSlot|SetSize (Class|WidgetLayoutLibrary|SlotasCanvasSlot _fill) (Math|Vector2D|MakeVector2D _returnvalue_5 _returnvalue_5))
  (Appearance|SetColorandOpacity _fill (select (== _returnvalue_5 3e+02) "(R=0.436045,G=1.000000,B=0.340369,A=1.000000)" "(R=1.000000,G=1.000000,B=1.000000,A=1.000000)") :!class /Script/UMG.Image))