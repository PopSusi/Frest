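; Checkpoint actor that saves player progress on overlap and updates the level's platform reset actor.
; Each player overlap, after a brief delay, sends health, gold flies and the capsule's transform (not the player's) to the Game Instance.
; The first time only, it swaps the flag material, plays a sound, broadcasts its checkpoint index and passes PlatformsToDelete to PlatformResets for removal.
; Older SaveGame slot code remains disconnected.
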(event OnComponentBeginOverlap(Box)
  (params (OverlappedComponent :type Primitive%20Component%20Object%20Reference) (OtherActor :type Actor%20Object%20Reference) (OtherComp :type Primitive%20Component%20Object%20Reference) (OtherBodyIndex :type Integer) (bFromSweep :type Boolean) (SweepResult :type Hit%20Result%20Structure%20%28by%20ref%29))
  ;[1 1 1] Checkpoint System. Saves the values associated with the player when overlapping the collider, except transform, which is the center of the checkpoint collider  - Ryan
  (bind _asbp_player (Utilities|Casting|CastToBP_Player OtherActor))
  (Utilities|FlowControl|Delay 0.1)
  (bind _playersave (Default|GetPlayerData _asbp_player))
  (Class|BPISaveGameInterface|SavePlayerData(Message) (Game|GetGameInstance) (Utilities|Struct|MakeS_PlayerData (Transformation|GetWorldTransform (Variables|Default|GetCapsule)) (.health _playersave) (.goldflies _playersave)) false)
  (Utilities|FlowControl|DoOnce false
    (:Completed
      (Rendering|Material|SetMaterial (Variables|Default|GetCylinder) 0 "/Game/Art/Props/Materials/Material_Instances/MI_CheckpointFlagUnlocked.MI_CheckpointFlagUnlocked")
      (Audio|PlaySound2D "/Game/Sounds/SFX/Gameplay/GoodJob.GoodJob" 1.0 1.0 0.0 0 0)
      (Default|CallNewCheckpointIndex (Variables|Default|GetCheckpointIndex))
      (CallFunction|OverlappedPlayer))))

(event Custom|OverlappedPlayer
  (bind _reset (Variables|Default|GetReset))
  ;[1 1 1] Checkpoint System. Saves the values associated with the player when overlapping the collider, except transform, which is the center of the checkpoint collider  - Ryan
  (Utilities|IsValid _reset
    (:Is%20Valid
      (Default|Remove _reset (Variables|Default|GetPlatforms%20to%20delete)))))

(event EventBeginPlay
  (bind _returnvalue (Actor|GetActorOfClass "/Game/Maps/BenProvince/Sequences/Platforms/PlatformResets.PlatformResets_C"))
  (Utilities|IsValid _returnvalue
    (:Is%20Valid
      (Variables|Default|SetReset _returnvalue))))

(fn ConstructionScript)