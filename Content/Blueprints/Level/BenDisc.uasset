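; BenDisc is a level actor that acts as the entry point to the "Benjamin" level.
; Overlapping its sphere shows a widget through a gate, and leaving hides it.
; Start hides the widget, closes the gate to keep it hidden, and after a short delay async-loads the 4Ben asset.
; A LoadWithImage screen takes UI-only input during loading and is notified through LoadDone when loading completes.
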(event OnComponentBeginOverlap(Sphere)
  (params (OverlappedComponent :type Primitive%20Component%20Object%20Reference) (OtherActor :type Actor%20Object%20Reference) (OtherComp :type Primitive%20Component%20Object%20Reference) (OtherBodyIndex :type Integer) (bFromSweep :type Boolean) (SweepResult :type Hit%20Result%20Structure%20%28by%20ref%29))
  (Utilities|FlowControl|Gate false
    (:Exit
      (Rendering|SetVisibility (Variables|Default|GetWidget) true false))))

(event OnComponentEndOverlap(Sphere)
  (params (OverlappedComponent :type Primitive%20Component%20Object%20Reference) (OtherActor :type Actor%20Object%20Reference) (OtherComp :type Primitive%20Component%20Object%20Reference) (OtherBodyIndex :type Integer))
  (Rendering|SetVisibility (Variables|Default|GetWidget) false false))

(event EventBeginPlay
  (|CallParentFunction) ; This node is disabled and will not be called.\nDrag off pins to build functionality.
)

(event Collision|EventActorBeginOverlap
  (params (OtherActor :type Actor%20Object%20Reference))
  (|CallParentFunction OtherActor) ; This node is disabled and will not be called.\nDrag off pins to build functionality.
)

(event EventTick
  (params (DeltaSeconds :type Float%20%28single-precision%29))
  (|CallParentFunction DeltaSeconds) ; This node is disabled and will not be called.\nDrag off pins to build functionality.
)

(event EventStart
  (bind _widget (Variables|Default|GetWidget))
  (Utilities|FlowControl|Sequence
    (:then_0
      (Rendering|SetVisibility _widget false false))
    (:then_1
      (Utilities|FlowControl|Delay 2.7)
      (Utilities|AsyncLoadAsset "/Game/Maps/BenProvince/4-Ben.4-Ben"
        (:then
          (bind _returnvalue (UserInterface|CreateWidget "/Game/UI/Widgets/LevelLoad/LoadWithImage.LoadWithImage_C" (Game|GetPlayerController 0) "/Game/Art/LevelScreens/BenHigh.BenHigh" (Utilities|Struct|MakeSoftWorldReference "/Game/Maps/BenProvince/4-Ben.4-Ben") "Benjamin"))
          (UserInterface|Viewport|AddtoPlayerScreen _returnvalue)
          (Input|SetInputModeUIOnly (Game|GetPlayerController 0) _returnvalue "DoNotLock" false))
        (:Completed
          (Default|LoadDone _returnvalue))))
    (:then_2
      (Utilities|FlowControl|Gate false) ; enters at Close
    )))

(fn ConstructionScript
  (|CallParentFunction))