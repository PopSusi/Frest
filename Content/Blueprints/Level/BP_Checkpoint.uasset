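; Checkpoint actor that saves player progress when BP_Player overlaps its box.
; After a short delay it reads the player's health and gold flies, then passes them to the GameInstance's SavePlayerDataMessage.
; The saved checkpoint transform comes from the checkpoint's capsule rather than from the player.
; Older game mode SaveGame-to-slot code remains in the graph but is disconnected.
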(event OnComponentBeginOverlap(Box)
  (params (OverlappedComponent :type Primitive%20Component%20Object%20Reference) (OtherActor :type Actor%20Object%20Reference) (OtherComp :type Primitive%20Component%20Object%20Reference) (OtherBodyIndex :type Integer) (bFromSweep :type Boolean) (SweepResult :type Hit%20Result%20Structure%20%28by%20ref%29))
  ;[1 1 1] Checkpoint System. Saves the values associated with the player when overlapping the collider, except transform, which is the center of the checkpoint collider  - Ryan
  (bind _asbp_player (Utilities|Casting|CastToBP_Player OtherActor))
  (Utilities|FlowControl|Delay 0.1)
  (bind _playersave (Default|GetPlayerData _asbp_player))
  (Class|BPISaveGameInterface|SavePlayerData(Message) (Game|GetGameInstance) (Utilities|Struct|MakeS_PlayerData (Transformation|GetWorldTransform (Variables|Default|GetCapsule)) (.health _playersave) (.goldflies _playersave)) false))

(fn ConstructionScript)