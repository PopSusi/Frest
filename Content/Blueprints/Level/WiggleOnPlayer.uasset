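; Component that makes its owning actor wiggle in scale when BP_Player begins overlapping the owner's static mesh.
; Each overlap restarts a short stop timer, but a wiggle only starts once the actor has returned to normal.
; While wiggling, Tick sets scale with a vector spring toward an offset along the right vector.
; Afterwards it interpolates scale back to one, then re-arms.
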(event Custom|StartWiggle
  (if (Variables|Default|GetNormal)
    (Variables|Default|SetWiggling true)
    (Variables|Default|SetNormal false)))

(event Custom|StopWiggle
  (Variables|Default|SetWiggling false))

(event Custom|OnComponentBeginOverlap_Event
  (params (OverlappedComponent :type Primitive%20Component%20Object%20Reference) (OtherActor :type Actor%20Object%20Reference) (OtherComp :type Primitive%20Component%20Object%20Reference) (OtherBodyIndex :type Integer) (bFromSweep :type Boolean) (SweepResult :type Hit%20Result%20Structure%20%28by%20ref%29))
  (Utilities|Casting|CastToBP_Player OtherActor)
  (if (Utilities|Time|IsValidTimerHandle (Variables|Default|GetCurrentTimer))
    (Utilities|Time|ClearandInvalidateTimerbyHandle (Variables|Default|GetCurrentTimer)))
  (bind _returnvalue (Utilities|Time|SetTimerbyEvent (delegate Custom|StopWiggle) 0.3 false true))
  (Variables|Default|SetCurrentTimer _returnvalue)
  (CallFunction|StartWiggle))

(event EventBeginPlay
  (Collision|AssignOnComponentBeginOverlap (Actor|GetComponentbyClass (Components|GetOwner) "/Script/Engine.StaticMeshComponent") (delegate Custom|OnComponentBeginOverlap_Event)))

(event EventTick
  (params (DeltaSeconds :type Float%20%28single-precision%29))
  (bind _returnvalue (Components|GetOwner))
  (bind _returnvalue_2 (Components|GetOwner))
  (bind _returnvalue_3 (Transformation|GetActorScale3D _returnvalue_2))
  (bind _returnvalue_4 (Math|Interpolation|VInterpTo _returnvalue_3 "1.000000,1.000000,1.000000" DeltaSeconds 1.0))
  (if (Variables|Default|GetWiggling)
    (bind _returnvalue_5 (Class|KismetMathLibrary|VectorSpringInterp "1.000000,1.000000,1.000000" (+ (* (Math|Vector|GetRightVector (Transformation|GetActorRotation _returnvalue)) 0.3) "1.000000,1.000000,1.000000") (Variables|Default|GetSpring%20State) 1e+02 0.0 DeltaSeconds 0.1 3.0))
    (Transformation|SetActorScale3D _returnvalue _returnvalue_5)
    (elif (not (Variables|Default|GetNormal))
      (Transformation|SetActorScale3D _returnvalue_2 _returnvalue_4)
      (if (Utilities|Operators|EqualEqual _returnvalue_4 "1.000000,1.000000,1.000000" 0.01)
        (Variables|Default|SetNormal true)))))