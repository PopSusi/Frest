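; Game is a set of shared helper functions for audio playback, player dialogue state and cone checks; LoadNewLevel is an empty stub.
; The Frest sound helpers load the Settings save on every call to choose mono or stereo assets, played in 2D or at a location.
; Movement helpers toggle BP_Player's HUD and IsTalking flag; enabling restores walking, while disabling either disables movement or only stops it, depending on MovementType.
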(fn LoadNewLevel
  (params (Level :type Level%20Data%20Structure) (World%20Context%20Object :type Object%20Object%20Reference)))

(fn WithinCone
  (params (SampleVector :type Vector) (TestVector :type Vector) (Precision :type Float%20%28double-precision%29))
  (return (> (Math|Vector|DotProduct SampleVector TestVector) Precision)))

(fn PlayFrestSound
  (params (Mono%20Sound%20Asset :type Sound%20Base%20Object%20Reference) (Stereo%20Sound%20Asset :type Sound%20Base%20Object%20Reference) (Location :type Vector))
  (bind _returnvalue (SaveGame|LoadGamefromSlot "Settings"))
  (bind _is_mono (Class|FromSaveInterface|IsMono(Message) _returnvalue))
  (if _is_mono
    (Audio|SpawnSoundatLocation 0 Mono%20Sound%20Asset Location "0, 0, 0" 1.0 1.0 0.0 0 0)
    (else
      (Audio|SpawnSoundatLocation 0 Stereo%20Sound%20Asset Location "0, 0, 0" 1.0 1.0 0.0 0 0))))

(fn PlayFrestSound2D
  (params (Mono%20Sound%20Asset :type Sound%20Base%20Object%20Reference) (Stereo%20Sound%20Asset :type Sound%20Base%20Object%20Reference))
  (bind _returnvalue (SaveGame|LoadGamefromSlot "Settings"))
  (bind _is_mono (Class|FromSaveInterface|IsMono(Message) _returnvalue))
  (if _is_mono
    (Audio|PlaySound2D 0 Mono%20Sound%20Asset 1.0 1.0 0.0 0 0)
    (else
      (Audio|PlaySound2D 0 Stereo%20Sound%20Asset 1.0 1.0 0.0 0 0))))

(fn FrestEnableMovement
  (params (WorldObjectReference :type Object%20Object%20Reference))
  (bind _returnvalue (Game|GetPlayerCharacter WorldObjectReference))
  (bind _asbp_player (Utilities|Casting|CastToBP_Player _returnvalue))
  (Widget|SetVisibility (Variables|/Game/Blueprints/Player/BP_Player.BP_Player_C|GetHUD _asbp_player) "Visible")
  (Pawn|Components|CharacterMovement|SetMovementMode (Variables|/Script/Engine.Character|GetCharacterMovement _returnvalue) "MOVE_Walking" 0)
  (Variables|/Game/Blueprints/Player/BP_Player.BP_Player_C|SetIsTalking _asbp_player false))

(fn FrestDisableMovement
  (params (WorldObjectReference :type Object%20Object%20Reference))
  (bind _returnvalue (Game|GetPlayerCharacter WorldObjectReference))
  (bind _charactermovement (Variables|/Script/Engine.Character|GetCharacterMovement _returnvalue))
  (bind _asbp_player (Utilities|Casting|CastToBP_Player _returnvalue))
  (Widget|SetVisibility (Variables|/Game/Blueprints/Player/BP_Player.BP_Player_C|GetHUD _asbp_player) "Hidden")
  (Variables|/Game/Blueprints/Player/BP_Player.BP_Player_C|SetIsTalking _asbp_player true)
  (if (Utilities|Enum|Equal(Enum) (Variables|/Game/Blueprints/Player/BP_Player.BP_Player_C|GetMovementType _asbp_player) "NewEnumerator0")
    (Pawn|Components|CharacterMovement|DisableMovement _charactermovement)
    (else
      (Components|Movement|StopMovementImmediately _charactermovement))))