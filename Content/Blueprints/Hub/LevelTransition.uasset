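; Hub level transition trigger that sends the player to another level when they overlap its box.
; On overlap it disables input, hides the player and its BenActor, then plays a sequence if its player is valid.
; Alongside the sequence it async-loads the target world, runs a delayed iris-in, and spins in a while loop on a ready flag before opening the level.
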(event OnComponentBeginOverlap(Box)
  (params (OverlappedComponent :type Primitive%20Component%20Object%20Reference) (OtherActor :type Actor%20Object%20Reference) (OtherComp :type Primitive%20Component%20Object%20Reference) (OtherBodyIndex :type Integer) (bFromSweep :type Boolean) (SweepResult :type Hit%20Result%20Structure%20%28by%20ref%29))
  (bind _sequence (Variables|Default|GetSequence))
  (bind _leveltoload (Variables|Default|GetLevelToLoad))
  (bind _sequenceplayer (Variables|/Script/LevelSequence.LevelSequenceActor|GetSequencePlayer _sequence))
  (bind _asbp_player (Utilities|Casting|CastToBP_Player OtherActor))
  (Input|DisableInput _asbp_player (Game|GetPlayerController 0))
  (Rendering|SetActorHiddenInGame (Variables|/Game/Blueprints/Player/BP_Player.BP_Player_C|GetBenActor _asbp_player) true)
  (Rendering|SetActorHiddenInGame _asbp_player true)
  (Utilities|IsValid _sequenceplayer
    (:Is%20Valid
      (Sequencer|Player|Play _sequenceplayer :!class /Script/MovieScene.MovieSceneSequencePlayer)
      (Utilities|AsyncLoadAsset (.worldasset (.leveltoload _leveltoload))
        (:then
          (Utilities|FlowControl|Delay 0.3)
          (Default|Irisin _asbp_player)
          (Utilities|FlowControl|Delay 1.0)
          (while (not (Variables|Default|GetReadyToLoad))
            _)
          (Game|OpenLevel(byObjectReference) (.worldasset (.leveltoload _leveltoload))))
        (:Completed
          (Variables|Default|SetReadyToLoad true))))))

(event EventBeginPlay)

(event Collision|EventActorBeginOverlap
  (params (OtherActor :type Actor%20Object%20Reference)))

(event EventTick
  (params (DeltaSeconds :type Float%20%28single-precision%29)))

(fn ConstructionScript)