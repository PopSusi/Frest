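; Boss key pickup that ends the level and returns the player to the hub world.
; On pickup it starts a camera fade, saves collected codexes and the player's GoldFlies through Game Instance messages, runs the parent pickup logic and opens HubWorld.
; With codexes present, the parent call, GoldFlies save and level open sit inside the per-codex loop.
; An async-load path with a loading-screen widget is left unconnected.
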(event EventBeginPlay
  (|CallParentFunction) ; This node is disabled and will not be called.\nDrag off pins to build functionality.
)

(event Collision|EventActorBeginOverlap
  (params (OtherActor :type Actor%20Object%20Reference))
  (|CallParentFunction OtherActor) ; This node is disabled and will not be called.\nDrag off pins to build functionality.
)

(event EventTick
  (params (DeltaSeconds :type Float%20%28single-precision%29))
  (|CallParentFunction DeltaSeconds) ; This node is disabled and will not be called.\nDrag off pins to build functionality.
)

(event EventOnPickup
  (params (Player :type BP%20Player%20Object%20Reference))
  (bind _codexes (Variables|Default|GetCodexes))
  (bind _codexes_2 (Variables|/Game/Maps/CodexUnlocks/CodexsToUnlock.CodexsToUnlock_C|GetCodexes _codexes))
  (CameraFades|StartCameraFade :self (Game|GetPlayerCameraManager 0) :ToAlpha 2.0 :Duration 2.0 :bHoldWhenFinished true)
  (if (Utilities|Array|IsNotEmpty _codexes_2)
    (for _array_element _codexes_2
      (Class|BPISaveGameInterface|SaveLevelCodexes(Message) (Game|GetGameInstance) _array_element)
      (|CallParentFunction 0)
      (Class|BPISaveGameInterface|SavePlayerData(Message) (Game|GetGameInstance) (Utilities|Struct|MakeS_PlayerData "0.000000,0.000000,0.000000|0.000000,0.000000,0.000000|1.000000,1.000000,1.000000" 3 (Variables|/Game/Blueprints/Player/BP_Player.BP_Player_C|GetGoldFlies Player)) false)
      (Game|OpenLevel(byObjectReference) "/Game/Maps/HubWorld/HubWorld.HubWorld" true "Default"))
    (else
      (|CallParentFunction 0)
      (Class|BPISaveGameInterface|SavePlayerData(Message) (Game|GetGameInstance) (Utilities|Struct|MakeS_PlayerData "0.000000,0.000000,0.000000|0.000000,0.000000,0.000000|1.000000,1.000000,1.000000" 3 (Variables|/Game/Blueprints/Player/BP_Player.BP_Player_C|GetGoldFlies Player)) false)
      (Game|OpenLevel(byObjectReference) "/Game/Maps/HubWorld/HubWorld.HubWorld" true "Default"))))

(fn ConstructionScript
  (|CallParentFunction))