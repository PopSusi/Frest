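; LevelMapTable is a hub actor that shows an interaction prompt when the player comes near the map table.
; It creates a WB_MapPrompt widget on BeginPlay and stores it for reuse.
; Sphere overlap events add the widget to the viewport or remove it, filtered by an exact BP_Player class check.
; The Interact event is present but has no logic.
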(event OnComponentEndOverlap(Sphere)
  (params (OverlappedComponent :type Primitive%20Component%20Object%20Reference) (OtherActor :type Actor%20Object%20Reference) (OtherComp :type Primitive%20Component%20Object%20Reference) (OtherBodyIndex :type Integer))
  (if (== (Utilities|GetClass OtherActor) "/Game/Blueprints/Player/BP_Player.BP_Player_C")
    (Widget|RemovefromParent (Variables|Default|GetInteractWithMapUI))))

(event OnComponentBeginOverlap(Sphere)
  (params (OverlappedComponent :type Primitive%20Component%20Object%20Reference) (OtherActor :type Actor%20Object%20Reference) (OtherComp :type Primitive%20Component%20Object%20Reference) (OtherBodyIndex :type Integer) (bFromSweep :type Boolean) (SweepResult :type Hit%20Result%20Structure%20%28by%20ref%29))
  (if (== (Utilities|GetClass OtherActor) "/Game/Blueprints/Player/BP_Player.BP_Player_C")
    (UserInterface|Viewport|AddtoViewport (Variables|Default|GetInteractWithMapUI) 0)))

(event EventBeginPlay
  (bind _returnvalue (UserInterface|CreateWidget "/Game/UI/Widgets/Menus/WB_MapPrompt.WB_MapPrompt_C"))
  (Variables|Default|SetInteractWithMapUI _returnvalue))

(event Collision|EventActorBeginOverlap
  (params (OtherActor :type Actor%20Object%20Reference)))

(event EventTick
  (params (DeltaSeconds :type Float%20%28single-precision%29)))

(event EventInteract)

(fn ConstructionScript)