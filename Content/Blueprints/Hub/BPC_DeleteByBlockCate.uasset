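; BPC_DeleteByBlockCate is an actor component that removes its owner when a given block category is already recorded in game data.
; On BeginPlay, if CateThatDeletesMe is valid, it checks the game instance's game data for that category among the world-block codex entries.
; On a match it destroys all of the owner's child actors, then the owner itself.
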(event EventBeginPlay
  (bind _returnvalue (Components|GetOwner))
  (Utilities|IsValid (Variables|Default|GetCateThatDeletesMe)
    (:Is%20Valid
      (bind _savegamedata (Class|BPISaveGameInterface|GetGameData(Message) (Game|GetGameInstance)))
      (if (Utilities|Array|ContainsItem (Variables|/Game/Blueprints/Saving/BP_SaveGame.BP_SaveGame_C|GetCodexEntries%20-%20WorldBlocks _savegamedata) (Variables|Default|GetCateThatDeletesMe))
        (for _array_element (Actor|GetAllChildActors _returnvalue true)
          (Actor|DestroyActor _array_element))
        (Actor|DestroyActor _returnvalue)))))

(event EventTick
  (params (DeltaSeconds :type Float%20%28single-precision%29)))