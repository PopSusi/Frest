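; Level select node on the hub overworld map that either loads a level or, as a back-out node, returns control to BP_Player and closes the map.
; BeginPlay sets the icon on a dynamic material and greys it unless back-out or found in saved codex entries.
; Sphere overlap toggles the player's level or locked UI, scaling the visual by timeline when active.
; Interacting with an active node async-loads the level behind an image loading widget.
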(event OnComponentEndOverlap(Sphere)
  (params (OverlappedComponent :type Primitive%20Component%20Object%20Reference) (OtherActor :type Actor%20Object%20Reference) (OtherComp :type Primitive%20Component%20Object%20Reference) (OtherBodyIndex :type Integer))
  (bind _asbp_overworld_player (Utilities|Casting|CastToBP_OverworldPlayer OtherActor))
  (if (Variables|Default|GetActive)
    (Widget|RemovefromParent (Variables|/Game/Blueprints/Player/BP_OverworldPlayer.BP_OverworldPlayer_C|GetLevelUI _asbp_overworld_player))
    (bind _scale (Timeline|Scale%20Plane ReverseFromEnd)
      (:Update
        (Transformation|SetRelativeScale3D (Variables|Default|GetVisual) (Math|Conversions|ToVector(Float) _scale))))
    (else
      (Widget|RemovefromParent (Variables|/Game/Blueprints/Player/BP_OverworldPlayer.BP_OverworldPlayer_C|GetNotUnlockedUI _asbp_overworld_player)))))

(event OnComponentBeginOverlap(Sphere)
  (params (OverlappedComponent :type Primitive%20Component%20Object%20Reference) (OtherActor :type Actor%20Object%20Reference) (OtherComp :type Primitive%20Component%20Object%20Reference) (OtherBodyIndex :type Integer) (bFromSweep :type Boolean) (SweepResult :type Hit%20Result%20Structure%20%28by%20ref%29))
  (bind _asbp_overworld_player (Utilities|Casting|CastToBP_OverworldPlayer OtherActor))
  (if (Variables|Default|GetActive)
    (UserInterface|Viewport|AddtoViewport (Variables|/Game/Blueprints/Player/BP_OverworldPlayer.BP_OverworldPlayer_C|GetLevelUI _asbp_overworld_player) 0)
    (bind _scale (Timeline|Scale%20Plane PlayFromStart)
      (:Update
        (Transformation|SetRelativeScale3D (Variables|Default|GetVisual) (Math|Conversions|ToVector(Float) _scale))))
    (else
      (UserInterface|Viewport|AddtoViewport (Variables|/Game/Blueprints/Player/BP_OverworldPlayer.BP_OverworldPlayer_C|GetNotUnlockedUI _asbp_overworld_player) 0))))

(event Custom|Load
  (bind _leveldata (Variables|Default|GetLevelData))
  (Utilities|FlowControl|DoOnce false
    (:Completed
      (bind _asbp_overworld_player (Utilities|Casting|CastToBP_OverworldPlayer (Game|Player|GetPlayerPawn 0))
        (:then
          (Utilities|IsValid (Variables|/Game/Blueprints/Player/BP_OverworldPlayer.BP_OverworldPlayer_C|GetLevelUI _asbp_overworld_player)
            (:Is%20Valid
              (Widget|RemovefromParent (Variables|/Game/Blueprints/Player/BP_OverworldPlayer.BP_OverworldPlayer_C|GetLevelUI _asbp_overworld_player)))
            (:Is%20Not%20Valid
              _)))
        (:CastFailed
          _))
      (Utilities|AsyncLoadAsset (.worldasset (.leveltoload _leveldata))
        (:then
          ;[1 1 1] If image, load image widget
          (bind _returnvalue (UserInterface|CreateWidget "/Game/UI/Widgets/LevelLoad/LoadWithImage.LoadWithImage_C" (Game|GetPlayerController 0) (.customimage _leveldata) (Utilities|Struct|MakeSoftWorldReference (Variables|Default|GetLevel))))
          (Variables|/Game/UI/Widgets/LevelLoad/LoadWithImage.LoadWithImage_C|SetSpawnTag _returnvalue "NoLoadMenu")
          (UserInterface|Viewport|AddtoViewport _returnvalue 0))
        (:Completed
          (Default|LoadDone _returnvalue))))))

(event EventBeginPlay
  (bind _visual (Variables|Default|GetVisual))
  (bind _leveldata (Variables|Default|GetLevelData))
  (bind _returnvalue (Rendering|Material|CreateDynamicMaterialInstance _visual 0 (Rendering|Material|GetMaterial _visual 0) "None" :!class /Script/Engine.PrimitiveComponent))
  (Rendering|Material|SetTextureParameterValue _returnvalue "IconRef" (Variables|Default|GetIcon))
  (if (Variables|Default|GetBackOut)
    (Variables|Default|SetActive true)
    (else
      (bind _savegamedata (Class|BPISaveGameInterface|GetGameData(Message) (Game|GetGameInstance)))
      (if (Utilities|Array|ContainsItem (Variables|/Game/Blueprints/Saving/BP_SaveGame.BP_SaveGame_C|GetCodexEntries%20-%20Levels _savegamedata) (Variables|Default|GetEntry))
        (Variables|Default|SetActive true)
        (Utilities|FlowControl|DoOnce false) ; enters at Reset
        (else
          (Rendering|Material|SetScalarParameterValue _returnvalue "Grey" 1.0 :!class /Script/Engine.MaterialInstanceDynamic))))))

(event Collision|EventActorBeginOverlap
  (params (OtherActor :type Actor%20Object%20Reference)))

(event EventTick
  (params (DeltaSeconds :type Float%20%28single-precision%29)))

(fn ConstructionScript)

(fn Interact
  (bind _returnvalue (Game|GetPlayerController 0))
  (if (Variables|Default|GetBackOut)
    (bind _returnvalue_2 (Actor|GetActorOfClass "/Game/Blueprints/Player/BP_Player.BP_Player_C"))
    (Pawn|Components|CharacterMovement|SetMovementMode (Variables|/Script/Engine.Character|GetCharacterMovement _returnvalue_2) "MOVE_Walking" 0)
    (Pawn|UnPossess _returnvalue)
    (Pawn|Possess _returnvalue _returnvalue_2)
    (Game|Player|SetViewTargetwithBlend _returnvalue _returnvalue_2 0.0 "VTBlend_Linear" 0.0 false)
    (bind _outactors (Actor|GetAllActorsOfClass "/Game/Blueprints/Hub/LevelMapTable.LevelMapTable_C"))
    (for _array_element _outactors
      (Default|AttemptDestroyMap _array_element))
    (return false)
    (elif (Variables|Default|GetActive)
      (CallFunction|Load))))