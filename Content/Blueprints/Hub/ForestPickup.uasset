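; Forest pickup that returns the player to the hub world when collected.
; On pickup it saves the level name via the game instance, starts a camera fade, unlocks its codex entry if valid and still locked, and runs the parent pickup logic.
; It then saves the player's gold flies and immediately opens the hub level.
; An async-load loading-screen widget path is present but never runs.
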(event EventBeginPlay
  (|CallParentFunction) ; This node is disabled and will not be called.\nDrag off pins to build functionality.
)

(event Collision|EventActorBeginOverlap
  (params (OtherActor :type Actor%20Object%20Reference))
  (|CallParentFunction OtherActor) ; This node is disabled and will not be called.\nDrag off pins to build functionality.
)

(event EventTick
  (params (DeltaSeconds :type Float%20%28single-precision%29))
  (|CallParentFunction DeltaSeconds) ; This node is disabled and will not be called.\nDrag off pins to build functionality.
)

(event EventOnPickup
  (params (Player :type BP%20Player%20Object%20Reference))
  (bind _codextounlock (Variables|Default|GetCodexToUnlock))
  (Class|BPISaveGameInterface|SaveLevel(Message) (Game|GetGameInstance) (Variables|Default|GetSaveLevelName))
  (CameraFades|StartCameraFade :self (Game|GetPlayerCameraManager 0) :ToAlpha 2.0 :Duration 2.0 :bHoldWhenFinished true)
  (Utilities|IsValid _codextounlock
    (:Is%20Valid
      (if (Variables|/Game/UI/Blueprints/BP_CodexEntry.BP_CodexEntry_C|GetUnlocked _codextounlock)
        (|CallParentFunction 0 :!label _label)
        (else
          (Default|Unlock _codextounlock)
          (|CallParentFunction 0))))
    (:Is%20Not%20Valid
      (goto _label)))
  (Class|BPISaveGameInterface|SavePlayerData(Message) (Game|GetGameInstance) (Utilities|Struct|MakeS_PlayerData "0.000000,0.000000,0.000000|0.000000,0.000000,0.000000|1.000000,1.000000,1.000000" 3 (Variables|/Game/Blueprints/Player/BP_Player.BP_Player_C|GetGoldFlies Player)) false)
  (Game|OpenLevel(byObjectReference) "/Game/Maps/HubWorld/HubWorld.HubWorld" true "Default"))

(fn ConstructionScript
  (|CallParentFunction))