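; CateHouse is a hub building actor that shows a tent or house mesh according to its HouseLevel.
; SetHouse switches the HouseTemp static mesh and its relative offset for each level, destroying the actor for any unhandled level.
; UpdateHouse plays a success sound and a temporary Niagara effect, calling SetHouse shortly after the effect starts so the swap accompanies it.
; BeginPlay only waits a tick and does not set the mesh.
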(event Custom|SetHouse
  (bind _housetemp (Variables|Default|GetHouseTemp))
  (switch int (Variables|Default|GetHouseLevel)
    (:Default
      (Actor|DestroyActor))
    (:0
      (Components|StaticMesh|SetStaticMesh _housetemp "/Game/Art/Props/Models/SM_Tent3.SM_Tent3")
      (Transformation|SetRelativeLocation _housetemp "0, 0, 0" false false))
    (:1
      (Components|StaticMesh|SetStaticMesh _housetemp "/Game/Art/Props/Models/SM_Tent.SM_Tent")
      (Transformation|SetRelativeLocation _housetemp "0, 0, 0" false false))
    (:2
      (Components|StaticMesh|SetStaticMesh _housetemp "/Game/Art/ProgrammerArt/SM_SM_HouseTemp.SM_SM_HouseTemp")
      (Transformation|SetRelativeLocation _housetemp "0.000000,50.000000,1250.000000" false false))))

(event Custom|UpdateHouse
  (Audio|PlaySound2D "/Game/Sounds/SFX/Gameplay/GoodJob.GoodJob" 1.0 1.0 0.0 0 0)
  (bind _returnvalue (AddComponent|AddNiagaraComponent false))
  (Components|Activation|Activate _returnvalue false)
  (Utilities|FlowControl|Delay 0.2)
  (CallFunction|SetHouse)
  (Utilities|FlowControl|Delay 1.0)
  (Components|DestroyComponent _returnvalue))

(event EventBeginPlay
  (Utilities|FlowControl|DelayUntilNextTick))

(event Collision|EventActorBeginOverlap
  (params (OtherActor :type Actor%20Object%20Reference)))

(event EventTick
  (params (DeltaSeconds :type Float%20%28single-precision%29)))

(fn ConstructionScript)