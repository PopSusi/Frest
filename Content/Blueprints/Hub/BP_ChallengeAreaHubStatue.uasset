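; BP_ChallengeAreaHubStatue is a hub statue that appears only if the player has completed its associated time trial challenge.
; On BeginPlay it reads game data from the game instance and checks whether ChallengeAreaCollectibles contains its AssetThatSpawnsMe.
; If the entry is missing, it disables the static mesh's collision, deactivates it and hides it in game rather than destroying the actor.
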(event EventBeginPlay
  (bind _staticmesh (Variables|Default|GetStaticMesh))
  ;[1 1 1] Time Trial Statue only appears if the player has completed the associated time trial - Ryan
  (bind _savegamedata (Class|BPISaveGameInterface|GetGameData(Message) (Game|GetGameInstance)))
  (if (not (Utilities|Array|ContainsItem (Variables|/Game/Blueprints/Saving/BP_SaveGame.BP_SaveGame_C|GetChallenge%20Area%20Collectibles _savegamedata) (Variables|Default|GetAssetThatSpawnsMe)))
    (Collision|SetCollisionEnabled (Variables|Default|GetStaticMesh) "NoCollision")
    (Components|Activation|SetActive _staticmesh false false)
    (Development|SetHiddeninGame _staticmesh true false)))

(event Collision|EventActorBeginOverlap
  (params (OtherActor :type Actor%20Object%20Reference)))

(event EventTick
  (params (DeltaSeconds :type Float%20%28single-precision%29)))

(fn ConstructionScript)