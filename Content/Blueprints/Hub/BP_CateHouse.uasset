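; BP_CateHouse is a hub house actor whose static mesh reflects its HouseLevel, progressing from tents to Cate houses.
; UpdateHouse plays a sound and a temporary Niagara effect, calling SetHouse after a short delay to swap the HouseTemp mesh.
; The top two levels share one mesh, and any unhandled level destroys the actor.
; BeginPlay only waits a tick without setting the house, and an SM_Catehouse2 branch is disconnected.
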(event Custom|SetHouse
  (bind _housetemp (Variables|Default|GetHouseTemp))
  (bind _housetemp_2 (Variables|Default|GetHouseTemp))
  (bind _housetemp_3 (Variables|Default|GetHouseTemp))
  (bind _housetemp_4 (Variables|Default|GetHouseTemp))
  (switch int (Variables|Default|GetHouseLevel)
    (:Default
      (Actor|DestroyActor))
    (:0
      (Components|StaticMesh|SetStaticMesh _housetemp_3 "/Game/Art/Props/Models/SM_Tent3.SM_Tent3")
      (Transformation|SetRelativeLocation _housetemp_3 "0, 0, 0" false false))
    (:1
      (Components|StaticMesh|SetStaticMesh _housetemp "/Game/Art/Props/Models/SM_Tent.SM_Tent")
      (Transformation|SetRelativeLocation _housetemp "0, 0, 0" false false))
    (:2
      (Components|StaticMesh|SetStaticMesh _housetemp_4 "/Game/Art/Props/Models/SM_Catehouse3.SM_Catehouse3")
      (Transformation|SetRelativeLocation _housetemp_4 "0, 0, 0" false false))
    (:3
      (Components|StaticMesh|SetStaticMesh _housetemp_2 "/Game/Art/Props/Models/SM_Catehouse1.SM_Catehouse1" :!label _label)
      (Transformation|SetRelativeLocation _housetemp_2 "0, 0, 0" false false))
    (:4
      (goto _label))))

(event Custom|UpdateHouse
  (Audio|PlaySound2D "/Game/Sounds/SFX/Gameplay/GoodJob.GoodJob" 1.0 1.0 0.0 0 0)
  (bind _returnvalue (AddComponent|AddNiagaraComponent false))
  (Components|Activation|Activate _returnvalue false)
  (Utilities|FlowControl|Delay 0.2)
  (CallFunction|SetHouse)
  (Utilities|FlowControl|Delay 1.0)
  (Components|DestroyComponent _returnvalue))

(event EventBeginPlay
  (Utilities|FlowControl|DelayUntilNextTick))

(event Collision|EventActorBeginOverlap
  (params (OtherActor :type Actor%20Object%20Reference)))

(fn ConstructionScript)