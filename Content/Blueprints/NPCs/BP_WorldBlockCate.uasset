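; BP_WorldBlockCate is an NPC tied to a world blocker that a conversation clears, gated by level and codex unlocks.
; One tick after BeginPlay it destroys itself if its level is absent from the game instance's unlocked levels.
; Otherwise it destroys a valid Block if its codex is already unlocked, or sets up UI with the Block intact.
; TalkDone marks the codex unlocked and plays a level sequence.
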(event EventBeginPlay
  (bind _block (Variables|Default|GetBlock))
  (Utilities|FlowControl|DelayUntilNextTick)
  (bind _savegamedata (Class|BPISaveGameInterface|GetGameData(Message) (Game|GetGameInstance)))
  (if (Utilities|Array|ContainsItem (Variables|/Game/Blueprints/Saving/BP_SaveGame.BP_SaveGame_C|GetLevelsUnlocked _savegamedata) (Variables|Default|GetLevelToBaseOffOf))
    (if (Variables|/Game/UI/Blueprints/BP_CodexEntry.BP_CodexEntry_C|GetUnlocked (Variables|Default|GetCodexThatUnlocksMe))
      (Utilities|IsValid _block
        (:Is%20Valid
          (Actor|DestroyActor _block))))
    (CallFunction|SetupUI)
    (else
      (Actor|DestroyActor))))

(event Collision|EventActorBeginOverlap
  (params (OtherActor :type Actor%20Object%20Reference))
  (|CallParentFunction OtherActor) ; This node is disabled and will not be called.\nDrag off pins to build functionality.
)

(event EventTick
  (params (DeltaSeconds :type Float%20%28single-precision%29))
  (|CallParentFunction DeltaSeconds) ; This node is disabled and will not be called.\nDrag off pins to build functionality.
)

(event EventTalkDone
  (Variables|/Game/UI/Blueprints/BP_CodexEntry.BP_CodexEntry_C|SetUnlocked (Variables|Default|GetCodexThatUnlocksMe) true)
  (Sequencer|Player|Play (Variables|/Script/LevelSequence.LevelSequenceActor|GetSequencePlayer (Variables|Default|GetLevelSequence)) :!class /Script/MovieScene.MovieSceneSequencePlayer))

(fn ConstructionScript
  (|CallParentFunction))