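; Side quest NPC that appears only once its level is beaten and starts a time trial after its conversation.
; On BeginPlay it destroys itself unless its assigned codex entry is unlocked, otherwise it runs the parent setup.
; Interact, once the conversation has ended, adds a WB_Timer widget to the viewport, clears the end-of-conversation flag and disables the dialogue trigger's collision.
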(event EventBeginPlay
  ;[1 1 1] Sidequest NPC only appears if the level has been beaten - Ryan
  (if (Variables|/Game/UI/Blueprints/BP_CodexEntry.BP_CodexEntry_C|GetUnlocked (Variables|Default|GetCodexThatUnlocksMe))
    (|CallParentFunction)
    (else
      (Actor|DestroyActor))))

(event Collision|EventActorBeginOverlap
  (params (OtherActor :type Actor%20Object%20Reference))
  (|CallParentFunction OtherActor) ; This node is disabled and will not be called.\nDrag off pins to build functionality.
)

(event EventTick
  (params (DeltaSeconds :type Float%20%28single-precision%29))
  (|CallParentFunction DeltaSeconds) ; This node is disabled and will not be called.\nDrag off pins to build functionality.
)

(fn ConstructionScript
  (|CallParentFunction))

(fn Interact
  ;[1 1 1] After talking to this NPC, the time trial will start - Ryan
  (if (Variables|Default|GetEndOfConversation)
    (bind _returnvalue (UserInterface|CreateWidget "/Game/UI/Widgets/HUD/WB_Timer.WB_Timer_C"))
    (UserInterface|Viewport|AddtoViewport _returnvalue 0)
    (Variables|Default|SetEndOfConversation false)
    (Collision|SetCollisionEnabled (Variables|Default|GetDialogue%20Trigger) "NoCollision")
    (return false)))