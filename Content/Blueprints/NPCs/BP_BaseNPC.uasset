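; Base NPC actor that shows a talk prompt while the player overlaps its trigger and plays click-through dialogue.
; BeginPlay creates the prompt and dialogue widgets, and Interact calls Talk to advance one line of the Dialogue array per call.
; Player movement is disabled during conversation and restored after the last line, when the index resets for replay, completion flags are set and the empty EndDialogue event fires.
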(event OnComponentBeginOverlap(DialogueTrigger)
  (params (OverlappedComponent :type Primitive%20Component%20Object%20Reference) (OtherActor :type Actor%20Object%20Reference) (OtherComp :type Primitive%20Component%20Object%20Reference) (OtherBodyIndex :type Integer) (bFromSweep :type Boolean) (SweepResult :type Hit%20Result%20Structure%20%28by%20ref%29))
  ;[1 1 1] Shows and Removes "Talk to NPC" UI Prompt on Enter and Exit Overlap with the NPC - Ryan
  (if (== (Utilities|GetClass OtherActor) "/Game/Blueprints/Player/BP_Player.BP_Player_C")
    (UserInterface|Viewport|AddtoViewport (Variables|Default|GetDialogue%20Prompt%20UI) 0)))

(event OnComponentEndOverlap(DialogueTrigger)
  (params (OverlappedComponent :type Primitive%20Component%20Object%20Reference) (OtherActor :type Actor%20Object%20Reference) (OtherComp :type Primitive%20Component%20Object%20Reference) (OtherBodyIndex :type Integer))
  ;[1 1 1] Shows and Removes "Talk to NPC" UI Prompt on Enter and Exit Overlap with the NPC - Ryan
  (if (== (Utilities|GetClass OtherActor) "/Game/Blueprints/Player/BP_Player.BP_Player_C")
    (Widget|RemovefromParent (Variables|Default|GetDialogue%20Prompt%20UI))))

(event Custom|EndDialogue)

(event EventBeginPlay
  ;[1 1 1] Creating Dialogue UI Widget on Begin Play - Ryan
  (bind _returnvalue (UserInterface|CreateWidget "/Game/UI/Widgets/Menus/WB_Dialogue.WB_Dialogue_C" (Game|GetPlayerController 0)))
  (Variables|Default|SetDialogue%20UI _returnvalue)
  (bind _returnvalue_2 (UserInterface|CreateWidget "/Game/UI/Widgets/Menus/WB_DialoguePrompt.WB_DialoguePrompt_C"))
  (Variables|Default|SetDialogue%20Prompt%20UI _returnvalue_2))

(event Collision|EventActorBeginOverlap
  (params (OtherActor :type Actor%20Object%20Reference)))

(event EventTick
  (params (DeltaSeconds :type Float%20%28single-precision%29)))

(event EventTalk
  ;[1 1 1] NPC Dialogue. If the player is in range, they can interact with an NPC to click through their dialogue. Movement is halted while talking to the NPC. They can talk to the NPC as many times as they want - Ryan
  (if (<= (Variables|Default|GetDialogue%20Index) (- (Utilities|Array|Length (Variables|Default|GetDialogue)) 1))
    (if (== (Variables|Default|GetDialogue%20Index) 0)
      (UserInterface|Viewport|AddtoViewport (Variables|Default|GetDialogue%20UI) 0)
      (Pawn|Components|CharacterMovement|DisableMovement (Variables|/Script/Engine.Character|GetCharacterMovement (Game|GetPlayerCharacter 0))))
    (Rendering|Components|TextRender|SetText (Variables|/Game/UI/Widgets/Menus/WB_Dialogue.WB_Dialogue_C|GetDialogueText (Variables|Default|GetDialogue%20UI)) (Utilities|Text|ToText(String) (Utilities|Array|Get(acopy) (Variables|Default|GetDialogue) (Variables|Default|GetDialogue%20Index))))
    (Math|Integer|IncrementInt (Variables|Default|GetDialogue%20Index))
    (else
      (Widget|RemovefromParent (Variables|Default|GetDialogue%20UI))
      (Pawn|Components|CharacterMovement|SetMovementMode (Variables|/Script/Engine.Character|GetCharacterMovement (Game|GetPlayerCharacter 0)) "MOVE_Walking" 0)
      (Variables|Default|SetDialogue%20Index 0)
      (if (Variables|Default|GetFirstTalkComplete)
        _
        (else
          (Variables|Default|SetFirstTalkComplete true)))
      (Variables|Default|SetEndOfConversation true)
      (CallFunction|EndDialogue))))

(fn ConstructionScript)

(fn Interact
  (CallFunction|Talk)
  (return false))