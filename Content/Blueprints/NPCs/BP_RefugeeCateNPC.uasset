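; Refugee Cate NPC, a rescuable collectible that unlocks a Codex entry through dialogue.
; Interact calls Talk, which meows, runs the parent dialogue and, once the first talk completes, saves the entry through the GameInstance.
; A new unlock also increments the game mode's rescued count and animates the player's HUD tracker.
; BeginPlay names the NPC from its Codex header and despawns it after a short delay if already rescued.
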(event EventBeginPlay
  ;[1 1 1] Despawn Refugee Cate if they have been rescued already on repeat plays - Ryan
  (Variables|Default|SetName (Variables|/Game/UI/Blueprints/BP_CodexEntry.BP_CodexEntry_C|GetCodexHeader (Variables|Default|GetCodexToUnlock)))
  (|CallParentFunction)
  (bind _savegamedata (Class|BPISaveGameInterface|GetGameData(Message) (Game|GetGameInstance)))
  (if (Utilities|Array|ContainsItem (Variables|/Game/Blueprints/Saving/BP_SaveGame.BP_SaveGame_C|GetCodexEntries%20-%20Cates _savegamedata) (Variables|Default|GetCodexToUnlock))
    (Utilities|FlowControl|Delay 0.2)
    (Actor|DestroyActor)))

(event Collision|EventActorBeginOverlap
  (params (OtherActor :type Actor%20Object%20Reference))
  (|CallParentFunction OtherActor) ; This node is disabled and will not be called.\nDrag off pins to build functionality.
)

(event EventTick
  (params (DeltaSeconds :type Float%20%28single-precision%29))
  ;[1 1 1] Despawn Refugee Cate if they have been rescued already on repeat plays - Ryan
  (|CallParentFunction DeltaSeconds) ; This node is disabled and will not be called.\nDrag off pins to build functionality.
)

(event EventTalk
  (bind _returnvalue (Game|GetGameInstance))
  ;[1 1 1] When Talking to an NPC that unlocks a Codex Entry, it will unlock once dialogue with the NPC has been completed once, and update the progress on the collected codex entries - Ryan
  (Audio|PlaySound2D "/Game/Sounds/SFX/meow.meow" 1.0 1.0 0.0 0 0)
  (|CallParentFunction)
  (bind _savegamedata (Class|BPISaveGameInterface|GetGameData(Message) _returnvalue))
  (if (not (Utilities|Array|ContainsItem (Variables|/Game/Blueprints/Saving/BP_SaveGame.BP_SaveGame_C|GetCodexEntries%20-%20Cates _savegamedata) (Variables|Default|GetCodexToUnlock)))
    (if (Variables|Default|GetFirstTalkComplete)
      (Class|BPISaveGameInterface|SaveCatesCodexes(Message) _returnvalue (Variables|Default|GetCodexToUnlock))
      (bind _asbp_player (Utilities|Casting|CastToBP_Player (Game|GetPlayerCharacter 0)))
      (bind _asplatforming_game_mode (Utilities|Casting|CastToPlatformingGameMode (Game|GetGameMode)))
      (bind _result (Math|Integer|IncrementInt (Variables|/Game/GameModes/PlatformingGameMode.PlatformingGameMode_C|GetCollectedRefugeeCates _asplatforming_game_mode))
        (:%20%20
          (bind _output_get (Variables|/Game/GameModes/PlatformingGameMode.PlatformingGameMode_C|SetCollectedRefugeeCates _asplatforming_game_mode _result))
          (Variables|/Script/UMG.TextBlock|SetText (Variables|/Game/UI/Widgets/HUD/WB_CollectiblesHUD.WB_CollectiblesHUD_C|GetRefugeeCateTracker (Variables|/Game/Blueprints/Player/BP_Player.BP_Player_C|GetCollectiblesHUD _asbp_player)) (Utilities|Text|FormatText "Refugee Cates: {X}/{Y}" _output_get (Variables|/Game/GameModes/PlatformingGameMode.PlatformingGameMode_C|GetTotalRefugeeCates _asplatforming_game_mode)))
          (UserInterface|Animation|PlayAnimation (Variables|/Game/Blueprints/Player/BP_Player.BP_Player_C|GetCollectiblesHUD _asbp_player) (Variables|/Game/UI/Widgets/HUD/WB_CollectiblesHUD.WB_CollectiblesHUD_C|GetRefugeeCateUpdate (Variables|/Game/Blueprints/Player/BP_Player.BP_Player_C|GetCollectiblesHUD _asbp_player)) 0.0 1 "Forward" 1.0 true)
          (Class|Collectibles|UpdateRescuedCateCount(Message) (Game|GetGameMode)))))))

(fn ConstructionScript
  (|CallParentFunction))

(fn Interact
  (CallFunction|Talk)
  (return false))