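; NPC for a rescued refugee whose house the player can upgrade through dialogue.
; On BeginPlay it looks up its codex entry in game instance data, then sets the linked house actor's level, or destroys itself and the house if none is found.
; Talking opens an upgrade widget until the house reaches max level, then falls back to parent dialogue.
; The widget's exit event updates the house and HUD on purchase, then restores player control.
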(event Custom|CustomEvent
  (params (Bought :type Boolean))
  (bind _returnvalue (Game|GetPlayerController 0))
  (bind _houseactor (Variables|Default|GetHouseActor))
  (if Bought
    (bind _result (Math|Integer|IncrementInt (Variables|Default|GetHouselevelHouse))
      (:%20%20
        (Variables|/Game/Blueprints/Hub/CateHouse.CateHouse_C|SetHouseLevel _houseactor _result)
        (Default|UpdateHouse _houseactor)
        (bind _asbp_player (Utilities|Casting|CastToBP_Player (Game|Player|GetPlayerPawn 0))
          (:then
            (Default|UpdateGoldfly (Variables|/Game/Blueprints/Player/BP_Player.BP_Player_C|GetHUD _asbp_player)))
          (:CastFailed
            _))))
    (else
      (Variables|/Script/UMG.TextBlock|SetText (Variables|/Game/UI/Widgets/CUIWB_HouseUpgrade.CUIWB_HouseUpgrade_C|GetDialogueText (Variables|Default|GetHouse)) "Aww, man. Well, come back some other time!")
      (Utilities|FlowControl|Delay 2.0)))
  (CallFunction|TalkDone)
  (EventDispatchers|UnbindallEventsfromExit (stale EventTalk _returnvalue_2))
  (Widget|RemovefromParent (Variables|Default|GetHouse))
  (Utilities|Platform|CollectGarbage)
  (Variables|Default|SetHouse 0)
  (Variables|/Script/Engine.PlayerController|SetbShowMouseCursor _returnvalue false)
  (Input|SetInputModeGameOnly _returnvalue false)
  (Pawn|Components|CharacterMovement|SetMovementMode (Variables|/Script/Engine.Character|GetCharacterMovement (Game|GetPlayerCharacter 0)) "MOVE_Walking" 0))

(event EventBeginPlay
  (bind _houseactor (Variables|Default|GetHouseActor))
  (bind _codexthatunlocksme (Variables|Default|GetCodexThatUnlocksMe))
  (Variables|Default|SetName (Variables|/Game/UI/Blueprints/BP_CodexEntry.BP_CodexEntry_C|GetCodexHeader (Variables|Default|GetCodexThatUnlocksMe)))
  (bind _savegamedata (Class|BPISaveGameInterface|GetGameData(Message) (Game|GetGameInstance)))
  (if (!= (Utilities|Array|FindItem (Variables|/Game/Blueprints/Saving/BP_SaveGame.BP_SaveGame_C|GetCodexEntries%20-%20Levels _savegamedata) _codexthatunlocksme) -1)
    (bind _asrefugee_cate (Utilities|Casting|CastToRefugeeCate (Utilities|Array|Get(acopy) (Variables|/Game/Blueprints/Saving/BP_SaveGame.BP_SaveGame_C|GetCodexEntries%20-%20Levels _savegamedata)))
      (:then
        (Variables|Default|SetHouselevelHouse (Variables|/Game/Maps/CodexEntries/RefugeeCates/RefugeeCate.RefugeeCate_C|GetHouseLevel _asrefugee_cate))
        (Utilities|IsValid _houseactor :!label _label
          (:Is%20Valid
            (Variables|/Game/Blueprints/Hub/CateHouse.CateHouse_C|SetHouseLevel _houseactor (Math|Integer|Clamp(Integer) (Variables|Default|GetHouselevelHouse) 0 2))
            (Default|SetHouse _houseactor)
            (CallFunction|SetupUI)
            (Variables|Default|SetState "NewEnumerator2"))
          (:Is%20Not%20Valid
            (Actor|DestroyActor :!label _label_2))))
      (:CastFailed
        (Utilities|IsValid _houseactor :!label _label_3
          (:Is%20Valid
            (Actor|DestroyActor _houseactor)
            (goto _label_2))
          (:Is%20Not%20Valid
            (goto _label_2)))))
    (elif (!= (Utilities|Array|FindItem (Variables|/Game/Blueprints/Saving/BP_SaveGame.BP_SaveGame_C|GetCodexEntries%20-%20Cates _savegamedata) _codexthatunlocksme) -1)
      (bind _asrefugee_cate_2 (Utilities|Casting|CastToRefugeeCate (Utilities|Array|Get(acopy) (Variables|/Game/Blueprints/Saving/BP_SaveGame.BP_SaveGame_C|GetCodexEntries%20-%20Cates _savegamedata) (Utilities|Array|FindItem (Variables|/Game/Blueprints/Saving/BP_SaveGame.BP_SaveGame_C|GetCodexEntries%20-%20Cates _savegamedata) _codexthatunlocksme)))
        (:then
          (Variables|Default|SetHouselevelHouse (Variables|/Game/Maps/CodexEntries/RefugeeCates/RefugeeCate.RefugeeCate_C|GetHouseLevel _asrefugee_cate_2))
          (goto _label))
        (:CastFailed
          (goto _label_3)))
      (else
        (goto _label_3)))))

(event Collision|EventActorBeginOverlap
  (params (OtherActor :type Actor%20Object%20Reference))
  (|CallParentFunction OtherActor) ; This node is disabled and will not be called.\nDrag off pins to build functionality.
)

(event EventTick
  (params (DeltaSeconds :type Float%20%28single-precision%29))
  (|CallParentFunction DeltaSeconds) ; This node is disabled and will not be called.\nDrag off pins to build functionality.
)

(event EventTalk
  (bind _returnvalue (Game|GetPlayerController 0))
  (Input|SetInputModeUIOnly _returnvalue (Variables|Default|GetHouse) "DoNotLock" false)
  (if (>= (Variables|Default|GetHouselevelHouse) 3)
    (Input|SetInputModeGameandUI _returnvalue (Variables|Default|GetHouse) "DoNotLock" true false)
    (|CallParentFunction)
    (else
      (Variables|/Script/Engine.PlayerController|SetbShowMouseCursor _returnvalue true)
      (Pawn|Components|CharacterMovement|DisableMovement (Variables|/Script/Engine.Character|GetCharacterMovement (Game|GetPlayerCharacter 0)))
      (bind _returnvalue_2 (UserInterface|CreateWidget "/Game/UI/Widgets/CUIWB_HouseUpgrade.CUIWB_HouseUpgrade_C"))
      (bind _output_get (Variables|Default|SetHouse _returnvalue_2))
      (Variables|/Script/UMG.TextBlock|SetText (Variables|/Game/UI/Widgets/CUIWB_HouseUpgrade.CUIWB_HouseUpgrade_C|GetName_1 _returnvalue_2) (Variables|Default|GetName))
      (Variables|/Game/UI/Widgets/CUIWB_HouseUpgrade.CUIWB_HouseUpgrade_C|SetCateToRepresent _output_get (Variables|Default|GetCodexThatUnlocksMe))
      (Default|SetDialogue _output_get (Variables|Default|GetHouselevelHouse))
      (UserInterface|Viewport|AddtoViewport _output_get 0)
      (EventDispatchers|BindEventtoExit _returnvalue_2 (delegate Custom|CustomEvent))
      (Variables|/Script/Engine.PlayerController|SetbShowMouseCursor (Game|GetPlayerController 0) true)
      (Widget|RemovefromParent (Variables|Default|GetDialogue%20Prompt%20UI)))))

(fn ConstructionScript
  (|CallParentFunction))