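; BP_WardrobeCate is an NPC Blueprint that shows a talk prompt while the player overlaps its DialogueTrigger.
; BeginPlay creates the dialogue and prompt widgets and sets the NPC's name.
; Interact calls Talk, which is empty here; the click-through dialogue logic that halts movement and the happy-dance montage are disconnected.
; TalkDone restores the pickup input context and re-shows the prompt if the player remains in range.
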(event OnComponentBeginOverlap(DialogueTrigger)
  (params (OverlappedComponent :type Primitive%20Component%20Object%20Reference) (OtherActor :type Actor%20Object%20Reference) (OtherComp :type Primitive%20Component%20Object%20Reference) (OtherBodyIndex :type Integer) (bFromSweep :type Boolean) (SweepResult :type Hit%20Result%20Structure%20%28by%20ref%29))
  ;[1 1 1] Shows and Removes "Talk to NPC" UI Prompt on Enter and Exit Overlap with the NPC - Ryan
  (if (== (Utilities|GetClass OtherActor) "/Game/Blueprints/Player/BP_Player.BP_Player_C")
    (UserInterface|Viewport|AddtoViewport (Variables|Default|GetDialogue%20Prompt%20UI) 0)))

(event OnComponentEndOverlap(DialogueTrigger)
  (params (OverlappedComponent :type Primitive%20Component%20Object%20Reference) (OtherActor :type Actor%20Object%20Reference) (OtherComp :type Primitive%20Component%20Object%20Reference) (OtherBodyIndex :type Integer))
  ;[1 1 1] Shows and Removes "Talk to NPC" UI Prompt on Enter and Exit Overlap with the NPC - Ryan
  (if (== (Utilities|GetClass OtherActor) "/Game/Blueprints/Player/BP_Player.BP_Player_C")
    (Widget|RemovefromParent (Variables|Default|GetDialogue%20Prompt%20UI))))

(event Custom|SetupUI
  ;[1 1 1] Creating Dialogue UI Widget on Begin Play - Ryan
  (bind _returnvalue (UserInterface|CreateWidget "/Game/UI/Widgets/Menus/WB_Dialogue.WB_Dialogue_C" (Game|GetPlayerController 0)))
  (bind _output_get (Variables|Default|SetDialogue%20UI _returnvalue))
  (Variables|/Script/UMG.TextBlock|SetText (Variables|/Game/UI/Widgets/Menus/WB_Dialogue.WB_Dialogue_C|GetName _output_get) (Variables|Default|GetName))
  (bind _returnvalue_2 (UserInterface|CreateWidget "/Game/UI/Widgets/Menus/WB_DialoguePrompt.WB_DialoguePrompt_C"))
  (Variables|Default|SetDialogue%20Prompt%20UI _returnvalue_2))

(event Custom|TalkDone
  (Input|AddMappingContext (Game|GetPlayerController 0) "/Game/Inputs/InputActions/IMC_Pickups.IMC_Pickups" 0 "(bIgnoreAllPressedKeysUntilRelease=True,bForceImmediately=False,bNotifyUserSettings=False)")
  (if (Collision|IsOverlappingActor (Variables|Default|GetDialogue%20Trigger) (Game|Player|GetPlayerPawn 0) :!class /Script/Engine.PrimitiveComponent)
    (UserInterface|Viewport|AddtoViewport (Variables|Default|GetDialogue%20Prompt%20UI) 0)))

(event EventBeginPlay
  (CallFunction|SetupUI))

(event Collision|EventActorBeginOverlap
  (params (OtherActor :type Actor%20Object%20Reference)))

(event EventTick
  (params (DeltaSeconds :type Float%20%28single-precision%29)))

(event EventTalk
  ;[1 1 1] NPC Dialogue. If the player is in range, they can interact with an NPC to click through their dialogue. Movement is halted while talking to the NPC. They can talk to the NPC as many times as they want - Ryan
)

(fn ConstructionScript)

(fn Interact
  (CallFunction|Talk)
  (return false))