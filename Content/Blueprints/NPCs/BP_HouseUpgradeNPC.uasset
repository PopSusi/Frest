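; BP_HouseUpgradeNPC is a talkable hub cate that only appears, with its house, once its codex entry is in the game data, and offers upgrades to that house.
; BeginPlay sets the house from the entry's HouseLevel, or destroys both NPC and house.
; Below level 3, Talk locks movement and opens CUIWB_HouseUpgrade; otherwise it uses parent dialogue.
; The widget's exit event upgrades the house if bought, then restores control.
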(event Custom|FinishedTalking
  (params (Bought :type Boolean))
  (bind _returnvalue (Game|GetPlayerController 0))
  (bind _houseactor (Variables|Default|GetHouseActor))
  ;[1 1 1] If the player upgraded the house, upgrade the house. If not, exit the conversation - Ryan
  (if Bought
    (bind _result (Math|Integer|IncrementInt (Variables|Default|GetHouselevelHouse))
      (:%20%20
        (Variables|/Game/Blueprints/Hub/BP_CateHouse.BP_CateHouse_C|SetHouseLevel _houseactor _result)
        (Default|UpdateHouse _houseactor)
        (bind _asbp_player (Utilities|Casting|CastToBP_Player (Game|Player|GetPlayerPawn 0))
          (:then
            (Default|UpdateGoldfly (Variables|/Game/Blueprints/Player/BP_Player.BP_Player_C|GetHUD _asbp_player)))
          (:CastFailed
            _)))))
  (CallFunction|TalkDone)
  (EventDispatchers|UnbindallEventsfromExit (stale EventTalk _returnvalue_2))
  (Widget|RemovefromParent (Variables|Default|GetHouse))
  (Utilities|Platform|CollectGarbage)
  (Variables|Default|SetHouse 0)
  (Variables|/Script/Engine.PlayerController|SetbShowMouseCursor _returnvalue false)
  (Input|SetInputModeGameOnly _returnvalue true)
  (Pawn|Components|CharacterMovement|SetMovementMode (Variables|/Script/Engine.Character|GetCharacterMovement (Game|GetPlayerCharacter 0)) "MOVE_Walking" 0))

(event EventBeginPlay
  (bind _houseactor (Variables|Default|GetHouseActor))
  ;[1 1 1] If this cate has been rescued, they will appear in the hub with a house based on its current upgrade progress - Ryan
  (|CallParentFunction)
  (Variables|Default|SetName (Variables|/Game/UI/Blueprints/BP_CodexEntry.BP_CodexEntry_C|GetCodexHeader (Variables|Default|GetCodexThatUnlocksMe)))
  (bind _savegamedata (Class|BPISaveGameInterface|GetGameData(Message) (Game|GetGameInstance)))
  (if (Utilities|Array|ContainsItem (Variables|/Game/Blueprints/Saving/BP_SaveGame.BP_SaveGame_C|GetCodexEntries%20-%20Cates _savegamedata) (Variables|Default|GetCodexThatUnlocksMe))
    (Variables|Default|SetHouselevelHouse (Variables|/Game/Maps/CodexEntries/RefugeeCates/RefugeeCate.RefugeeCate_C|GetHouseLevel (Variables|Default|GetCodexThatUnlocksMe)))
    (Utilities|IsValid _houseactor
      (:Is%20Valid
        (Variables|/Game/Blueprints/Hub/BP_CateHouse.BP_CateHouse_C|SetHouseLevel _houseactor (Math|Integer|Clamp(Integer) (Variables|Default|GetHouselevelHouse) 0 3))
        (Default|SetHouse _houseactor)))
    (else
      (Actor|DestroyActor)
      (Actor|DestroyActor (Variables|Default|GetHouseActor)))))

(event Collision|EventActorBeginOverlap
  (params (OtherActor :type Actor%20Object%20Reference))
  (|CallParentFunction OtherActor) ; This node is disabled and will not be called.\nDrag off pins to build functionality.
)

(event EventTick
  (params (DeltaSeconds :type Float%20%28single-precision%29))
  (|CallParentFunction DeltaSeconds) ; This node is disabled and will not be called.\nDrag off pins to build functionality.
)

(event EventTalk
  (bind _returnvalue (Game|GetPlayerController 0))
  ;[1 1 1] If House is fully upgraded, just talk normally - Ryan
  (if (>= (Variables|Default|GetHouselevelHouse) 3)
    (|CallParentFunction)
    (Audio|PlaySound2D "/Game/Sounds/SFX/meow.meow" 1.0 1.0 0.0 0 0)
    (else
      ;[1 1 1] If not fully upgraded house, gives player the option to upgrade this cate's house. They can accept or deny - Ryan
      (Input|SetInputModeUIOnly _returnvalue (Variables|Default|GetHouse) "DoNotLock" true)
      (Variables|/Script/Engine.PlayerController|SetbShowMouseCursor _returnvalue true)
      (Pawn|Components|CharacterMovement|DisableMovement (Variables|/Script/Engine.Character|GetCharacterMovement (Game|GetPlayerCharacter 0)))
      (bind _returnvalue_2 (UserInterface|CreateWidget "/Game/UI/Widgets/CUIWB_HouseUpgrade.CUIWB_HouseUpgrade_C"))
      (bind _output_get (Variables|Default|SetHouse _returnvalue_2))
      (Variables|/Script/UMG.TextBlock|SetText (Variables|/Game/UI/Widgets/CUIWB_HouseUpgrade.CUIWB_HouseUpgrade_C|GetName_1 _returnvalue_2) (Variables|Default|GetName))
      (Variables|/Game/UI/Widgets/CUIWB_HouseUpgrade.CUIWB_HouseUpgrade_C|SetCateToRepresent _output_get (Variables|Default|GetCodexThatUnlocksMe))
      (Default|SetDialogue _output_get (Variables|Default|GetHouselevelHouse))
      (UserInterface|Viewport|AddtoViewport _output_get 0)
      (EventDispatchers|BindEventtoExit _returnvalue_2 (delegate Custom|FinishedTalking))
      (Variables|/Script/Engine.PlayerController|SetbShowMouseCursor (Game|GetPlayerController 0) true)
      (Rendering|SetVisibility (Variables|Default|GetWidget) true false)
      (Audio|PlaySound2D "/Game/Sounds/SFX/meow.meow" 1.0 1.0 0.0 0 0))))

(fn ConstructionScript
  (|CallParentFunction))