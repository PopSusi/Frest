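; BP_CodexNPC is an NPC whose dialogue unlocks a Codex entry for the player.
; It extends the parent Talk event, always running the parent dialogue first.
; Once FirstTalkComplete is set, it sets CodexUnlocked and calls Unlock on CodexToUnlock, with the flag preventing repeat unlocks on later conversations.
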(event EventBeginPlay
  (|CallParentFunction) ; This node is disabled and will not be called.\nDrag off pins to build functionality.
)

(event Collision|EventActorBeginOverlap
  (params (OtherActor :type Actor%20Object%20Reference))
  (|CallParentFunction OtherActor) ; This node is disabled and will not be called.\nDrag off pins to build functionality.
)

(event EventTick
  (params (DeltaSeconds :type Float%20%28single-precision%29))
  (|CallParentFunction DeltaSeconds) ; This node is disabled and will not be called.\nDrag off pins to build functionality.
)

(event EventTalk
  ;[1 1 1] When Talking to an NPC that unlocks a Codex Entry, it will unlock once dialogue with the NPC has been completed once - Ryan
  (if (Variables|Default|GetCodexUnlocked)
    (|CallParentFunction)
    (else
      (|CallParentFunction)
      (if (Variables|Default|GetFirstTalkComplete)
        (Variables|Default|SetCodexUnlocked true)
        (Default|Unlock (Variables|Default|GetCodexToUnlock))))))

(fn ConstructionScript
  (|CallParentFunction))