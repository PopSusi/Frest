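; BP_SubHubNPC is a rescued Cate NPC that opens the path to a sub hub.
; On BeginPlay it destroys itself unless its unlocking codex entry is saved, and removes its Block if the path's codex entry is saved too.
; Talk, called by Interact, plays a meow and parent dialogue; once FirstTalkComplete, it plays the unblock sequence and saves the world-block codex.
; After that, it only shows a fixed dismissive line.
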(event EventBeginPlay
  ;[1 1 1] Once a Cate has been rescued, functions like a normal NPC - Ryan
  (bind _savegamedata (Class|BPISaveGameInterface|GetGameData(Message) (Game|GetGameInstance)))
  (if (Utilities|Array|ContainsItem (Variables|/Game/Blueprints/Saving/BP_SaveGame.BP_SaveGame_C|GetCodexEntries%20-%20Levels _savegamedata) (Variables|Default|GetCodexThatUnlocksMe))
    (Variables|Default|SetName (Utilities|Text|ToText(Name) (Variables|/Game/UI/Blueprints/BP_CodexEntry.BP_CodexEntry_C|GetCodexHeader (Variables|Default|GetWorldBlockCodex))))
    (CallFunction|SetupUI)
    (if (Utilities|Array|ContainsItem (Variables|/Game/Blueprints/Saving/BP_SaveGame.BP_SaveGame_C|GetCodexEntries%20-%20WorldBlocks _savegamedata) (Variables|Default|GetWorldBlockCodex))
      (Actor|DestroyActor (Variables|Default|GetBlock)))
    (else
      (Actor|DestroyActor))))

(event Collision|EventActorBeginOverlap
  (params (OtherActor :type Actor%20Object%20Reference))
  (|CallParentFunction OtherActor) ; This node is disabled and will not be called.\nDrag off pins to build functionality.
)

(event EventTick
  (params (DeltaSeconds :type Float%20%28single-precision%29))
  (|CallParentFunction DeltaSeconds) ; This node is disabled and will not be called.\nDrag off pins to build functionality.
)

(event EventTalk
  ;[1 1 1] Determines if the Cate needs to open the path to a sub hub or not - Ryan
  (bind _savegamedata (Class|BPISaveGameInterface|GetGameData(Message) (Game|GetGameInstance)))
  (if (Utilities|Array|ContainsItem (Variables|/Game/Blueprints/Saving/BP_SaveGame.BP_SaveGame_C|GetCodexEntries%20-%20WorldBlocks _savegamedata) (Variables|Default|GetWorldBlockCodex))
    (Variables|Default|SetDialogue (Utilities|Array|MakeArray "Don't talk to me"))
    (Audio|PlaySound2D "/Game/Sounds/SFX/meow.meow" 1.0 1.0 0.0 0 0)
    (|CallParentFunction)
    (Widget|SetVisibility (Variables|Default|GetDialogue%20UI) "Visible")
    (else
      (Audio|PlaySound2D "/Game/Sounds/SFX/meow.meow" 1.0 1.0 0.0 0 0)
      (|CallParentFunction)
      (if (Variables|Default|GetFirstTalkComplete)
        (Sequencer|Player|Play (Variables|/Script/LevelSequence.LevelSequenceActor|GetSequencePlayer (Variables|Default|GetUnblockSequence)) :!class /Script/MovieScene.MovieSceneSequencePlayer)
        (Widget|SetVisibility (Variables|Default|GetDialogue%20UI) "Collapsed")
        (bind _asbp_game_instance (Utilities|Casting|CastToBP_GameInstance (Game|GetGameInstance)))
        (Default|SaveAnyCodex _asbp_game_instance (Variables|Default|GetWorldBlockCodex))))))

(fn ConstructionScript
  (|CallParentFunction))

(fn Interact
  (CallFunction|Talk)
  (return false))