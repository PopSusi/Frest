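; One-shot trigger that starts a dialogue with the Ben NPC when the player enters its box, and destroys itself on BeginPlay if that dialogue is already saved as completed.
; The first overlap calls Talk, flags the player as Talking and blends the camera to the player's BenActor.
; EndDialogue saves the dialogue name through the GameInstance and blends back to the pawn, with input disabled during both blends.
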(event OnComponentBeginOverlap(Box)
  (params (OverlappedComponent :type Primitive%20Component%20Object%20Reference) (OtherActor :type Actor%20Object%20Reference) (OtherComp :type Primitive%20Component%20Object%20Reference) (OtherBodyIndex :type Integer) (bFromSweep :type Boolean) (SweepResult :type Hit%20Result%20Structure%20%28by%20ref%29))
  (bind _returnvalue (Game|GetPlayerController 0))
  (bind _asbp_player (Utilities|Casting|CastToBP_Player OtherActor))
  (Utilities|FlowControl|DoOnce false
    (:Completed
      (CallFunction|Talk)
      (Variables|/Game/Blueprints/Player/BP_Player.BP_Player_C|SetTalking _asbp_player true)
      (Input|DisableInput _asbp_player _returnvalue)
      (Game|Player|SetViewTargetwithBlend _returnvalue (Variables|/Game/Blueprints/Player/BP_Player.BP_Player_C|GetBenActor _asbp_player) 1.0 "VTBlend_EaseOut" 0.5 true)
      (Utilities|FlowControl|Delay 1.0)
      (Input|EnableInput _asbp_player _returnvalue))))

(event EventBeginPlay
  (|CallParentFunction)
  (bind _savegamedata (Class|BPISaveGameInterface|GetGameData(Message) (Game|GetGameInstance)))
  (if (Utilities|Array|ContainsItem (Variables|/Game/Blueprints/Saving/BP_SaveGame.BP_SaveGame_C|GetBenDialoguesCompleted _savegamedata) (Variables|Default|GetDialogueName))
    (Actor|DestroyActor)))

(event Collision|EventActorBeginOverlap
  (params (OtherActor :type Actor%20Object%20Reference))
  (|CallParentFunction OtherActor) ; This node is disabled and will not be called.\nDrag off pins to build functionality.
)

(event EventTick
  (params (DeltaSeconds :type Float%20%28single-precision%29))
  (|CallParentFunction DeltaSeconds) ; This node is disabled and will not be called.\nDrag off pins to build functionality.
)

(event EventEndDialogue
  (bind _returnvalue (Game|Player|GetPlayerPawn 0))
  (bind _returnvalue_2 (Game|GetPlayerController 0))
  (Input|DisableInput (stale OnComponentBeginOverlap(Box) _asbp_player) _returnvalue_2)
  (Class|BPISaveGameInterface|SaveBenDialogue(Message) (Game|GetGameInstance) (Variables|Default|GetDialogueName))
  (bind _asbp_player (Utilities|Casting|CastToBP_Player _returnvalue))
  (Variables|/Game/Blueprints/Player/BP_Player.BP_Player_C|SetTalking _asbp_player false)
  (Game|Player|SetViewTargetwithBlend (Game|GetPlayerController 0) _returnvalue 1.0 "VTBlend_EaseInOut" 0.0 false)
  (Utilities|FlowControl|Delay 1.0)
  (Input|EnableInput (stale OnComponentBeginOverlap(Box) _asbp_player) _returnvalue_2))

(fn ConstructionScript
  (|CallParentFunction))