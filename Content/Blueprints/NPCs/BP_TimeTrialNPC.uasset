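; Sidequest NPC that starts a time trial once the player finishes talking to it.
; On BeginPlay it destroys itself unless the game instance's data contains its unlocking codex entry, which marks the level as beaten.
; Interact runs the parent's Talk until the conversation ends, then adds a WB_Timer widget set to the NPC's minutes and seconds.
; It then disables dialogue trigger collision and flags the trial active, blocking further talk.
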(event EventBeginPlay
  ;[1 1 1] Sidequest NPC only appears if the level has been beaten - Ryan
  (bind _savegamedata (Class|BPISaveGameInterface|GetGameData(Message) (Game|GetGameInstance)))
  (if (Utilities|Array|ContainsItem (Variables|/Game/Blueprints/Saving/BP_SaveGame.BP_SaveGame_C|GetMasterCodexEntries%20-%20Levels _savegamedata) (Variables|Default|GetCodexThatUnlocksMe))
    (|CallParentFunction)
    (else
      (Actor|DestroyActor))))

(event Collision|EventActorBeginOverlap
  (params (OtherActor :type Actor%20Object%20Reference))
  (|CallParentFunction OtherActor) ; This node is disabled and will not be called.\nDrag off pins to build functionality.
)

(event EventTick
  (params (DeltaSeconds :type Float%20%28single-precision%29))
  (|CallParentFunction DeltaSeconds) ; This node is disabled and will not be called.\nDrag off pins to build functionality.
)

(event EventTalk
  ;[1 1 1] After talking to this NPC, the time trial will start - Ryan
  (|CallParentFunction)
  (if (Variables|Default|GetEndOfConversation)
    (bind _returnvalue (UserInterface|CreateWidget "/Game/UI/Widgets/HUD/WB_Timer.WB_Timer_C"))
    (bind _output_get (Variables|Default|SetTimer%20Widget _returnvalue))
    (Variables|/Game/UI/Widgets/HUD/WB_Timer.WB_Timer_C|SetMinutes _output_get (Variables|Default|GetMinutes))
    (Variables|/Game/UI/Widgets/HUD/WB_Timer.WB_Timer_C|SetSeconds _output_get (Variables|Default|GetSeconds))
    (UserInterface|Viewport|AddtoViewport _output_get 0)
    (Variables|Default|SetEndOfConversation false)
    (Collision|SetCollisionEnabled (Variables|Default|GetDialogue%20Trigger) "NoCollision")
    (Variables|Default|SetTimeTrialActive true)))

(fn ConstructionScript
  (|CallParentFunction))

(fn Interact
  (if (not (Variables|Default|GetTimeTrialActive))
    (CallFunction|Talk)
    (return false)))