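; Tutorial dialogue actor for the NPC Ben, which halts the player and steps through an array of lines.
; BeginPlay creates the widget and arms a DoOnce only if the tutorial's codex entry is unsaved, so box overlap auto-starts the talk once.
; Interact advances lines; the last restores walking and saves the entry.
; MakeTextFromEnum turns button enums into inline rich-text icons, switching between gamepad and default glyphs by input device.
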(event OnComponentBeginOverlap(Box)
  (params (OverlappedComponent :type Primitive%20Component%20Object%20Reference) (OtherActor :type Actor%20Object%20Reference) (OtherComp :type Primitive%20Component%20Object%20Reference) (OtherBodyIndex :type Integer) (bFromSweep :type Boolean) (SweepResult :type Hit%20Result%20Structure%20%28by%20ref%29))
  (bind _asbp_player (Utilities|Casting|CastToBP_Player OtherActor))
  (Variables|Default|SetAs%20BP%20Player _asbp_player)
  (Utilities|FlowControl|DoOnce true
    (:Completed
      (Default|BenTalkto _asbp_player true)
      (CallFunction|Talk))))

(event Custom|ResetCam
  (Default|BenTalkto (Variables|Default|GetAs%20BP%20Player) false))

(event EventBeginPlay
  (bind _savegamedata (Class|BPISaveGameInterface|GetGameData(Message) (Game|GetGameInstance)))
  (if (not (Utilities|Array|ContainsItem (Variables|/Game/Blueprints/Saving/BP_SaveGame.BP_SaveGame_C|GetCodexEntries%20-%20Tutorials _savegamedata) (Variables|Default|GetTutorialEntry)))
    ;[1 1 1] Creating Dialogue UI Widget on Begin Play - Ryan
    (bind _returnvalue (UserInterface|CreateWidget "/Game/UI/Widgets/Menus/WB_BenDialogue.WB_BenDialogue_C" (Game|GetPlayerController 0)))
    (Default|CustomName _returnvalue "Ben" "/Game/Art/LevelScreens/LevelIcons/Benny.Benny")
    (Variables|Default|SetDialogue%20UI _returnvalue)
    (Utilities|FlowControl|DoOnce true) ; enters at Reset
  ))

(event Collision|EventActorBeginOverlap
  (params (OtherActor :type Actor%20Object%20Reference)))

(event EventTick
  (params (DeltaSeconds :type Float%20%28single-precision%29)))

(event EventTalk
  (bind _returnvalue (Game|GetPlayerCharacter 0))
  (bind _tutorialentry (Variables|Default|GetTutorialEntry))
  (bind _dialogue_ui (Variables|Default|GetDialogue%20UI))
  (bind _bendialogue (Variables|/Game/UI/Widgets/Menus/WB_BenDialogue.WB_BenDialogue_C|GetBenDialogue _dialogue_ui))
  ;[1 1 1] NPC Dialogue. If the player is in range, they can interact with an NPC to click through their dialogue. Movement is halted while talking to the NPC. They can talk to the NPC as many times as they want - Ryan
  (if (<= (Variables|Default|GetDialogue%20Index) (- (Utilities|Array|Length (Variables|Default|GetDialogue)) 1))
    (bind _asbp_player (Utilities|Casting|CastToBP_Player _returnvalue))
    (Variables|/Game/Blueprints/Player/BP_Player.BP_Player_C|SetIsTalking _asbp_player true)
    (if (== (Variables|Default|GetDialogue%20Index) 0)
      (UserInterface|Viewport|AddtoViewport (Variables|Default|GetDialogue%20UI) 0)
      (Class|NavMovementComponent|StopActiveMovement (Variables|/Script/Engine.Character|GetCharacterMovement _returnvalue)))
    (if (Utilities|Array|IsNotEmpty (.buttons (Utilities|Array|Get(acopy) (Variables|Default|GetDialogue) (Variables|Default|GetDialogue%20Index))))
      (bind _searchtext (CallFunction|MakeTextfromEnum (.buttons (Utilities|Array|Get(acopy) (Variables|Default|GetDialogue) (Variables|Default|GetDialogue%20Index)))))
      (Rendering|Components|TextRender|SetText _bendialogue (Utilities|Text|FormatText "{FirstText}{Buttonprompts}{SecondText}" (.textbeforebuttons (Utilities|Array|Get(acopy) (Variables|Default|GetDialogue) (Variables|Default|GetDialogue%20Index))) _searchtext (.textafterbuttons (Utilities|Array|Get(acopy) (Variables|Default|GetDialogue) (Variables|Default|GetDialogue%20Index)))))
      (else
        (Rendering|Components|TextRender|SetText _bendialogue (Utilities|Text|FormatText "{FirstText}{SecondText}" (.textbeforebuttons (Utilities|Array|Get(acopy) (Variables|Default|GetDialogue) (Variables|Default|GetDialogue%20Index))) (.textafterbuttons (Utilities|Array|Get(acopy) (Variables|Default|GetDialogue) (Variables|Default|GetDialogue%20Index)))))))
    (Math|Integer|IncrementInt (Variables|Default|GetDialogue%20Index))
    (else
      (Widget|RemovefromParent (Variables|Default|GetDialogue%20UI))
      (Pawn|Components|CharacterMovement|SetMovementMode (Variables|/Script/Engine.Character|GetCharacterMovement (Game|GetPlayerCharacter 0)) "MOVE_Walking" 0)
      (Variables|Default|SetDialogue%20Index 0)
      (if (Variables|Default|GetFirstTalkComplete)
        _
        (else
          (Variables|Default|SetFirstTalkComplete true)))
      (Variables|Default|SetEndOfConversation true)
      (Default|BenTalkto (Variables|Default|GetAs%20BP%20Player) false)
      (Utilities|IsValid _tutorialentry
        (:Is%20Valid
          (Class|BPISaveGameInterface|SaveTutorialCodex(Message) (Game|GetGameInstance) _tutorialentry))))))

(fn ConstructionScript)

(fn MakeTextfromEnum
  (params (Prompts :type Array%20of%20ButtonInputs%20Enums :default "NewEnumerator0"))
  (if (Utilities|Array|IsNotEmpty Prompts)
    (switch Utilities|FlowControl|Switch|SwitchonEHardwareDevicePrimaryType (.primarydevicetype (Class|InputDeviceSubsystem|GetInputDeviceHardwareIdentifier (|InputDeviceSubsystem)))
      (:Unspecified
        _)
      (:KeyboardAndMouse
        _)
      (:Gamepad
        (LocalVariables|SetControlType "Gamepad")
        (for _array_element Prompts
          (switch Utilities|FlowControl|Switch|SwitchonButtonInputs _array_element
            (:NewEnumerator0
              (LocalVariables|SetButton "Aim" :!label _label))
            (:NewEnumerator1
              (LocalVariables|SetButton "Look"))
            (:NewEnumerator2
              (LocalVariables|SetButton "Crouch"))
            (:NewEnumerator3
              (LocalVariables|SetButton "Jump"))
            (:NewEnumerator4
              (LocalVariables|SetButton "Grapple"))
            (:NewEnumerator5
              (goto _label))
            (:NewEnumerator6
              (LocalVariables|SetButton "Move"))
            (:NewEnumerator10
              (goto _label))
            (:NewEnumerator11
              (goto _label)))
          (LocalVariables|SetOutputText (Utilities|Text|FormatText "{ExistingOutput}{Addition}" (LocalVariables|GetOutputText) (Utilities|Text|FormatText "<img id=\"{SearchText}\" height=\"30\"/>" (Utilities|Text|FormatText "{Device}{Input}" (LocalVariables|GetControlType) (LocalVariables|GetButton))))))
        (return (LocalVariables|GetOutputText)))
      (:Touch
        _)
      (:MotionTracking
        _)
      (:RacingWheel
        _)
      (:FlightStick
        _)
      (:Camera
        _)
      (:Instrument
        _)
      (:CustomTypeA
        _)
      (:CustomTypeB
        _)
      (:CustomTypeC
        _)
      (:CustomTypeD
        _))
    (for _array_element_2 Prompts
      (switch Utilities|FlowControl|Switch|SwitchonButtonInputs _array_element_2
        (:NewEnumerator0
          (LocalVariables|SetButton "Talk"))
        (:NewEnumerator1
          (LocalVariables|SetButton "Look"))
        (:NewEnumerator2
          (LocalVariables|SetButton "Crouch"))
        (:NewEnumerator3
          (LocalVariables|SetButton "Jump"))
        (:NewEnumerator4
          (LocalVariables|SetButton "Grapple"))
        (:NewEnumerator5
          (LocalVariables|SetButton "Interact"))
        (:NewEnumerator6
          (LocalVariables|SetButton "MoveForward"))
        (:NewEnumerator7
          (LocalVariables|SetButton "MoveBack"))
        (:NewEnumerator8
          (LocalVariables|SetButton "MoveLeft"))
        (:NewEnumerator9
          (LocalVariables|SetButton "MoveRight")))
      (LocalVariables|SetOutputText (Utilities|Text|FormatText "{ExistingOutput}{Addition}" (LocalVariables|GetOutputText) (Utilities|Text|FormatText "<img id=\"{SearchText}\" height=\"30\"/>" (Utilities|Text|FormatText "{Device}{Input}" (LocalVariables|GetControlType) (LocalVariables|GetButton))))))
    (return (LocalVariables|GetOutputText))))

(fn Interact
  (CallFunction|Talk)
  (return false))