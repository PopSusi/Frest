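; Knight boss character that attaches its sword to its hand, damages the player on contact and stomps with a sphere trace or spawned shockwave.
; A looping timer drives a state enum, switching Idle to Whirlwind, while Rotating gates Tick's turn toward the player.
; Damage is limited by DoOnce until reset, and slow events freeze mesh animation.
; The distance and dodge-count attack selection is disconnected, and debug prints remain.
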(event OnComponentHit(CapsuleComponent)
  (params (HitComponent :type Primitive%20Component%20Object%20Reference) (OtherActor :type Actor%20Object%20Reference) (OtherComp :type Primitive%20Component%20Object%20Reference) (NormalImpulse :type Vector :default "0, 0, 0") (Hit :type Hit%20Result%20Structure%20%28by%20ref%29))
  (if (== OtherActor (Game|Player|GetPlayerPawn 0))
    (Game|Damage|ApplyDamage OtherActor 1.0 0 self)))

(event Custom|SelectAttack
  (bind _returnvalue (Game|Player|GetPlayerPawn 0))
  (bind _returnvalue_2 (Transformation|GetActorLocation))
  (bind _returnvalue_3 (Transformation|GetActorRotation))
  (bind _returnvalue_4 (Transformation|GetActorLocation _returnvalue))
  (bind _yaw (Math|Rotator|BreakRotator _returnvalue_3))
  (bind _returnvalue_5 (Math|Rotator|FindLookatRotation _returnvalue_2 _returnvalue_4))
  (bind _yaw_2 (Math|Rotator|BreakRotator _returnvalue_5))
  (switch Utilities|FlowControl|Switch|SwitchonEnum_KnightStates (Variables|Default|GetState)
    (:NewEnumerator0
      (Variables|Default|SetState "NewEnumerator4"))
    (:NewEnumerator5
      (if (and (> _yaw (- _yaw_2 5e+01)) (< _yaw (+ _yaw_2 5e+01)))
        (Variables|Default|SetState "NewEnumerator0")
        (Utilities|FlowControl|Gate true) ; enters at Close
        (else
          (Variables|Default|SetState "NewEnumerator5")
          (Utilities|FlowControl|Gate true) ; enters at Open
        )))))

(event Custom|EndAttack
  (Variables|Default|SetState "NewEnumerator0")
  (Variables|Default|SetAttackState "NewEnumerator3")
  (Utilities|FlowControl|Delay 8.0)
  (CallFunction|SelectAttack))

(event Custom|AttackHit
  (Variables|Default|SetAttacksDodged 0))

(event Custom|StopWhirlwind
  (Variables|Default|SetState "NewEnumerator0"))

(event Custom|SpawnHourglasses)

(event Custom|B_Stomp
  (bind _mesh (Variables|Character|GetMesh))
  (bind _returnvalue (Transformation|GetSocketLocation _mesh "JNT_Foot_Ball_RSocket"))
  (bind _outhits (Collision|MultiSphereTraceByChannel _returnvalue _returnvalue 2.5e+02 "TraceTypeQuery1" false (Utilities|Array|MakeArray self) "ForDuration"))
  (for _array_element _outhits
    (Game|Damage|ApplyDamage (.HitActor (Collision|BreakHitResult _array_element)) 1.0 0 self)))

(event Custom|F_Stomp
  (Game|SpawnActorfromClass "/Game/Blueprints/Mechanics/Boss3Stuff/BP_KnightShockwave.BP_KnightShockwave_C" (Math|Transform|MakeTransform (Transformation|GetSocketLocation (Variables|Character|GetMesh) "JNT_Foot_Ball_LSocket") "0, 0, 0" "1.000000,1.000000,1.000000") "Undefined" "MultiplyWithRoot" 0 0))

(event Custom|TakeDamage
  (Utilities|FlowControl|DoOnce false
    (:Completed
      (Variables|Default|SetAttackState "NewEnumerator3")
      (Variables|Default|SetState "NewEnumerator1")
      (bind _result (Math|Integer|DecrementInt (Variables|Default|GetHealth))
        (:%20%20
          (if (== _result 0)
            (bind _returnvalue (Actor|GetActorOfClass "/Game/Blueprints/Mechanics/Boss3Stuff/BP_KnightSword.BP_KnightSword_C"))
            (Actor|DestroyActor _returnvalue)
            (Actor|DestroyActor)
            (else
              (Development|PrintString "DAMAGED"))))))))

(event Custom|Reset%20To%20Idle
  (Variables|Default|SetState "NewEnumerator0")
  (Utilities|FlowControl|DoOnce false) ; enters at Reset
)

(event Custom|ResetDamage
  (Variables|Default|SetState "NewEnumerator0")
  (Utilities|FlowControl|DoOnce false) ; enters at Reset
)

(event EventBeginPlay
  (Utilities|Time|SetTimerbyEvent (delegate Custom|SelectAttack) 1.0 true)
  (bind _returnvalue (Actor|GetActorOfClass "/Game/Blueprints/Mechanics/Boss3Stuff/BP_KnightSword.BP_KnightSword_C"))
  (Collision|IgnoreActorwhenMoving (Variables|Collision|GetCapsuleComponent) _returnvalue true)
  (Transformation|AttachComponentToComponent _returnvalue (Variables|Character|GetMesh) "JNT_Socket_R_Hand" "SnapToTarget" "SnapToTarget" "SnapToTarget" true))

(event Collision|EventActorBeginOverlap
  (params (OtherActor :type Actor%20Object%20Reference)))

(event EventTick
  (params (DeltaSeconds :type Float%20%28single-precision%29))
  (Development|PrintString (Utilities|String|EnumtoString (Variables|Default|GetState)) true true "(R=0.000000,G=0.660000,B=1.000000,A=1.000000)" 0.0)
  (Utilities|FlowControl|Gate true
    (:Exit
      (Transformation|SetActorRotation (Math|Rotator|MakeRotator 0.0 0.0 (.yaw (Math|Interpolation|RInterpTo (Transformation|GetActorRotation) (Math|Rotator|FindLookatRotation (Transformation|GetActorLocation) (Transformation|GetActorLocation (Game|Player|GetPlayerPawn 0))) DeltaSeconds 8.0)))))))

(event EventStartSlow
  (Development|PrintString "!!!!!!!!!!!!!!!!!!!")
  (Components|Timeline|SetPlayRate (Variables|Character|GetMesh) 0.0))

(event EventBreakSlow
  (Components|Timeline|SetPlayRate (Variables|Character|GetMesh) 1.0))

(fn ConstructionScript)

(fn SlowStats
  (return 0.0 0.0))