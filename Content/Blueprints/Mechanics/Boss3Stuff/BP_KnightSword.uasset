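; BP_KnightSword is the sword of the Knight boss, which ignores movement collision with its parent actor shortly after spawning.
; When the player overlaps its box while slammable and in a specific movement state, it damages BP_Knight, spawns an impact effect and calls BreakSlowMessage.
; SpawnVFX plays a slash shockwave at the blade's tip socket.
; Ping reports ShouldDamage, while the sword's own player-damage logic is left unwired.
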(event OnComponentHit(StaticMesh)
  (params (HitComponent :type Primitive%20Component%20Object%20Reference) (OtherActor :type Actor%20Object%20Reference) (OtherComp :type Primitive%20Component%20Object%20Reference) (NormalImpulse :type Vector :default "0, 0, 0") (Hit :type Hit%20Result%20Structure%20%28by%20ref%29)))

(event OnComponentBeginOverlap(Box)
  (params (OverlappedComponent :type Primitive%20Component%20Object%20Reference) (OtherActor :type Actor%20Object%20Reference) (OtherComp :type Primitive%20Component%20Object%20Reference) (OtherBodyIndex :type Integer) (bFromSweep :type Boolean) (SweepResult :type Hit%20Result%20Structure%20%28by%20ref%29))
  (if (Variables|Default|GetCanBeSlammed)
    (if (== OtherActor (Game|Player|GetPlayerPawn 0))
      (bind _asbp_player (Utilities|Casting|CastToBP_Player OtherActor))
      (if (Utilities|Enum|Equal(Enum) (Variables|/Game/Blueprints/Player/BP_Player.BP_Player_C|GetMovementType _asbp_player) "NewEnumerator15")
        (bind _returnvalue (Actor|GetActorOfClass "/Game/Blueprints/Mechanics/Boss3Stuff/BP_Knight.BP_Knight_C"))
        (Default|TakeDamage _returnvalue)
        (Niagara|SpawnSystematLocation "/Game/Art/Jack_VFX/LightningFX/FX_NS_BossImpact.FX_NS_BossImpact" (Transformation|GetWorldLocation (Variables|Default|GetBox)))
        (bind _returnvalue_2 (Actor|GetActorOfClass "/Game/Blueprints/Mechanics/Boss3Stuff/BP_Knight.BP_Knight_C"))
        (Class|SlowDown|BreakSlow(Message) _returnvalue_2)))))

(event Custom|SpawnVFX
  (Niagara|SpawnSystematLocation "/Game/Art/Jack_VFX/BossFX/KnightBossFX/FX_SlashShockwave.FX_SlashShockwave" (Transformation|GetSocketLocation (Variables|Default|GetStaticMesh) "TipSocket")))

(event EventBeginPlay
  (Utilities|FlowControl|Delay 0.2)
  (Collision|IgnoreActorwhenMoving (Variables|Default|GetStaticMesh) (Actor|GetParentActor) true))

(event Collision|EventActorBeginOverlap
  (params (OtherActor :type Actor%20Object%20Reference)))

(event EventTick
  (params (DeltaSeconds :type Float%20%28single-precision%29)))

(fn ConstructionScript)

(fn Ping
  (return (Variables|Default|GetShouldDamage) false))