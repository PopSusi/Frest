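; Spawner actor for the knight boss fight (Boss 3) that delivers an hourglass time pickup along a path.
; SpawnHourglass reveals a static mesh and a timeline moves it along the spline by distance, with sweep enabled.
; When the timeline finishes, the mesh is hidden and a BP_TimePickUp actor spawns at its final location.
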(event Custom|SpawnHourglass
  (bind _staticmesh (Variables|Default|GetStaticMesh))
  (bind _spline (Variables|Default|GetSpline))
  (Development|SetHiddeninGame (Variables|Default|GetStaticMesh) false false)
  (bind _newtrack_0 (Timeline|Timeline PlayFromStart)
    (:Update
      (Transformation|SetWorldLocation _staticmesh (Spline|GetLocationatDistanceAlongSpline _spline (* _newtrack_0 (Spline|GetSplineLength _spline)) "World") true false))
    (:Finished
      (Development|SetHiddeninGame (Variables|Default|GetStaticMesh) true false)
      (Game|SpawnActorfromClass "/Game/Blueprints/Mechanics/Actor/BP_TimePickUp.BP_TimePickUp_C" (Math|Transform|MakeTransform (Transformation|GetWorldLocation _staticmesh) "0, 0, 0" "1.000000,1.000000,1.000000") "Undefined" "MultiplyWithRoot" 0 0))))

(event EventBeginPlay)

(event Collision|EventActorBeginOverlap
  (params (OtherActor :type Actor%20Object%20Reference)))

(event EventTick
  (params (DeltaSeconds :type Float%20%28single-precision%29)))

(fn ConstructionScript)