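; Time effect actor: a sphere that grows, lasts for a set duration, then shrinks and destroys itself.
; The Growth timeline scales the sphere, then plays in reverse with a Kill flag set so its finish destroys the actor.
; Overlap with a PostProcessCheck-tagged player component caches the camera's post-process settings and applies slowdown ones, restoring them on exit.
; The file changes only visuals, not time, and prints a debug "Hello" on every begin overlap.
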(event OnComponentBeginOverlap(Sphere)
  (params (OverlappedComponent :type Primitive%20Component%20Object%20Reference) (OtherActor :type Actor%20Object%20Reference) (OtherComp :type Primitive%20Component%20Object%20Reference) (OtherBodyIndex :type Integer) (bFromSweep :type Boolean) (SweepResult :type Hit%20Result%20Structure%20%28by%20ref%29))
  (Development|PrintString "Hello")
  (if (Components|ComponentHasTag OtherComp "PostProcessCheck")
    (bind _asbp_player (Utilities|Casting|CastToBP_Player OtherActor))
    (Variables|Default|SetDefault (Variables|/Script/Engine.CameraComponent|GetPostProcessSettings (Variables|/Game/Blueprints/Player/BP_Player.BP_Player_C|GetCamera _asbp_player)))
    (Variables|/Script/Engine.CameraComponent|SetPostProcessSettings (Variables|/Game/Blueprints/Player/BP_Player.BP_Player_C|GetCamera _asbp_player) (Variables|Default|GetSlowdown%20Post%20Processing))))

(event OnComponentEndOverlap(Sphere)
  (params (OverlappedComponent :type Primitive%20Component%20Object%20Reference) (OtherActor :type Actor%20Object%20Reference) (OtherComp :type Primitive%20Component%20Object%20Reference) (OtherBodyIndex :type Integer))
  (if (Components|ComponentHasTag OtherComp "PostProcessCheck")
    (bind _asbp_player (Utilities|Casting|CastToBP_Player OtherActor))
    (Variables|/Script/Engine.CameraComponent|SetPostProcessSettings (Variables|/Game/Blueprints/Player/BP_Player.BP_Player_C|GetCamera _asbp_player) (Variables|Default|GetDefault))))

(event Custom|Grow
  (bind _output_get (Variables|Default|SetTimeline%20start 0.02))
  (bind _scale (Timeline|Growth Play)
    (:Update
      (Transformation|SetWorldScale3D (Variables|Default|GetSphere) (Math|Vector|MakeVector (* _scale (Variables|Default|GetScale)) (* _scale (Variables|Default|GetScale)) (* _scale (Variables|Default|GetScale)))))
    (:Finished
      (if (Variables|Default|GetKill)
        (Actor|DestroyActor)))))

(event Custom|Shrink
  (Variables|Default|SetKill true)
  (bind _scale (Timeline|Growth ReverseFromEnd)
    (:Update
      (Transformation|SetWorldScale3D (Variables|Default|GetSphere) (Math|Vector|MakeVector (* _scale (Variables|Default|GetScale)) (* _scale (Variables|Default|GetScale)) (* _scale (Variables|Default|GetScale)))))
    (:Finished
      (if (Variables|Default|GetKill)
        (Actor|DestroyActor)))))

(event EventBeginPlay
  (CallFunction|Grow)
  (Utilities|FlowControl|Delay (Variables|Default|GetDuration))
  (CallFunction|Shrink))

(event Collision|EventActorBeginOverlap
  (params (OtherActor :type Actor%20Object%20Reference)))

(event EventTick
  (params (DeltaSeconds :type Float%20%28single-precision%29)))

(fn ConstructionScript)