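; Throwable time pod that the player carries and that slows the objects it lands near.
; PickBackUp attaches it to the player's PickupSocket with physics and collisions off, while Detach sets world state and re-enables both.
; A hit in world state runs a sphere trace ignoring the player, sends StartSlowMessage to hit actors and spawns BP_TimeEffect with a sound.
; The pod then plays a break sound and destroys itself, even if nothing was found.
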(event OnComponentHit(StaticMesh)
  (params (HitComponent :type Primitive%20Component%20Object%20Reference) (OtherActor :type Actor%20Object%20Reference) (OtherComp :type Primitive%20Component%20Object%20Reference) (NormalImpulse :type Vector :default "0, 0, 0") (Hit :type Hit%20Result%20Structure%20%28by%20ref%29))
  (bind _returnvalue (Transformation|GetActorLocation))
  (if (Variables|Default|GetWorldState)
    (bind (_outhits _returnvalue_2) (Collision|MultiSphereTraceForObjects _returnvalue _returnvalue 1e+02 (Variables|Default|GetObject%20Types) false (Utilities|Array|MakeArray (Game|Player|GetPlayerPawn 0)) "ForDuration"))
    (if _returnvalue_2
      (for _array_element _outhits
        (Class|SlowDown|StartSlow(Message) (.hitactor _array_element))
        ;[1 1 1] Effect and slow sound when hitting something
        (Game|SpawnActorfromClass "/Game/Blueprints/Mechanics/Actor/BP_TimeEffect.BP_TimeEffect_C" (Math|Transform|MakeTransform (Transformation|GetActorLocation) "0, 0, 0" "1.000000,1.000000,1.000000") "Undefined" "MultiplyWithRoot" 0 0)
        (Audio|PlaySound2D "/Game/Sounds/SFX/Gameplay/GoodJob.GoodJob" 1.0 1.0 0.0 0 0)
        (CallFunction|Break))
      (else
        (CallFunction|Break)))))

(event Custom|Break
  ;[1 1 1] Break Noise
  (Audio|PlaySoundatLocation "/Game/Sounds/SFX/Movement/DoubleJump2.DoubleJump2" (Transformation|GetActorLocation) "0, 0, 0" 1.0 1.0 0.0 0 0 0 0)
  (Actor|DestroyActor))

(event EventBeginPlay)

(event Collision|EventActorBeginOverlap
  (params (OtherActor :type Actor%20Object%20Reference)))

(event EventTick
  (params (DeltaSeconds :type Float%20%28single-precision%29)))

(fn ConstructionScript)

(fn Detach
  (Transformation|DetachFromActor self "KeepWorld" "KeepWorld" "KeepWorld")
  (Physics|SetSimulatePhysics (Variables|Default|GetStaticMesh) true)
  (Variables|Default|SetWorldState true)
  (CallFunction|ChangeCollisionSettings))

(fn ChangeCollisionSettings
  (if (Variables|Default|GetWorldState)
    ;[1 1 1] If in world state, collide
    (Collision|SetCollisionResponsetoChannel (Variables|Default|GetStaticMesh) "ECC_WorldStatic" "ECR_Block")
    (Collision|SetCollisionResponsetoChannel (Variables|Default|GetStaticMesh) "ECC_WorldDynamic" "ECR_Block")
    (Collision|SetCollisionResponsetoChannel (Variables|Default|GetStaticMesh) "ECC_PhysicsBody" "ECR_Block")
    (Collision|SetCollisionResponsetoChannel (Variables|Default|GetStaticMesh) "ECC_PhysicsBody" "ECR_Block")
    (else
      ;[1 1 1] If in Player state, ignore
      (Collision|SetCollisionResponsetoChannel (Variables|Default|GetStaticMesh) "ECC_WorldStatic" "ECR_Ignore")
      (Collision|SetCollisionResponsetoChannel (Variables|Default|GetStaticMesh) "ECC_WorldDynamic" "ECR_Ignore")
      (Collision|SetCollisionResponsetoChannel (Variables|Default|GetStaticMesh) "ECC_PhysicsBody" "ECR_Ignore")
      (Collision|SetCollisionResponsetoChannel (Variables|Default|GetStaticMesh) "ECC_Pawn" "ECR_Ignore"))))

(fn PickBackUp
  (params (Player :type BP%20Player%20Object%20Reference))
  (bind _mesh (Variables|/Script/Engine.Character|GetMesh Player))
  ;[1 1 1] Change goo pod to World instead of player, and adjust physics
  (Variables|Default|SetWorldState false)
  (Physics|SetSimulatePhysics (Variables|Default|GetStaticMesh) false)
  (CallFunction|ChangeCollisionSettings)
  ;[1 1 1] Move BP_Object to socket
  (Transformation|SetActorTransform (Transformation|GetSocketTransform _mesh "PickupSocket" "RTS_World") false true)
  ;[1 1 1] Attach
  (Transformation|AttachComponentToComponent _mesh "PickupSocket" "SnapToTarget" "SnapToTarget" "SnapToTarget" true))