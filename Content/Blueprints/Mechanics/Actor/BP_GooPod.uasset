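; BP_GooPod is a goo pod actor that players carry and release, bursting into GooArea actors when it hits something while Active.
; PickBackUp attaches it to the player's PickupSocket without physics, while Detach restores physics, with WorldState toggling Sphere collision responses.
; On hit, it spawns a large GooArea at impact, then sphere-traces nearby surfaces for smaller attached patches.
; Each patch receives the pod's Type as MovementMod before the pod destroys itself.
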(event OnComponentHit(Sphere)
  (params (HitComponent :type Primitive%20Component%20Object%20Reference) (OtherActor :type Actor%20Object%20Reference) (OtherComp :type Primitive%20Component%20Object%20Reference) (NormalImpulse :type Vector :default "0, 0, 0") (Hit :type Hit%20Result%20Structure%20%28by%20ref%29))
  (bind _sphere (Variables|Default|GetSphere))
  (bind _returnvalue (Transformation|GetWorldLocation _sphere))
  (if (Variables|Default|GetActive)
    (Audio|PlaySoundatLocation "/Game/Sounds/SFX/Movement/DoubleJump.DoubleJump" (.impactpoint Hit) "0, 0, 0" 1.0 1.0 0.0 0 0 0 0)
    (bind _returnvalue_2 (Game|SpawnActorfromClass "/Game/Blueprints/Mechanics/SpawnedActors/GooArea.GooArea_C" (Math|Transform|MakeTransform (.impactpoint Hit) (Math|Rotator|MakeRotfromZ (.impactnormal Hit)) "9.000000,9.000000,9.000000") "Undefined" "MultiplyWithRoot" 0 0))
    (Variables|/Game/Blueprints/Mechanics/SpawnedActors/GooArea.GooArea_C|SetMovementMod _returnvalue_2 (Variables|Default|GetType))
    (bind _outhits (Collision|MultiSphereTraceByChannel _returnvalue _returnvalue 5e+02 "TraceTypeQuery1" false 0 "None"))
    (for _array_element _outhits
      (bind _returnvalue_3 (Game|SpawnActorfromClass "/Game/Blueprints/Mechanics/SpawnedActors/GooArea.GooArea_C" (Math|Transform|MakeTransform (.impactpoint _array_element) (Math|Rotator|MakeRotfromX (.impactnormal _array_element)) "6.000000,6.000000,6.000000") "Undefined" "MultiplyWithRoot" 0 0))
      (Transformation|AttachActorToActor _returnvalue_3 (.hitactor _array_element) "None" "KeepWorld" "KeepWorld" "KeepWorld" true)
      (Variables|/Game/Blueprints/Mechanics/SpawnedActors/GooArea.GooArea_C|SetMovementMod _returnvalue_3 (Variables|Default|GetType)))
    (Actor|DestroyActor)))

(event EventBeginPlay)

(event Collision|EventActorBeginOverlap
  (params (OtherActor :type Actor%20Object%20Reference)))

(event EventTick
  (params (DeltaSeconds :type Float%20%28single-precision%29)))

(fn ConstructionScript)

(fn Detach
  (bind _self self)
  (Transformation|DetachFromActor _self "KeepWorld" "KeepWorld" "KeepWorld")
  (Physics|SetSimulatePhysics (Variables|Default|GetSphere _self) true)
  (Variables|Default|SetWorldState true)
  (CallFunction|ChangeCollisionSettings))

(fn ChangeCollisionSettings
  (if (Variables|Default|GetWorldState)
    ;[1 1 1] If in world state, collide
    (Collision|SetCollisionResponsetoChannel (Variables|Default|GetSphere) "ECC_WorldStatic" "ECR_Block")
    (Collision|SetCollisionResponsetoChannel (Variables|Default|GetSphere) "ECC_WorldDynamic" "ECR_Block")
    (Collision|SetCollisionResponsetoChannel (Variables|Default|GetSphere) "ECC_PhysicsBody" "ECR_Block")
    (Collision|SetCollisionResponsetoChannel (Variables|Default|GetSphere) "ECC_PhysicsBody" "ECR_Block")
    (else
      ;[1 1 1] If in Player state, ignore
      (Collision|SetCollisionResponsetoChannel (Variables|Default|GetSphere) "ECC_WorldStatic" "ECR_Ignore")
      (Collision|SetCollisionResponsetoChannel (Variables|Default|GetSphere) "ECC_WorldDynamic" "ECR_Ignore")
      (Collision|SetCollisionResponsetoChannel (Variables|Default|GetSphere) "ECC_PhysicsBody" "ECR_Ignore")
      (Collision|SetCollisionResponsetoChannel (Variables|Default|GetSphere) "ECC_PhysicsBody" "ECR_Ignore")
      (Development|PrintString "ignoring"))))

(fn PickBackUp
  (params (Player :type BP%20Player%20Object%20Reference))
  (bind _mesh (Variables|/Script/Engine.Character|GetMesh Player))
  ;[1 1 1] Change goo pod to World instead of player, and adjust physics
  (Variables|Default|SetWorldState false)
  (Physics|SetSimulatePhysics (Variables|Default|GetSphere) false)
  (CallFunction|ChangeCollisionSettings)
  ;[1 1 1] Move BP_GooPod to socket
  (Transformation|SetActorTransform (Transformation|GetSocketTransform _mesh "PickupSocket" "RTS_World"))
  ;[1 1 1] Attach
  (Transformation|AttachComponentToComponent _mesh "PickupSocket" "SnapToTarget" "SnapToTarget" "SnapToTarget" true))