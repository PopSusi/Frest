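; BP_GooPlant is an interactable plant whose pod the player can pick up and that regrows after a cooldown.
; A sphere overlap shows a prompt widget to the player while the plant is interactable.
; Pickup hides the pod, locks interaction and passes pod type and plant reference to the pickup component's AttachPlant.
; CooldownOver restores both and rechecks overlaps for the prompt; Reset clears the cooldown timer, which this file never starts, and calls it immediately.
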(event OnComponentBeginOverlap(Sphere)
  (params (OverlappedComponent :type Primitive%20Component%20Object%20Reference) (OtherActor :type Actor%20Object%20Reference) (OtherComp :type Primitive%20Component%20Object%20Reference) (OtherBodyIndex :type Integer) (bFromSweep :type Boolean) (SweepResult :type Hit%20Result%20Structure%20%28by%20ref%29))
  (if (and (== OtherActor (Game|Player|GetPlayerPawn 0)) (Variables|Default|GetInteractable))
    (Rendering|SetVisibility (Variables|Default|GetWidget) true false)))

(event OnComponentEndOverlap(Sphere)
  (params (OverlappedComponent :type Primitive%20Component%20Object%20Reference) (OtherActor :type Actor%20Object%20Reference) (OtherComp :type Primitive%20Component%20Object%20Reference) (OtherBodyIndex :type Integer))
  (if (== OtherActor (Game|Player|GetPlayerPawn 0))
    (Rendering|SetVisibility (Variables|Default|GetWidget) false true)))

(event EventBeginPlay
  (Rendering|SetVisibility (Variables|Default|GetWidget) false false))

(event Collision|EventActorBeginOverlap
  (params (OtherActor :type Actor%20Object%20Reference)))

(event EventTick
  (params (DeltaSeconds :type Float%20%28single-precision%29)))

(event EventReset
  (Utilities|Time|ClearandInvalidateTimerbyHandle (Variables|Default|GetCooldownTimer))
  (CallFunction|CooldownOver))

(fn ConstructionScript)

(fn Pickup
  (params (PickupComponentRef :type BPC%20Goo%20Pickup%20Object%20Reference))
  ;[1 1 1] Make sure plant isn't on cooldown
  (if (Variables|Default|GetInteractable)
    (Variables|Default|SetInteractable false)
    ;[1 1 1] Remove the Plant's Pod and call cooldown
    (Rendering|SetVisibility (Variables|Default|GetGooPlantPickup) false false)
    ;[1 1 1] Call on component to add mesh to player
    (Default|AttachPlant PickupComponentRef (Variables|Default|GetType) self)
    (Rendering|SetVisibility (Variables|Default|GetWidget) false false)
    (return true)
    (else
      (return false))))

(fn CooldownOver
  ;[1 1 1] Reset pod and interaction
  (Variables|Default|SetInteractable true)
  (Rendering|SetVisibility (Variables|Default|GetGooPlantPickup) true false)
  (bind _array_element (Utilities|Array|ForEachLoopwithBreak (Collision|GetOverlappingActors 0 :!class /Script/Engine.Actor) :!label _label)
    (:LoopBody
      (if (== (Game|Player|GetPlayerPawn 0) _array_element)
        (Rendering|SetVisibility (Variables|Default|GetWidget) true false)
        (goto _label Break)))))