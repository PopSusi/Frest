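; BP_TimePickUp is a plant pickup actor whose pod can be taken, then reappears after a cooldown.
; Pickup only succeeds while Interactable: it hides the mesh, starts a named-function timer, calls AttachSlow on the passed pickup component and returns whether it succeeded.
; CooldownOver restores visibility and interactability when the timer fires.
; The event graph is unused, so pickup relies on an external caller.
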(event EventBeginPlay)

(event Collision|EventActorBeginOverlap
  (params (OtherActor :type Actor%20Object%20Reference)))

(event EventTick
  (params (DeltaSeconds :type Float%20%28single-precision%29)))

(fn ConstructionScript)

(fn Pickup
  (params (PickUpComponent :type BPC%20Slow%20Object%20Reference))
  ;[1 1 1] Make sure plant isn't on cooldown
  (if (Variables|Default|GetInteractable)
    (Variables|Default|SetInteractable false)
    ;[1 1 1] Remove the Plant's Pod and call cooldown
    (Rendering|SetVisibility (Variables|Default|GetStaticMesh) false false)
    (Utilities|Time|SetTimerbyFunctionName 0 "CooldownOver" (Variables|Default|GetCooldownTime))
    ;[1 1 1] Call on component to add mesh to player
    (Default|AttachSlow PickUpComponent)
    (Development|PrintString "Attaching Plant")
    (return true)
    (else
      (return false))))

(fn CooldownOver
  (Variables|Default|SetInteractable true)
  (Rendering|SetVisibility (Variables|Default|GetStaticMesh) true false))