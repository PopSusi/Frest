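; Grapple point actor that shows a detection-node widget while activated and marks when the player is within grapple range.
; Activate stores the player and shows the widget; Deactivate hides it and is the starting state.
; While active, Tick maps player distance between detection radius and throw distance to grow the fill, turning it green within throw range.
; An inner sphere disables the main sphere's collision while the player is too close to grapple.
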(event OnComponentBeginOverlap(Sphere1)
  (params (OverlappedComponent :type Primitive%20Component%20Object%20Reference) (OtherActor :type Actor%20Object%20Reference) (OtherComp :type Primitive%20Component%20Object%20Reference) (OtherBodyIndex :type Integer) (bFromSweep :type Boolean) (SweepResult :type Hit%20Result%20Structure%20%28by%20ref%29))
  ;[1 1 1] Bounding Box for Level Designers that outlines when Player is too close to Grapple to the Grapple Point - Ryan
  (if (== OtherActor (Variables|Default|GetPlayer%20Ref))
    (Collision|SetCollisionEnabled (Variables|Default|GetSphere) "NoCollision")))

(event OnComponentEndOverlap(Sphere1)
  (params (OverlappedComponent :type Primitive%20Component%20Object%20Reference) (OtherActor :type Actor%20Object%20Reference) (OtherComp :type Primitive%20Component%20Object%20Reference) (OtherBodyIndex :type Integer))
  ;[1 1 1] Bounding Box for Level Designers that outlines when Player is too close to Grapple to the Grapple Point - Ryan
  (if (== OtherActor (Variables|Default|GetPlayer%20Ref))
    (Collision|SetCollisionEnabled (Variables|Default|GetSphere) "QueryAndPhysics")))

(event EventBeginPlay
  ;[1 1 1] Initializing all Grapple Point UI and Deactivating them - Ryan
  (bind _aswb_new_detection_node (Utilities|Casting|CastToWB_NewDetectionNode (UserInterface|GetUserWidgetObject (Variables|Default|GetWidget))))
  (Variables|Default|SetWidget%20Ref _aswb_new_detection_node)
  (CallFunction|Deactivate))

(event Collision|EventActorBeginOverlap
  (params (OtherActor :type Actor%20Object%20Reference)))

(event EventTick
  (params (DeltaSeconds :type Float%20%28single-precision%29))
  ;[1 1 1] Calculating Distance from Player to see if Grapple Point is in Range - Ryan
  (if (Variables|Default|GetIsActive)
    (CallFunction|CheckDistancefromPlayer)))

(fn ConstructionScript)

(fn Activate
  (params (Player%20Ref :type BP%20Player%20Object%20Reference))
  ;[1 1 1] Makes Grapple Point available to Grapple to - Ryan
  (Variables|Default|SetIsActive true)
  (Widget|SetVisibility (Variables|Default|GetWidget%20Ref) "Visible")
  (Variables|Default|SetPlayer%20Ref Player%20Ref))

(fn Deactivate
  ;[1 1 1] Deactivates Grapple Point making it unable to be Grappled to - Ryan
  (Variables|Default|SetIsActive false)
  (Widget|SetVisibility (Variables|Default|GetWidget%20Ref) "Hidden"))

(fn CheckDistancefromPlayer
  (bind _returnvalue (Transformation|GetActorLocation))
  (bind _player_ref (Variables|Default|GetPlayer%20Ref))
  (bind _player_ref_2 (Variables|Default|GetPlayer%20Ref))
  (bind _returnvalue_2 (Transformation|GetActorLocation _player_ref))
  (bind _grappledetectionradius (Variables|/Game/Blueprints/Player/BP_Player.BP_Player_C|GetGrappleDetectionRadius _player_ref_2))
  (bind _grapplethrowdistance (Variables|/Game/Blueprints/Player/BP_Player.BP_Player_C|GetGrappleThrowDistance _player_ref_2))
  (bind _returnvalue_3 (- _returnvalue_2 _returnvalue))
  (bind _returnvalue_4 (Math|Vector|VectorLength _returnvalue_3))
  (bind _returnvalue_5 (Math|Float|MapRangeClamped _returnvalue_4 _grapplethrowdistance _grappledetectionradius 1e+02 1e+01))
  ;[1 1 1] Controlling how the UI for the Grapple Point is displayed based on distance from the player. Gradually gets bigger as the player gets closer, and turns green when the player is in Grapple Range - Ryan
  (Class|CanvasPanelSlot|SetSize (Class|WidgetLayoutLibrary|SlotasCanvasSlot (Variables|/Game/UI/GameplayUI/GrappleUI/WB_NewDetectionNode.WB_NewDetectionNode_C|GetFill (Variables|Default|GetWidget%20Ref))) (Math|Vector2D|MakeVector2D _returnvalue_5 _returnvalue_5))
  (Appearance|SetColorandOpacity (Variables|/Game/UI/GameplayUI/GrappleUI/WB_NewDetectionNode.WB_NewDetectionNode_C|GetFill (Variables|Default|GetWidget%20Ref)) (select (== _returnvalue_5 1e+02) "(R=0.436045,G=1.000000,B=0.340369,A=1.000000)" "(R=0.442708,G=0.442708,B=0.442708,A=1.000000)") :!class /Script/UMG.Image))