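; BP_Painting is a painting actor for the Boss 1 mechanics that the player pushes by touching it.
; On BeginPlay it finds BP_King and the Boss1Manager, then snaps itself to the King's spineSocket.
; When the player pawn enters its Box while CanPush is set, it reports the push to the manager and clears CanPush.
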(event OnComponentBeginOverlap(Box)
  (params (OverlappedComponent :type Primitive%20Component%20Object%20Reference) (OtherActor :type Actor%20Object%20Reference) (OtherComp :type Primitive%20Component%20Object%20Reference) (OtherBodyIndex :type Integer) (bFromSweep :type Boolean) (SweepResult :type Hit%20Result%20Structure%20%28by%20ref%29))
  (if (== OtherActor (Game|Player|GetPlayerPawn 0))
    (if (Variables|Default|GetCanPush)
      (CallFunction|PaintingPushed))))

(event Custom|PaintingPushed
  (Default|PaintingPushed (Variables|Default|GetManager))
  (Variables|Default|SetCanPush false))

(event EventBeginPlay
  (bind _returnvalue (Actor|GetActorOfClass "/Game/Blueprints/Enemies/King/BP_King.BP_King_C"))
  (Variables|Default|SetKing _returnvalue)
  (bind _returnvalue_2 (Actor|GetActorOfClass "/Game/Blueprints/Mechanics/Boss1Stuff/Boss1Manager.Boss1Manager_C"))
  (Variables|Default|SetManager _returnvalue_2)
  (Transformation|AttachActorToActor (Variables|Default|GetKing) "spineSocket" "SnapToTarget" "SnapToTarget" "SnapToTarget" true))

(event Collision|EventActorBeginOverlap
  (params (OtherActor :type Actor%20Object%20Reference)))

(event EventTick
  (params (DeltaSeconds :type Float%20%28single-precision%29)))

(fn ConstructionScript)