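; Light manager Blueprint in the Boss 1 mechanics folder that switches a room's lighting on and off.
; TurnOnRoomLights sets two rect lights to the LightIntensity variable and a referenced directional light to a fixed intensity.
; TurnOffRoomLights sets all three lights to zero intensity.
; It has no active logic of its own, so switching depends on those two events being called.
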(event Custom|TurnOnRoomLights
  (Rendering|Components|Light|SetIntensity (Variables|Default|GetRectLight1) (Variables|Default|GetLightIntensity))
  (Rendering|Components|Light|SetIntensity (Variables|/Script/Engine.Light|GetLightComponent (Variables|Default|GetDirectional)) 1.0))

(event Custom|TurnOffRoomLights
  (Rendering|Components|Light|SetIntensity (Variables|Default|GetRectLight1) 0.0)
  (Rendering|Components|Light|SetIntensity (Variables|/Script/Engine.Light|GetLightComponent (Variables|Default|GetDirectional)) 0.0))

(event EventBeginPlay)

(event Collision|EventActorBeginOverlap
  (params (OtherActor :type Actor%20Object%20Reference)))

(event EventTick
  (params (DeltaSeconds :type Float%20%28single-precision%29)))

(fn ConstructionScript)