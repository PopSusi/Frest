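; Spotlight button for the first boss fight that reports presses to the Boss1Manager found at BeginPlay.
; A box overlap by the player in one specific movement type calls ButtonPressed on the manager, gated by a DoOnce.
; ResetButton moves the mesh to a randomly picked child of the Scene component and re-arms the DoOnce.
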(event OnComponentBeginOverlap(Box)
  (params (OverlappedComponent :type Primitive%20Component%20Object%20Reference) (OtherActor :type Actor%20Object%20Reference) (OtherComp :type Primitive%20Component%20Object%20Reference) (OtherBodyIndex :type Integer) (bFromSweep :type Boolean) (SweepResult :type Hit%20Result%20Structure%20%28by%20ref%29))
  (bind _asbp_player (Utilities|Casting|CastToBP_Player OtherActor))
  (if (Utilities|Enum|Equal(Enum) (Variables|/Game/Blueprints/Player/BP_Player.BP_Player_C|GetMovementType _asbp_player) "NewEnumerator15")
    (Utilities|FlowControl|DoOnce false
      (:Completed
        (Default|ButtonPressed (Variables|Default|GetManager))))))

(event Custom|ResetButton
  (Transformation|SetWorldLocation (Variables|Default|GetStaticMesh) (Transformation|GetWorldLocation (.OutItem (Utilities|Array|Random (Components|GetChildrenComponents (Variables|Default|GetScene) false)))) false false)
  (Utilities|FlowControl|DoOnce false) ; enters at Reset
)

(event EventBeginPlay
  (bind _returnvalue (Actor|GetActorOfClass "/Game/Blueprints/Mechanics/Boss1Stuff/Boss1Manager.Boss1Manager_C"))
  (Variables|Default|SetManager _returnvalue))

(event Collision|EventActorBeginOverlap
  (params (OtherActor :type Actor%20Object%20Reference)))

(event EventTick
  (params (DeltaSeconds :type Float%20%28single-precision%29)))

(fn ConstructionScript)