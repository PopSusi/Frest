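; BP_FakePainting is a Boss 1 painting actor that reports Goo Pod hits to the fight's manager.
; PaintingPushed calls PaintingHitWithPod on the manager and clears CanPush to block repeat pushes.
; BeginPlay is empty, and the logic to find the manager and attach to the King's spine is disconnected.
; The hit check that would trigger pushes from pods or damage the player is also disconnected.
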(event Custom|PaintingPushed
  ;[1 1 1] Update Manager about Push - Austin
  (Default|PaintingHitwithPod (Variables|Default|GetManager))
  (Variables|Default|SetCanPush false))

(event EventBeginPlay
  ;[1 1 1] Attach Real Painting to Boss when the level starts - Austin
)

(fn ConstructionScript)