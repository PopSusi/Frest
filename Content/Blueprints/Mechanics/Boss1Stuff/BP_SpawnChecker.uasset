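; BP_SpawnChecker is a helper actor in the Boss1 mechanics that stops enemy spawners near the player from spawning.
; On BeginPlay it snaps its root component onto the player character's root, so its Sphere follows the player.
; Any BP_EnemySpawner entering the Sphere gets ShouldSpawn set to false, and it is set back to true when that spawner leaves.
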(event OnComponentBeginOverlap(Sphere)
  (params (OverlappedComponent :type Primitive%20Component%20Object%20Reference) (OtherActor :type Actor%20Object%20Reference) (OtherComp :type Primitive%20Component%20Object%20Reference) (OtherBodyIndex :type Integer) (bFromSweep :type Boolean) (SweepResult :type Hit%20Result%20Structure%20%28by%20ref%29))
  (if (== (Utilities|GetClass OtherActor) "/Game/Blueprints/Mechanics/Boss1Stuff/BP_EnemySpawner.BP_EnemySpawner_C")
    (bind _asbp_enemy_spawner (Utilities|Casting|CastToBP_EnemySpawner OtherActor))
    (Variables|/Game/Blueprints/Mechanics/Boss1Stuff/BP_EnemySpawner.BP_EnemySpawner_C|SetShouldSpawn _asbp_enemy_spawner false)))

(event OnComponentEndOverlap(Sphere)
  (params (OverlappedComponent :type Primitive%20Component%20Object%20Reference) (OtherActor :type Actor%20Object%20Reference) (OtherComp :type Primitive%20Component%20Object%20Reference) (OtherBodyIndex :type Integer))
  (if (== (Utilities|GetClass OtherActor) "/Game/Blueprints/Mechanics/Boss1Stuff/BP_EnemySpawner.BP_EnemySpawner_C")
    (bind _asbp_enemy_spawner (Utilities|Casting|CastToBP_EnemySpawner OtherActor))
    (Variables|/Game/Blueprints/Mechanics/Boss1Stuff/BP_EnemySpawner.BP_EnemySpawner_C|SetShouldSpawn _asbp_enemy_spawner true)))

(event EventBeginPlay
  (Transformation|AttachComponentToComponent (Variables|Default|GetDefaultSceneRoot) (Variables|/Script/Engine.Actor|GetRootComponent (Game|GetPlayerCharacter 0)) "None" "SnapToTarget" "SnapToTarget" "SnapToTarget" true))

(event Collision|EventActorBeginOverlap
  (params (OtherActor :type Actor%20Object%20Reference)))

(event EventTick
  (params (DeltaSeconds :type Float%20%28single-precision%29)))

(fn ConstructionScript)