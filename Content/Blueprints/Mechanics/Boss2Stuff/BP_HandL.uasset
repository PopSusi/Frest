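; BP_HandL is a floating hand of the BP_Scholar2 boss that fires a ScholarLaser attack shortly after spawning.
; A looping FlipFlop timeline bobs the mesh, while another pitches the hand before it attaches the spawned laser.
; Tick switches on an enum: the laser state eases above the player, and idle eases to an offset beside the boss, both matching boss yaw.
; A timer ends the attack, destroying the laser and returning to idle.
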(event Custom|StartFloat
  (if (not (Variables|Default|GetStopFloat))
    (Utilities|FlowControl|FlipFlop
      (:A
        (bind _newtrack_0 (Timeline|Timeline PlayFromStart)
          (:Update
            (Transformation|SetRelativeLocation (Variables|Default|GetStaticMesh) (Math|Vector|MakeVector 0.0 0.0 _newtrack_0) false false))
          (:Finished
            (CallFunction|StartFloat))))
      (:B
        (Timeline|Timeline ReverseFromEnd)))))

(event Custom|StartLaserAttack
  (bind _returnvalue (Transformation|GetActorRotation))
  (bind _newtrack_0 (Timeline|RotateHand PlayFromStart)
    (:Update
      (Transformation|SetActorRotation (Math|Rotator|MakeRotator (.roll _returnvalue) _newtrack_0 (.yaw _returnvalue))))
    (:Finished
      (Variables|Default|SetEnum "NewEnumerator0")
      (bind _returnvalue_2 (Game|SpawnActorfromClass "/Game/Blueprints/Mechanics/Boss2Stuff/ScholarLaser.ScholarLaser_C" (Transformation|GetActorTransform) "Undefined" "MultiplyWithRoot" 0 0))
      (Transformation|AttachComponentToComponent _returnvalue_2 (Variables|Default|GetStaticMesh) "None" "SnapToTarget" "SnapToTarget" "SnapToTarget" true)
      (Utilities|Time|SetTimerbyEvent (delegate Custom|EndLaserAttack) 15.0))))

(event Custom|EndLaserAttack
  (bind _returnvalue (Transformation|GetActorRotation))
  (Utilities|FlowControl|Sequence
    (:then_0
      (Actor|DestroyActor (stale Custom|StartLaserAttack _returnvalue_2))
      (Variables|Default|SetEnum "NewEnumerator2"))
    (:then_1
      (bind _newtrack_0 (Timeline|Timeline_0 ReverseFromEnd)
        (:Update
          (Transformation|SetActorRotation (Math|Rotator|MakeRotator (.roll _returnvalue) _newtrack_0 (.yaw _returnvalue))))))))

(event EventBeginPlay
  (Utilities|FlowControl|Delay 0.4)
  (CallFunction|StartFloat)
  (CallFunction|StartLaserAttack))

(event Collision|EventActorBeginOverlap
  (params (OtherActor :type Actor%20Object%20Reference)))

(event EventTick
  (params (DeltaSeconds :type Float%20%28single-precision%29))
  (switch Utilities|FlowControl|Switch|SwitchonBoss2States (Variables|Default|GetEnum)
    (:NewEnumerator0
      (Utilities|LaserAttackLogic DeltaSeconds))
    (:NewEnumerator2
      (Utilities|IdleLogic DeltaSeconds))))

(fn ConstructionScript)