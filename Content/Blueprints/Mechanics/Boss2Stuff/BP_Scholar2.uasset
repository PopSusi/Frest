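; BP_Scholar2 is a floating actor, filed with the second boss's mechanics, that constantly turns to face the player.
; Tick updates only the actor's yaw toward player pawn 0, preserving its pitch and roll.
; From BeginPlay, StartFloat alternates a timeline forward and in reverse through a FlipFlop, re-triggering on finish to bob the static mesh along relative Z.
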(event Custom|StartFloat
  (Utilities|FlowControl|FlipFlop
    (:A
      (bind _newtrack_0 (Timeline|FloatTimeline PlayFromStart)
        (:Update
          (Transformation|SetRelativeLocation (Variables|Default|GetStaticMesh) (Math|Vector|MakeVector 0.0 0.0 _newtrack_0) false false))
        (:Finished
          (CallFunction|StartFloat))))
    (:B
      (Timeline|FloatTimeline ReverseFromEnd))))

(event EventBeginPlay
  (CallFunction|StartFloat))

(event Collision|EventActorBeginOverlap
  (params (OtherActor :type Actor%20Object%20Reference)))

(event EventTick
  (params (DeltaSeconds :type Float%20%28single-precision%29))
  (bind _returnvalue (Transformation|GetActorRotation))
  (Transformation|SetActorRotation (Math|Rotator|MakeRotator (.roll _returnvalue) (.pitch _returnvalue) (.yaw (Math|Rotator|FindLookatRotation (Transformation|GetActorLocation) (Transformation|GetActorLocation (Game|Player|GetPlayerPawn 0)))))))

(fn ConstructionScript)