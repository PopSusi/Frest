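; BP_HandR is the floating right hand of the Scholar boss (BP_Scholar2).
; Each tick, IdleLogic eases it to an offset right and forward of the Scholar and matches its yaw.
; A flip-flopped timeline bobs the HAND mesh up and down.
; Laser attack code (hovering above the player, pitching, spawning ScholarLaser) is disconnected; its events, RaiseWall and the Tick state branches are empty.
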(event Custom|StartFloat
  (if (not (Variables|Default|GetStopFloat))
    (Utilities|FlowControl|FlipFlop
      (:A
        (bind _newtrack_0 (Timeline|Timeline PlayFromStart)
          (:Update
            (Transformation|SetRelativeLocation (Variables|Default|GetHAND) (Math|Vector|MakeVector 0.0 0.0 _newtrack_0) false false))
          (:Finished
            (CallFunction|StartFloat))))
      (:B
        (Timeline|Timeline ReverseFromEnd)))))

(event Custom|StartLaserAttack)

(event Custom|EndLaserAttack)

(event Custom|RaiseWall)

(event EventBeginPlay
  (Utilities|FlowControl|Delay 0.4)
  (CallFunction|StartFloat)
  (bind _returnvalue (Actor|GetActorOfClass "/Game/Blueprints/Mechanics/Boss2Stuff/BP_Scholar2.BP_Scholar2_C"))
  (Variables|Default|SetScholar _returnvalue))

(event Collision|EventActorBeginOverlap
  (params (OtherActor :type Actor%20Object%20Reference)))

(event EventTick
  (params (DeltaSeconds :type Float%20%28single-precision%29))
  (switch Utilities|FlowControl|Switch|SwitchonBoss2States (Variables|Default|GetEnum)
    (:NewEnumerator0
      _)
    (:NewEnumerator1
      _)
    (:NewEnumerator2
      _))
  (Utilities|IdleLogic DeltaSeconds))

(fn ConstructionScript)