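; PickUpCube is a cube actor that tells the player's BP_CubePickup component when it is within pickup range.
; On PickUpArea begin overlap with BP_Player, it sets InCubeRadius and adds itself to CurrentCubes, but only if that flag was false.
; On end overlap it calls the component's ArrayCheck, then removes itself from the list.
; Both events print debug messages, and the pickup itself is not handled here.
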(event OnComponentBeginOverlap(PickUpArea)
  (params (OverlappedComponent :type Primitive%20Component%20Object%20Reference) (OtherActor :type Actor%20Object%20Reference) (OtherComp :type Primitive%20Component%20Object%20Reference) (OtherBodyIndex :type Integer) (bFromSweep :type Boolean) (SweepResult :type Hit%20Result%20Structure%20%28by%20ref%29))
  (bind _asbp_player (Utilities|Casting|CastToBP_Player OtherActor))
  (Utilities|IsValid (Actor|GetComponentbyClass _asbp_player "/Game/Blueprints/Player/Components/BP_CubePickup.BP_CubePickup_C")
    (:Is%20Valid
      (if (not (Variables|/Game/Blueprints/Player/Components/BP_CubePickup.BP_CubePickup_C|GetInCubeRadius (Actor|GetComponentbyClass _asbp_player "/Game/Blueprints/Player/Components/BP_CubePickup.BP_CubePickup_C")))
        (Variables|/Game/Blueprints/Player/Components/BP_CubePickup.BP_CubePickup_C|SetInCubeRadius (Actor|GetComponentbyClass _asbp_player "/Game/Blueprints/Player/Components/BP_CubePickup.BP_CubePickup_C") true)
        (Development|PrintString "Player is in cube")
        (Utilities|Array|AddUnique (Variables|/Game/Blueprints/Player/Components/BP_CubePickup.BP_CubePickup_C|GetCurrentCubes (Actor|GetComponentbyClass _asbp_player "/Game/Blueprints/Player/Components/BP_CubePickup.BP_CubePickup_C")) self)))))

(event OnComponentEndOverlap(PickUpArea)
  (params (OverlappedComponent :type Primitive%20Component%20Object%20Reference) (OtherActor :type Actor%20Object%20Reference) (OtherComp :type Primitive%20Component%20Object%20Reference) (OtherBodyIndex :type Integer))
  (bind _asbp_player (Utilities|Casting|CastToBP_Player OtherActor))
  (Utilities|IsValid (Actor|GetComponentbyClass _asbp_player "/Game/Blueprints/Player/Components/BP_CubePickup.BP_CubePickup_C")
    (:Is%20Valid
      (Default|ArrayCheck (Actor|GetComponentbyClass _asbp_player "/Game/Blueprints/Player/Components/BP_CubePickup.BP_CubePickup_C"))
      (Utilities|Array|RemoveItem (Variables|/Game/Blueprints/Player/Components/BP_CubePickup.BP_CubePickup_C|GetCurrentCubes (Actor|GetComponentbyClass _asbp_player "/Game/Blueprints/Player/Components/BP_CubePickup.BP_CubePickup_C")) self)
      (Development|PrintString "Player is out of cube"))))

(event EventBeginPlay)

(event Collision|EventActorBeginOverlap
  (params (OtherActor :type Actor%20Object%20Reference)))

(event EventTick
  (params (DeltaSeconds :type Float%20%28single-precision%29)))

(fn ConstructionScript)