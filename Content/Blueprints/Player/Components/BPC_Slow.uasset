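; Player component for carrying and throwing goo pods, the time-slow objects (BP_TimeObject).
; IA_PickUp drops the held pod or sphere-overlaps for a BP_TimePickUp plant or loose pod, while AttachSlow spawns one at the hand socket.
; IA_Projectile detaches and activates the pod, launching it by camera-based impulse, either immediately in one movement type or on a gated hold-release.
; Separate functions toggle a timer-updated spline actor as aim visualization.
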(event Custom|Throw
  (bind _playerref (Variables|Default|GetPlayerRef))
  (bind _initialangle (Variables|Default|GetInitialAngle))
  (bind _returnvalue (Transformation|GetActorLocation _playerref))
  (bind _returnvalue_2 (Actor|GetComponentbyClass _playerref "/Script/Engine.CameraComponent"))
  (bind _returnvalue_3 (Math|Vector|GetForwardVector _returnvalue_2))
  (if (Variables|Default|GetThrowBool)
    (if (Variables|Default|GetHolding)
      (Variables|/Game/Blueprints/Mechanics/Actor/BP_TimeObject.BP_TimeObject_C|SetActive (Variables|Default|GetCurrentSlow) true)
      (Utilities|FlowControl|Delay 0.15)
      (Audio|PlaySound2D "/Game/Sounds/SFX/Movement/DoubleJump.DoubleJump" 1.0 1.0 0.0 0 0)
      (Variables|Default|SetThrowAngle (Math|Vector|MakeVector (* (.x _returnvalue_3) _initialangle) (* (.y _returnvalue_3) _initialangle) _initialangle))
      (Default|Detach (Variables|Default|GetCurrentSlow))
      (Class|PrimitiveComponent|SetAllPhysicsLinearVelocity (Variables|/Game/Blueprints/Mechanics/Actor/BP_TimeObject.BP_TimeObject_C|GetStaticMesh (Variables|Default|GetCurrentSlow)) "0, 0, 0" false)
      (Physics|AddImpulse (Variables|/Game/Blueprints/Mechanics/Actor/BP_TimeObject.BP_TimeObject_C|GetStaticMesh (Variables|Default|GetCurrentSlow)) (* (Variables|Default|GetThrowAngle) (Variables|Default|GetThrowVelocity)) "None" true)
      (Collision|BoxTraceByChannel _returnvalue (+ (* (Variables|Default|GetThrowAngle) (Variables|Default|GetThrowVelocity)) _returnvalue) "0, 0, 0" "0, 0, 0" "TraceTypeQuery1" false 0 "None")
      (Variables|Default|SetCurrentSlow 0)
      (Variables|Default|SetHolding false))))

(event Input|EnhancedActionEvents|EnhancedInputActionIA_PickUp
  (params (ActionValue :type Boolean) (ElapsedSeconds :type Float%20%28double-precision%29) (TriggeredSeconds :type Float%20%28double-precision%29) (InputAction :type Input%20Action%20Object%20Reference :default "/Game/Inputs/InputActions/IA_PickUp.IA_PickUp"))
  (bind _returnvalue (Components|GetOwner))
  (bind _pickupradius (Variables|Default|GetPickUpRadius))
  (bind _returnvalue_2 (Transformation|GetActorLocation _returnvalue))
  (:Started
    ;[1 1 1] Check if holding goo pod
    (if (Variables|Default|GetHolding)
      ;[1 1 1] If holding, drop
      (Default|Detach (Variables|Default|GetCurrentSlow))
      (Variables|Default|SetHolding false)
      (else
        ;[1 1 1] Check area for time pickup
        (bind (_outactors _returnvalue_3) (Collision|SphereOverlapActors _returnvalue_2 _pickupradius (Variables|Default|GetStatic%20Query) "/Game/Blueprints/Mechanics/Actor/BP_TimePickUp.BP_TimePickUp_C" (Utilities|Array|MakeArray _returnvalue)))
        ;[1 1 1] If true, cast and attempt pickup
        (if _returnvalue_3
          (bind _array_element (Utilities|Array|ForEachLoopwithBreak _outactors)
            (:LoopBody
              (bind _asbp_time_pick_up (Utilities|Casting|CastToBP_TimePickUp _array_element))
              (bind _pickedup (Default|Pickup _asbp_time_pick_up self))
              (Variables|Default|SetHolding _pickedup)
              (Rendering|SetVisibility (Variables|/Game/Blueprints/Mechanics/Actor/BP_TimePickUp.BP_TimePickUp_C|GetWidget _asbp_time_pick_up) false false)
              (if (not _pickedup)
                ;[1 1 1] If not goo plant, see if goo pod is nearby
                (bind _outactors_2 (Collision|SphereOverlapActors _returnvalue_2 _pickupradius (Utilities|Array|MakeArray "ObjectTypeQuery2") "/Game/Blueprints/Mechanics/Actor/BP_TimeObject.BP_TimeObject_C" :!label _label))
                (bind _array_element_2 (Utilities|Array|ForEachLoopwithBreak _outactors_2 :!label _label_2)
                  (:LoopBody
                    (bind _asbp_time_object (Utilities|Casting|CastToBP_TimeObject _array_element_2))
                    (bind _output_get (Variables|Default|SetCurrentSlow _asbp_time_object))
                    (Default|PickBackUp _output_get (Variables|Default|GetPlayerRef))
                    (Variables|Default|SetHolding true)
                    (goto _label_2 Break))))))
          (else
            (goto _label)))))))

(event Input|EnhancedActionEvents|EnhancedInputActionIA_Projectile
  (params (ActionValue :type Boolean) (ElapsedSeconds :type Float%20%28double-precision%29) (TriggeredSeconds :type Float%20%28double-precision%29) (InputAction :type Input%20Action%20Object%20Reference :default "/Game/Inputs/InputActions/IA_Projectile.IA_Projectile"))
  (bind _playerref (Variables|Default|GetPlayerRef))
  (bind _initialangle (Variables|Default|GetInitialAngle))
  (bind _returnvalue (Transformation|GetActorLocation _playerref))
  (bind _returnvalue_2 (Actor|GetComponentbyClass _playerref "/Script/Engine.CameraComponent"))
  (bind _returnvalue_3 (Math|Vector|GetForwardVector _returnvalue_2))
  (:Ongoing
    (if (Utilities|Enum|Equal(Enum) (Variables|/Game/Blueprints/Player/BP_Player.BP_Player_C|GetMovementType (Variables|Default|GetPlayerRef)) "NewEnumerator12")
      (if (Variables|Default|GetHolding)
        (Variables|/Game/Blueprints/Mechanics/Actor/BP_TimeObject.BP_TimeObject_C|SetActive (Variables|Default|GetCurrentSlow) true)
        (Utilities|FlowControl|Delay 0.15)
        (Audio|PlaySound2D "/Game/Sounds/SFX/Movement/DoubleJump.DoubleJump" 1.0 1.0 0.0 0 0)
        (Variables|Default|SetThrowAngle (Math|Vector|MakeVector (* (.x _returnvalue_3) _initialangle) (* (.y _returnvalue_3) _initialangle) _initialangle))
        (Default|Detach (Variables|Default|GetCurrentSlow))
        (Class|PrimitiveComponent|SetAllPhysicsLinearVelocity (Variables|/Game/Blueprints/Mechanics/Actor/BP_TimeObject.BP_TimeObject_C|GetStaticMesh (Variables|Default|GetCurrentSlow)) "0, 0, 0" false)
        (Physics|AddImpulse (Variables|/Game/Blueprints/Mechanics/Actor/BP_TimeObject.BP_TimeObject_C|GetStaticMesh (Variables|Default|GetCurrentSlow)) (* (Variables|Default|GetThrowAngle) (Variables|Default|GetThrowVelocity)) "None" true)
        (Collision|BoxTraceByChannel _returnvalue (+ (* (Variables|Default|GetThrowAngle) (Variables|Default|GetThrowVelocity)) _returnvalue) "0, 0, 0" "0, 0, 0" "TraceTypeQuery1" false 0 "None")
        (Variables|Default|SetCurrentSlow 0)
        (Variables|Default|SetHolding false))
      (elif (and (Variables|Default|GetHolding) (> 0.2 ElapsedSeconds))
        (Utilities|FlowControl|DoOnce false :!label _label))))
  (:Completed
    (if (not (> 0.2 ElapsedSeconds))
      (CallFunction|Throw)
      (Variables|Default|SetHeldSeconds 0.0)
      (goto _label Reset))))

(event EventBeginPlay
  (bind _returnvalue (Components|GetOwner))
  (bind _asbp_player (Utilities|Casting|CastToBP_Player _returnvalue))
  (Variables|Default|SetPlayerRef _asbp_player)
  (Variables|Default|SetCamera (Actor|GetComponentbyClass _returnvalue "/Script/Engine.CameraComponent")))

(event EventTick
  (params (DeltaSeconds :type Float%20%28single-precision%29)))

(event EventReadytoThrow
  (Variables|Default|SetThrowBool true))

(fn AttachSlow
  (bind _playerref (Variables|Default|GetPlayerRef))
  (bind _mesh (Variables|/Script/Engine.Character|GetMesh _playerref))
  (bind _returnvalue (Transformation|GetSocketTransform _mesh "PickupSocket" "RTS_World"))
  (bind (_location _rotation) (Math|Transform|BreakTransform _returnvalue))
  ;[1 1 1] Spawn and move BP_GooPod to socket
  (bind _returnvalue_2 (Game|SpawnActorfromClass "/Game/Blueprints/Mechanics/Actor/BP_TimeObject.BP_TimeObject_C" (Math|Transform|MakeTransform _location _rotation "1.000000,1.000000,1.000000") "Undefined" "MultiplyWithRoot" 0 0))
  (Variables|Default|SetCurrentSlow _returnvalue_2)
  ;[1 1 1] Attach
  (Transformation|AttachComponentToComponent _returnvalue_2 _mesh "PickupSocket" "SnapToTarget" "SnapToTarget" "KeepWorld" true)
  (Variables|Default|SetHolding true))

(fn AttemptDrop
  (bind _currentslow (Variables|Default|GetCurrentSlow))
  (Utilities|IsValid _currentslow
    (:Is%20Valid
      (Default|Detach _currentslow)
      (Variables|Default|SetHolding false))))

(fn RemoveArc
  (bind _currentvisualization (Variables|Default|GetCurrentVisualization))
  (Utilities|IsValid _currentvisualization
    (:Is%20Valid
      (Rendering|SetVisibility (Variables|/Game/Blueprints/Player/Components/Spline.Spline_C|GetStaticMesh _currentvisualization) false false)
      (Utilities|Time|ClearandInvalidateTimerbyHandle (Variables|Default|GetUpdateVisualTimer)))))

(fn ActivateArc
  (Utilities|IsValid (Variables|Default|GetCurrentVisualization)
    (:Is%20Valid
      _)
    (:Is%20Not%20Valid
      (bind _returnvalue (Game|SpawnActorfromClass "/Game/Blueprints/Player/Components/Spline.Spline_C" (Math|Transform|MakeTransform "0, 0, 0" "0, 0, 0" "1.000000,1.000000,1.000000") "Undefined" "MultiplyWithRoot" 0 0))
      (Variables|Default|SetCurrentVisualization _returnvalue)))
  (Rendering|SetVisibility (Variables|/Game/Blueprints/Player/Components/Spline.Spline_C|GetStaticMesh (Variables|Default|GetCurrentVisualization)) true false)
  (bind _returnvalue_2 (Utilities|Time|SetTimerbyFunctionName 0 "UpdateVisualization" 0.02 true))
  (Variables|Default|SetUpdateVisualTimer _returnvalue_2))

(fn UpdateVisualization
  (bind _camera (Variables|Default|GetCamera))
  (bind _playerref (Variables|Default|GetPlayerRef))
  (bind _returnvalue (Transformation|GetWorldLocation _camera))
  (bind _returnvalue_2 (Transformation|GetActorLocation _playerref))
  (bind _returnvalue_3 (- _returnvalue_2 _returnvalue))
  (bind _returnvalue_4 (Math|Vector|Normalize _returnvalue_3))
  (bind (_x _y) (Math|Vector|BreakVector _returnvalue_4))
  (Transformation|SetActorLocationAndRotation (Variables|Default|GetCurrentVisualization) _returnvalue_2 (Math|Conversions|RotationFromXVector (Math|Vector|MakeVector _x _y 0.0)))
  (Collision|LineTraceByChannel _returnvalue (Math|Vector|MakeVector _x _y 0.0) "TraceTypeQuery1" false 0 "None"))

(fn IsHolding
  (return (Variables|Default|GetHolding)))