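; Player component that handles player death, presumably in boss fights, by moving to the level set in its LevelData.
; On BeginPlay it binds Reload to the owning BP_Player's death event.
; Reload freezes time via global dilation, starts async-loading the level asset and immediately shows a LoadWithImage screen with the custom image and UI-only input.
; When the async load completes, it notifies that widget through LoadDone.
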(event Custom|Reload
  (bind _leveldata (Variables|Default|GetLevelData))
  (Utilities|Time|SetGlobalTimeDilation 0.0)
  (Utilities|AsyncLoadAsset (.worldasset (.leveltoload _leveldata))
    (:then
      (bind _returnvalue (UserInterface|CreateWidget "/Game/UI/Widgets/LevelLoad/LoadWithImage.LoadWithImage_C" 0 (.customimage _leveldata) (Utilities|Struct|MakeSoftWorldReference (.worldasset (.leveltoload _leveldata)))))
      (UserInterface|Viewport|AddtoViewport _returnvalue 0)
      (Input|SetInputModeUIOnly (Game|GetPlayerController 0) _returnvalue "DoNotLock" false))
    (:Completed
      (Default|LoadDone _returnvalue))))

(event EventBeginPlay
  (bind _asbp_player (Utilities|Casting|CastToBP_Player (Components|GetOwner)))
  (EventDispatchers|BindEventtoPlayerDied _asbp_player (delegate Custom|Reload)))

(event EventTick
  (params (DeltaSeconds :type Float%20%28single-precision%29)))