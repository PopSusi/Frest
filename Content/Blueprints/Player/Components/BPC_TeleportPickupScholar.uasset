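; Player component for a teleport pickup that launches the player as a flying yarn mesh and damages the Scholar boss.
; BeginPlay saves movement defaults and applies flight settings and a fixed yaw, while Tick sweeps the player along Direction.
; After half a second it calls TakeDamage on the found BP_Scholar, without checking contact, and ends.
; Ending, also reachable by timer, spawns impact effects, restores the player and destroys the component.
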(event Custom|DestroyThis
  (bind _as_bp_player (Variables|Default|GetAs%20BP%20Player))
  (bind _as_bp_player_2 (Variables|Default|GetAs%20BP%20Player))
  (bind _charactermovement (Variables|/Script/Engine.Character|GetCharacterMovement _as_bp_player_2))
  (Niagara|SpawnSystematLocation "/Game/Art/Jack_VFX/BossFX/FX_NS_BossImpact.FX_NS_BossImpact" (Transformation|GetActorLocation (Components|GetOwner)))
  (Utilities|FlowControl|Delay 0.1)
  (Pawn|Components|CharacterMovement|SetMovementMode _charactermovement "MOVE_Falling" 0)
  (Variables|/Game/Blueprints/Player/BP_Player.BP_Player_C|SetMovementType _as_bp_player_2 "NewEnumerator0")
  (Components|SkeletalMesh|SetSkeletalMeshAsset (Variables|/Script/Engine.Character|GetMesh _as_bp_player_2) "/Game/Art/Spencer_Assets/Riley_Anim_Test/Riley_Skeleton.Riley_Skeleton")
  (Variables|/Script/Engine.CharacterMovementComponent|SetbOrientRotationToMovement _charactermovement true)
  (Variables|/Script/Engine.CharacterMovementComponent|SetMaxFlySpeed _charactermovement (Variables|Default|GetDefaultFlyingSpeed))
  (Variables|/Script/Engine.CharacterMovementComponent|SetMaxAcceleration _charactermovement (Variables|Default|GetDefaultMaxAcceleration))
  (Variables|/Script/Engine.SpringArmComponent|SetbUsePawnControlRotation (Variables|/Game/Blueprints/Player/BP_Player.BP_Player_C|GetSpringArm _as_bp_player) true)
  (Class|PrimitiveComponent|SetConstraintMode (Variables|/Script/Engine.Character|GetCapsuleComponent _as_bp_player) "Default")
  (Audio|PlaySound2D (select (Math|Random|RandomBool) "/Game/Sounds/SFX/BossFunnyHit2.BossFunnyHit2" "/Game/Sounds/SFX/BossFunnyHit1.BossFunnyHit1") 1.0 1.0 0.0 0 0)
  (Components|DestroyComponent))

(event Custom|EndTeleport
  (Utilities|Time|ClearandInvalidateTimerbyHandle (stale EventBeginPlay _returnvalue))
  (Default|TeleportVFXOff (Variables|Default|GetAs%20BP%20Player))
  (CallFunction|DestroyThis))

(event EventBeginPlay
  (bind _asbp_player (Utilities|Casting|CastToBP_Player (Components|GetOwner)))
  (bind _output_get (Variables|Default|SetAs%20BP%20Player _asbp_player))
  (Default|TeleportVFXon _output_get)
  (bind _returnvalue (Utilities|Time|SetTimerbyEvent (delegate Custom|DestroyThis) (select (Variables|Default|GetSetFlyingTime) (Variables|Default|GetFlyingTime) (Variables|Default|GetDefaultFlyingSpeed))))
  (Variables|Default|SetDefaultFlyingSpeed (Variables|/Script/Engine.CharacterMovementComponent|GetMaxFlySpeed (Variables|/Script/Engine.Character|GetCharacterMovement _output_get)))
  (Variables|Default|SetDefaultMaxAcceleration (Class|CharacterMovementComponent|GetMaxAcceleration (Variables|/Script/Engine.Character|GetCharacterMovement _output_get)))
  (CallFunction|InitiateTeleport)
  (Utilities|FlowControl|Delay 0.5)
  (bind _returnvalue_2 (Actor|GetActorOfClass "/Game/Blueprints/Enemies/Scholar/BP_Scholar.BP_Scholar_C"))
  (bind _asbp_scholar (Utilities|Casting|CastToBP_Scholar _returnvalue_2))
  (Default|TakeDamage _asbp_scholar)
  (CallFunction|EndTeleport))

(event EventTick
  (params (DeltaSeconds :type Float%20%28single-precision%29))
  (bind _as_bp_player (Variables|Default|GetAs%20BP%20Player))
  (Transformation|SetActorLocation _as_bp_player (+ (Transformation|GetActorLocation _as_bp_player) (* (Math|Vector|GetForwardVector (Variables|Default|GetDirection)) (* DeltaSeconds (Variables|Default|GetTeleportForwardSpeed)))) true false))

(fn InitiateTeleport
  (bind _as_bp_player (Variables|Default|GetAs%20BP%20Player))
  (bind _charactermovement (Variables|/Script/Engine.Character|GetCharacterMovement _as_bp_player))
  (Class|PrimitiveComponent|SetConstraintMode (Variables|/Script/Engine.Character|GetCapsuleComponent _as_bp_player) "XYPlane")
  (Variables|/Script/Engine.CharacterMovementComponent|SetbOrientRotationToMovement (Variables|/Script/Engine.Character|GetCharacterMovement _as_bp_player) false)
  (Transformation|SetActorRotation _as_bp_player (Math|Rotator|MakeRotator 0.0 0.0 (.yaw (Variables|Default|GetDirection))))
  (Variables|/Script/Engine.SpringArmComponent|SetbUsePawnControlRotation (Variables|/Game/Blueprints/Player/BP_Player.BP_Player_C|GetSpringArm _as_bp_player) false)
  (Components|SkeletalMesh|SetSkeletalMeshAsset (Variables|/Script/Engine.Character|GetMesh _as_bp_player) "/Game/Art/PlayerBall/low_Poly_yarn.low_Poly_yarn")
  (Pawn|Components|CharacterMovement|SetMovementMode _charactermovement "MOVE_Flying" 0)
  (Variables|/Game/Blueprints/Player/BP_Player.BP_Player_C|SetMovementType (Variables|Default|GetAs%20BP%20Player) "NewEnumerator4")
  (Variables|/Script/Engine.CharacterMovementComponent|SetMaxFlySpeed _charactermovement (Variables|Default|GetTeleportFlyingSpeed))
  (Variables|/Script/Engine.CharacterMovementComponent|SetMaxAcceleration _charactermovement (Variables|Default|GetTeleportMaxAcceleration)))