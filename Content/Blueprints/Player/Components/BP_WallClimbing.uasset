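; Player component that handles entering, maintaining and leaving the wall climbing state on BP_Player.
; InitiateWallClimb zeroes velocity, switches to Flying movement and disables orient-to-movement; EndWallClimb restores orient-to-movement and switches to Falling.
; While climbing, Tick traces a short line forward and yaws the player to face into the hit surface's normal.
; The Wallnormal input is unused, and climb detection and movement input are not handled here.
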(event Custom|InitiateWallClimb
  (params (Wallnormal :type Vector))
  (bind _as_bp_player (Variables|Default|GetAs%20BP%20Player))
  (bind _charactermovement (Variables|/Script/Engine.Character|GetCharacterMovement _as_bp_player))
  (Variables|/Game/Blueprints/Player/BP_Player.BP_Player_C|SetIsWallClimbing _as_bp_player true)
  (Variables|/Script/Engine.MovementComponent|SetVelocity (Variables|/Script/Engine.Character|GetCharacterMovement _as_bp_player) "0, 0, 0")
  (Pawn|Components|CharacterMovement|SetMovementMode _charactermovement "MOVE_Flying" 0)
  (Variables|/Script/Engine.CharacterMovementComponent|SetbOrientRotationToMovement _charactermovement false))

(event Custom|EndWallClimb
  (bind _as_bp_player (Variables|Default|GetAs%20BP%20Player))
  (bind _charactermovement (Variables|/Script/Engine.Character|GetCharacterMovement _as_bp_player))
  (Variables|/Game/Blueprints/Player/BP_Player.BP_Player_C|SetIsWallClimbing _as_bp_player false)
  (Pawn|Components|CharacterMovement|SetMovementMode _charactermovement "MOVE_Falling" 0)
  (Variables|/Script/Engine.CharacterMovementComponent|SetbOrientRotationToMovement _charactermovement true))

(event EventBeginPlay
  (bind _asbp_player (Utilities|Casting|CastToBP_Player (Components|GetOwner)))
  (Variables|Default|SetAs%20BP%20Player _asbp_player))

(event EventTick
  (params (DeltaSeconds :type Float%20%28single-precision%29))
  (bind _as_bp_player (Variables|Default|GetAs%20BP%20Player))
  (bind _as_bp_player_2 (Variables|Default|GetAs%20BP%20Player))
  (bind _returnvalue (Transformation|GetActorLocation _as_bp_player_2))
  (if (Variables|/Game/Blueprints/Player/BP_Player.BP_Player_C|GetIsWallClimbing _as_bp_player)
    (bind (_outhit _returnvalue_2) (Collision|LineTraceByChannel _returnvalue (+ _returnvalue (* (Math|Vector|GetForwardVector (Transformation|GetActorRotation _as_bp_player_2)) 1e+02)) "TraceTypeQuery1" false 0 "None"))
    (if _returnvalue_2
      (Transformation|SetActorRotation _as_bp_player (Math|Rotator|MakeRotator 0.0 0.0 (+ (.yaw (Math|Conversions|RotationFromXVector (.Normal (Collision|BreakHitResult _outhit)))) 1.8e+02)) true))))