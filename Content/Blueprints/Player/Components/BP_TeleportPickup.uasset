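; Player component for a teleport pickup that flies BP_Player forward as a sphere for a limited time.
; On BeginPlay it faces the player along Direction's yaw, swaps the mesh, stops camera control rotation and applies boosted Flying movement.
; Tick adds forward input along the capsule.
; The FlyingTime timer or EndTeleport restores walking, speeds, camera and the hard-coded SK_Devvy_M mesh, then destroys the component.
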(event Custom|DestroyThis
  (bind _as_bp_player (Variables|Default|GetAs%20BP%20Player))
  (bind _charactermovement (Variables|/Script/Engine.Character|GetCharacterMovement _as_bp_player))
  (Pawn|Components|CharacterMovement|SetMovementMode _charactermovement "MOVE_Walking" 0)
  (Variables|/Game/Blueprints/Player/BP_Player.BP_Player_C|SetMovementType _as_bp_player "NewEnumerator0")
  (Components|SkeletalMesh|SetSkeletalMeshAsset (Variables|/Script/Engine.Character|GetMesh _as_bp_player) "/Game/TestCharAssets/Meshes/SK_Devvy_M.SK_Devvy_M")
  (Variables|/Script/Engine.CharacterMovementComponent|SetbOrientRotationToMovement _charactermovement true)
  (Variables|/Script/Engine.CharacterMovementComponent|SetMaxFlySpeed _charactermovement (Variables|Default|GetDefaultFlyingSpeed))
  (Variables|/Script/Engine.CharacterMovementComponent|SetMaxAcceleration _charactermovement (Variables|Default|GetDefaultMaxAcceleration))
  (Variables|/Script/Engine.SpringArmComponent|SetbUsePawnControlRotation (Variables|/Game/Blueprints/Player/BP_Player.BP_Player_C|GetSpringArm (Variables|Default|GetAs%20BP%20Player)) true)
  (Components|DestroyComponent))

(event Custom|EndTeleport
  (Utilities|Time|ClearandInvalidateTimerbyHandle (stale EventBeginPlay _returnvalue))
  (CallFunction|DestroyThis))

(event EventBeginPlay
  (bind _asbp_player (Utilities|Casting|CastToBP_Player (Components|GetOwner)))
  (bind _output_get (Variables|Default|SetAs%20BP%20Player _asbp_player))
  (CallFunction|InitiateTeleport)
  (bind _returnvalue (Utilities|Time|SetTimerbyEvent (delegate Custom|DestroyThis) (Variables|Default|GetFlyingTime)))
  (Variables|Default|SetDefaultFlyingSpeed (Variables|/Script/Engine.CharacterMovementComponent|GetMaxFlySpeed (Variables|/Script/Engine.Character|GetCharacterMovement _output_get)))
  (Variables|Default|SetDefaultMaxAcceleration (Class|CharacterMovementComponent|GetMaxAcceleration (Variables|/Script/Engine.Character|GetCharacterMovement _output_get))))

(event EventTick
  (params (DeltaSeconds :type Float%20%28single-precision%29))
  (bind _as_bp_player (Variables|Default|GetAs%20BP%20Player))
  (Pawn|Input|AddMovementInput _as_bp_player (Math|Vector|GetForwardVector (Variables|/Script/Engine.Character|GetCapsuleComponent _as_bp_player)) (Variables|Default|GetTeleportForwardSpeed) false))

(fn InitiateTeleport
  (bind _as_bp_player (Variables|Default|GetAs%20BP%20Player))
  (bind _charactermovement (Variables|/Script/Engine.Character|GetCharacterMovement _as_bp_player))
  (Variables|/Script/Engine.CharacterMovementComponent|SetbOrientRotationToMovement (Variables|/Script/Engine.Character|GetCharacterMovement _as_bp_player) false)
  (Transformation|SetActorRotation _as_bp_player (Math|Rotator|MakeRotator 0.0 0.0 (.yaw (Variables|Default|GetDirection))))
  (Variables|/Script/Engine.SpringArmComponent|SetbUsePawnControlRotation (Variables|/Game/Blueprints/Player/BP_Player.BP_Player_C|GetSpringArm _as_bp_player) false)
  (Components|SkeletalMesh|SetSkeletalMeshAsset (Variables|/Script/Engine.Character|GetMesh _as_bp_player) "/Game/Art/Characters/PlayerBall/SphereWithBone.SphereWithBone")
  (Pawn|Components|CharacterMovement|SetMovementMode _charactermovement "MOVE_Flying" 0)
  (Variables|/Game/Blueprints/Player/BP_Player.BP_Player_C|SetMovementType (Variables|Default|GetAs%20BP%20Player) "NewEnumerator4")
  (Variables|/Script/Engine.CharacterMovementComponent|SetMaxFlySpeed _charactermovement (Variables|Default|GetTeleportFlyingSpeed))
  (Variables|/Script/Engine.CharacterMovementComponent|SetMaxAcceleration _charactermovement (Variables|Default|GetTeleportMaxAcceleration)))