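; Player component that lets the character pick up, carry and drop PickUpCube actors with the IA_PickUp input.
; When inside a cube radius, RadiusCheck picks the cube hit by a short forward line trace, or searches CurrentCubes by distance if nothing is hit.
; The owner's PhysicsHandle grabs the cube, and Tick holds it in front of the owner, facing forward.
; ArrayCheck clears the in-radius flag when CurrentCubes is empty.
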(event Custom|Pickup_Event
  (bind _currentcube (Variables|Default|GetCurrentCube))
  (bind _cube (Variables|/Game/Blueprints/Mechanics/Actor/PickUpCube.PickUpCube_C|GetCube _currentcube))
  (Physics|Components|PhysicsHandle|GrabComponentatLocationwithRotation (Variables|Default|GetMyHandle) _cube "None" (Transformation|GetWorldLocation _cube) (Math|Rotator|MakeRotfromX (Transformation|GetActorForwardVector (Components|GetOwner)))))

(event Input|EnhancedActionEvents|EnhancedInputActionIA_PickUp
  (params (ActionValue :type Boolean) (ElapsedSeconds :type Float%20%28double-precision%29) (TriggeredSeconds :type Float%20%28double-precision%29) (InputAction :type Input%20Action%20Object%20Reference :default "/Game/Inputs/InputActions/IA_PickUp.IA_PickUp"))
  (:Started
    (if (Variables|Default|GetPickedUp)
      (Variables|Default|SetPickedUp false)
      (Development|PrintString "Dropped")
      (Physics|Components|PhysicsHandle|ReleaseComponent (Variables|Default|GetMyHandle))
      (elif (Variables|Default|GetInCubeRadius)
        (CallFunction|RadiusCheck)))))

(event EventBeginPlay
  (Variables|Default|SetMyHandle (Actor|GetComponentbyClass (Components|GetOwner) "/Script/Engine.PhysicsHandleComponent")))

(event EventTick
  (params (DeltaSeconds :type Float%20%28single-precision%29))
  (bind _returnvalue (Components|GetOwner))
  (bind _returnvalue_2 (Transformation|GetActorForwardVector _returnvalue))
  (if (Variables|Default|GetPickedUp)
    (Class|PhysicsHandleComponent|SetTargetLocationandRotation (Variables|Default|GetMyHandle) (+ (* _returnvalue_2 1e+02) (Transformation|GetActorLocation _returnvalue)) (Math|Rotator|MakeRotfromX _returnvalue_2))))

(fn RadiusCheck
  (bind _returnvalue (Game|GetPlayerCharacter 0))
  (bind _returnvalue_2 (Transformation|GetActorLocation _returnvalue))
  (Variables|Default|SetCurrentCube 0)
  (bind (_outhit _returnvalue_3) (Collision|LineTraceByChannel _returnvalue_2 (+ _returnvalue_2 (* (Math|Vector|Normalize (Transformation|GetActorForwardVector _returnvalue)) 7e+01)) "TraceTypeQuery1" false 0 "None"))
  (if _returnvalue_3
    (bind _aspick_up_cube (Utilities|Casting|CastToPickUpCube (.hitactor _outhit)))
    (Variables|Default|SetCurrentCube _aspick_up_cube)
    (else
      (for _array_element (Variables|Default|GetCurrentCubes)
        (if (< (Transformation|GetDistanceTo _array_element (Game|GetPlayerCharacter 0)) (LocalVariables|GetClosest%20Distance))
          (Variables|Default|SetCurrentCube _array_element)
          (LocalVariables|SetClosest%20Distance (Transformation|GetDistanceTo _array_element (Game|GetPlayerCharacter 0)))))))
  (Utilities|IsValid (Variables|Default|GetCurrentCube)
    (:Is%20Valid
      (Variables|Default|SetPickedUp true)
      (CallFunction|PickupEvent))))

(fn ArrayCheck
  (if (== (Utilities|Array|Length (Variables|Default|GetCurrentCubes)) 0)
    (Variables|Default|SetInCubeRadius false)))