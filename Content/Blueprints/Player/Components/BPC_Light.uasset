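; Player component that lets BP_Player pick up a light and throw it.
; Interact finds a nearby LightPickup by sphere overlap, uses it, and attaches a spawned LightProjectile to the mesh's PickupSocket.
; Releasing Aim after a short hold, or ThrowEvent once ReadytoThrow has fired, launches it.
; A camera trace sets the throw target, so the projectile flies from the socket toward the aimed point.
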(event Custom|ThrowEvent
  (bind _as_bp_player (Variables|Default|GetAs%20BP%20Player))
  (bind _heldlight (Variables|Default|GetHeldLight))
  (bind _returnvalue (Pawn|GetControlRotation _as_bp_player :!class /Script/Engine.Pawn))
  (bind _projectilemovement (Variables|/Game/Blueprints/Level/Puzzles/LightBridge/LightProjectile.LightProjectile_C|GetProjectileMovement _heldlight))
  (bind _camera (Variables|/Game/Blueprints/Player/BP_Player.BP_Player_C|GetCamera _as_bp_player))
  (bind _returnvalue_2 (Transformation|GetWorldLocation _camera))
  (if (and (Variables|Default|GetHolding) (Variables|Default|GetThrow))
    (Utilities|FlowControl|Delay 0.15)
    (bind (_outhit _returnvalue_3) (Collision|LineTraceByChannel _returnvalue_2 (+ _returnvalue_2 (* (Math|Vector|GetForwardVector _returnvalue) 1e+04)) "TraceTypeQuery1" false 0 "None"))
    (Variables|/Script/Engine.MovementComponent|SetVelocity _projectilemovement (* (Math|Vector|Normalize (- (Math|Vector|SelectVector (.location _outhit) (.traceend _outhit) _returnvalue_3) (Transformation|GetActorLocation _heldlight))) 2e+03))
    (Transformation|SetActorRotation _heldlight _returnvalue)
    (Components|Activation|Activate _projectilemovement false)
    (Transformation|DetachFromActor _heldlight "KeepWorld" "KeepWorld" "KeepWorld")
    (Variables|Default|SetHolding false)))

(event Input|EnhancedActionEvents|EnhancedInputActionIA_Interact
  (params (ActionValue :type Boolean) (ElapsedSeconds :type Float%20%28double-precision%29) (TriggeredSeconds :type Float%20%28double-precision%29) (InputAction :type Input%20Action%20Object%20Reference :default "/Game/Inputs/InputActions/IA_Interact.IA_Interact"))
  (bind _returnvalue (Components|GetOwner))
  (bind _as_bp_player (Variables|Default|GetAs%20BP%20Player))
  (bind _mesh (Variables|/Script/Engine.Character|GetMesh _as_bp_player))
  (bind _returnvalue_2 (Transformation|GetSocketTransform _mesh "PickupSocket" "RTS_World"))
  (bind (_location _rotation) (Math|Transform|BreakTransform _returnvalue_2))
  (:Started
    (if (not (Variables|Default|GetHolding))
      (bind (_outactors _returnvalue_3) (Collision|SphereOverlapActors (Transformation|GetActorLocation _returnvalue) 5e+02 (Variables|Default|GetStatic%20Query) "/Game/Blueprints/Level/Puzzles/LightBridge/LightPickup.LightPickup_C" (Utilities|Array|MakeArray _returnvalue)))
      (if _returnvalue_3
        (bind _aslight_pickup (Utilities|Casting|CastToLightPickup (Utilities|Array|Get(acopy) _outactors)))
        (Default|Used _aslight_pickup)
        (Variables|Default|SetHolding true)
        (bind _returnvalue_4 (Game|SpawnActorfromClass "/Game/Blueprints/Level/Puzzles/LightBridge/LightProjectile.LightProjectile_C" (Math|Transform|MakeTransform _location _rotation "0.250000,0.250000,0.250000") "Undefined" "OverrideRootScale" 0 0))
        (bind _output_get (Variables|Default|SetHeldLight _returnvalue_4))
        (Transformation|AttachComponentToComponent _output_get _mesh "PickupSocket" "SnapToTarget" "SnapToTarget" "SnapToTarget" true)))))

(event Input|EnhancedActionEvents|EnhancedInputActionIA_Aim
  (params (ActionValue :type Boolean) (ElapsedSeconds :type Float%20%28double-precision%29) (TriggeredSeconds :type Float%20%28double-precision%29) (InputAction :type Input%20Action%20Object%20Reference :default "/Game/Inputs/InputActions/IA_Aim.IA_Aim"))
  (bind _as_bp_player (Variables|Default|GetAs%20BP%20Player))
  (bind _heldlight (Variables|Default|GetHeldLight))
  (bind _returnvalue (Pawn|GetControlRotation _as_bp_player :!class /Script/Engine.Pawn))
  (bind _projectilemovement (Variables|/Game/Blueprints/Level/Puzzles/LightBridge/LightProjectile.LightProjectile_C|GetProjectileMovement _heldlight))
  (bind _camera (Variables|/Game/Blueprints/Player/BP_Player.BP_Player_C|GetCamera _as_bp_player))
  (bind _returnvalue_2 (Transformation|GetWorldLocation _camera))
  (:Completed
    (if (Variables|Default|GetHolding)
      (if (> ElapsedSeconds 0.2)
        (bind (_outhit _returnvalue_3) (Collision|LineTraceByChannel _returnvalue_2 (+ _returnvalue_2 (* (Math|Vector|GetForwardVector _returnvalue) 1e+04)) "TraceTypeQuery1" false 0 "None"))
        (Variables|/Script/Engine.MovementComponent|SetVelocity _projectilemovement (* (Math|Vector|Normalize (- (Math|Vector|SelectVector (.location _outhit) (.traceend _outhit) _returnvalue_3) (Transformation|GetActorLocation _heldlight))) 2e+03))
        (Transformation|SetActorRotation _heldlight _returnvalue)
        (Components|Activation|Activate _projectilemovement false)
        (Transformation|DetachFromActor _heldlight "KeepWorld" "KeepWorld" "KeepWorld")
        (Variables|Default|SetHolding false)))))

(event EventBeginPlay
  (bind _asbp_player (Utilities|Casting|CastToBP_Player (Components|GetOwner)))
  (Variables|Default|SetAs%20BP%20Player _asbp_player))

(event EventTick
  (params (DeltaSeconds :type Float%20%28single-precision%29)))

(event EventReadytoThrow
  (Variables|Default|SetThrow true))

(fn IsHolding
  (return (Variables|Default|GetHolding)))