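; A player debug component that adds a Debug Enhanced Input mapping context on BeginPlay to provide cheat controls.
; One action flips visibility on every actor implementing the DebugVisible interface.
; Another runs once to save all Forest, Cave and Beach levels as unlocked through the GameInstance, and destroys WorldBlock-tagged actors when in HubWorld.
; A check to remove the component in Shipping builds exists but is disconnected, so it never runs.
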(event Input|EnhancedActionEvents|EnhancedInputActionIA_DebugVis
  (params (ActionValue :type Boolean) (ElapsedSeconds :type Float%20%28double-precision%29) (TriggeredSeconds :type Float%20%28double-precision%29) (InputAction :type Input%20Action%20Object%20Reference :default "/Game/Inputs/DebugActions/IA_DebugVis.IA_DebugVis"))
  (bind _outactors (Actor|GetAllActorswithInterface "/Game/DebugStuff/DebugVisible.DebugVisible_C"))
  (for _array_element _outactors
    (Class|DebugVisible|FlipVisible(Message) _array_element)))

(event Input|EnhancedActionEvents|EnhancedInputActionIA_DebugAllLevels
  (params (ActionValue :type Boolean) (ElapsedSeconds :type Float%20%28double-precision%29) (TriggeredSeconds :type Float%20%28double-precision%29) (InputAction :type Input%20Action%20Object%20Reference :default "/Game/Inputs/DebugActions/IA_DebugAllLevels.IA_DebugAllLevels"))
  (:Started
    (Utilities|FlowControl|DoOnce false
      (:Completed
        (Class|BPISaveGameInterface|SaveLevel(Message) (Game|GetGameInstance) (Utilities|Array|MakeArray "ForestLevel1Main" "ForestLevel2Main" "ForestLevelBossMain" "CaveLevel1Main" "CaveLevel2Main" "CaveLevelBossMain" "BeachLevel1Main" "BeachLevel2Main" "BeachLevelBossMain "))
        (Development|PrintString "All unlocked")
        (bind _returnvalue (Game|GetCurrentLevelName true))
        (if (Utilities|Enum|Equal(Enum) _returnvalue "HubWorld")
          (bind _outactors (Actor|GetAllActorswithTag "WorldBlock"))
          (for _array_element _outactors
            (Actor|DestroyActor _array_element)))))))

(event EventBeginPlay
  (Input|AddMappingContext (PlayerController|LocalPlayerSubsystems|GetEnhancedInputLocalPlayerSubsystem (Game|GetPlayerController 0)) "/Game/Inputs/DebugActions/Debug.Debug" 0 "(bIgnoreAllPressedKeysUntilRelease=True,bForceImmediately=False,bNotifyUserSettings=False)"))

(event EventTick
  (params (DeltaSeconds :type Float%20%28single-precision%29)))