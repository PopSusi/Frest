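; Player component for picking up, carrying, dropping and throwing goo pods.
; The pickup input drops the held pod or searches nearby for goo plants, then loose pods; AttachPlant spawns new pods on the mesh's pickup socket.
; The projectile input aims by hold or tap-toggle, showing a timer-updated spline actor as the arc.
; Throwing requires a ready flag and launches the pod along control rotation, scaled by its force modifier.
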(event Custom|Throw
  (bind _playerref (Variables|Default|GetPlayerRef))
  (bind _forcemodification (Variables|Default|GetForceModification))
  (bind _playerref_2 (Variables|Default|GetPlayerRef))
  (bind _throwvelocity (Variables|Default|GetThrowVelocity))
  (bind _returnvalue (Transformation|GetActorLocation _playerref))
  (bind _returnvalue_2 (Pawn|GetControlRotation _playerref_2 :!class /Script/Engine.Pawn))
  (bind _returnvalue_3 (Math|Vector|GetForwardVector _returnvalue_2))
  (bind _returnvalue_4 (* _returnvalue_3 _throwvelocity))
  (bind _returnvalue_5 (* _returnvalue_4 _forcemodification))
  (if (and (Variables|Default|GetHolding) (Variables|Default|GetThrowBool))
    (Variables|/Game/Blueprints/Mechanics/Actor/BP_GooPod.BP_GooPod_C|SetActive (Variables|Default|GetCurrentPod) true)
    (Utilities|FlowControl|Delay 0.15)
    (Default|EnableNiagara (Variables|Default|GetCurrentPod))
    (Audio|PlaySound2D "/Game/Sounds/SFX/Movement/DoubleJump.DoubleJump" 1.0 1.0 0.0 0 0)
    (Default|Detach (Variables|Default|GetCurrentPod))
    (Class|PrimitiveComponent|SetAllPhysicsLinearVelocity (Variables|/Game/Blueprints/Mechanics/Actor/BP_GooPod.BP_GooPod_C|GetSphere (Variables|Default|GetCurrentPod)) "0, 0, 0" false)
    (Physics|AddImpulse (Variables|/Game/Blueprints/Mechanics/Actor/BP_GooPod.BP_GooPod_C|GetSphere (Variables|Default|GetCurrentPod)) _returnvalue_5 "None" true)
    (Collision|BoxTraceByChannel _returnvalue (+ _returnvalue_5 _returnvalue) "0, 0, 0" "0, 0, 0" "TraceTypeQuery1" false 0 "None")
    (Variables|Default|SetCurrentPod 0)
    (Variables|Default|SetHolding false)
    (Default|ExitState (Variables|Default|GetPlayerRef) "NewEnumerator0" "NewEnumerator9")))

(event Input|EnhancedActionEvents|EnhancedInputActionIA_PickUp
  (params (ActionValue :type Boolean) (ElapsedSeconds :type Float%20%28double-precision%29) (TriggeredSeconds :type Float%20%28double-precision%29) (InputAction :type Input%20Action%20Object%20Reference :default "/Game/Inputs/InputActions/IA_PickUp.IA_PickUp"))
  (bind _returnvalue (Components|GetOwner))
  (bind _pickupradius (Variables|Default|GetPickUpRadius))
  (bind _playerref (Variables|Default|GetPlayerRef))
  (bind _returnvalue_2 (Transformation|GetActorLocation _returnvalue))
  (:Started
    ;[1 1 1] Check if holding goo pod
    (if (Variables|Default|GetHolding)
      ;[1 1 1] If holding, drop
      (Default|Detach (Variables|Default|GetCurrentPod))
      (Variables|Default|SetHolding false)
      (else
        ;[1 1 1] Check area for goo plants
        (bind (_outactors _returnvalue_3) (Collision|SphereOverlapActors _returnvalue_2 _pickupradius (Variables|Default|GetStatic%20Query) "/Game/Blueprints/Mechanics/Actor/BP_GooPlant.BP_GooPlant_C" (Utilities|Array|MakeArray _returnvalue)))
        ;[1 1 1] If true, cast and attempt pickup
        (if _returnvalue_3
          (bind _array_element (Utilities|Array|ForEachLoopwithBreak _outactors :!label _label)
            (:LoopBody
              (bind _asbp_goo_plant (Utilities|Casting|CastToBP_GooPlant _array_element))
              (bind _pickedup (Default|Pickup _asbp_goo_plant self))
              (if _pickedup
                (Variables|Default|SetForceModification (Variables|/Game/Blueprints/Mechanics/Actor/BP_GooPlant.BP_GooPlant_C|GetForceModification _asbp_goo_plant))
                (if (Utilities|Enum|Equal(Enum) (Variables|/Game/Blueprints/Player/BP_Player.BP_Player_C|GetMovementType (Variables|Default|GetPlayerRef)) "NewEnumerator9")
                  (CallFunction|ActivateArc)
                  (goto _label Break)
                  (else
                    (goto _label Break)))
                (else
                  _)))))
        ;[1 1 1] If not goo plant, see if goo pod is nearby
        (bind _outactors_2 (Collision|SphereOverlapActors _returnvalue_2 _pickupradius (Utilities|Array|MakeArray "ObjectTypeQuery2") "/Game/Blueprints/Mechanics/Actor/BP_GooPod.BP_GooPod_C"))
        (bind _array_element_2 (Utilities|Array|ForEachLoopwithBreak _outactors_2 :!label _label_2)
          (:LoopBody
            (bind _asbp_goo_pod (Utilities|Casting|CastToBP_GooPod _array_element_2))
            (Variables|Default|SetCurrentPod _asbp_goo_pod)
            (Variables|Default|SetForceModification (Variables|/Game/Blueprints/Mechanics/Actor/BP_GooPod.BP_GooPod_C|GetForceMod _asbp_goo_pod))
            (Default|PickBackUp _asbp_goo_pod _playerref)
            (if (Utilities|Enum|Equal(Enum) (Variables|/Game/Blueprints/Player/BP_Player.BP_Player_C|GetMovementType _playerref) "NewEnumerator9")
              (CallFunction|ActivateArc))
            (Variables|Default|SetHolding true)
            (Development|PrintString "Pickup GooPod")
            (goto _label_2 Break)))))))

(event Input|EnhancedActionEvents|EnhancedInputActionIA_Projectile
  (params (ActionValue :type Boolean) (ElapsedSeconds :type Float%20%28double-precision%29) (TriggeredSeconds :type Float%20%28double-precision%29) (InputAction :type Input%20Action%20Object%20Reference :default "/Game/Inputs/InputActions/IA_Projectile.IA_Projectile"))
  (:Started
    (if (Variables|Default|GetHolding)
      (if (Variables|/Game/Blueprints/Player/BP_Player.BP_Player_C|GetTapAim (Variables|Default|GetPlayerRef))
        (Utilities|FlowControl|FlipFlop
          (:A
            _)
          (:B
            (CallFunction|RemoveArc :!label _label)
            (CallFunction|Throw)
            (goto _label_2 Reset))))
      (Default|EnterState (Variables|Default|GetPlayerRef) "NewEnumerator9" true "NewEnumerator0")
      (Utilities|FlowControl|DoOnce false :!label _label_2
        (:Completed
          (CallFunction|ActivateArc)))))
  (:Canceled
    (if (not (Variables|/Game/Blueprints/Player/BP_Player.BP_Player_C|GetTapAim (Variables|Default|GetPlayerRef))) :!label _label_3
      (goto _label)))
  (:Completed
    (goto _label_3)))

(event EventBeginPlay
  (bind _returnvalue (Components|GetOwner))
  (bind _asbp_player (Utilities|Casting|CastToBP_Player _returnvalue))
  (Variables|Default|SetPlayerRef _asbp_player)
  (Variables|Default|SetCamera (Actor|GetComponentbyClass _returnvalue "/Script/Engine.CameraComponent")))

(event EventTick
  (params (DeltaSeconds :type Float%20%28single-precision%29)))

(event EventReadytoThrow
  (Variables|Default|SetThrowBool true))

(fn AttachPlant
  (params (Type%20of%20Pod :type E_MovementModifications%20Enum :default "NewEnumerator0"))
  (bind _playerref (Variables|Default|GetPlayerRef))
  (bind _mesh (Variables|/Script/Engine.Character|GetMesh _playerref))
  (bind _returnvalue (Transformation|GetSocketTransform _mesh "PickupSocket" "RTS_World"))
  (bind (_location _rotation) (Math|Transform|BreakTransform _returnvalue))
  ;[1 1 1] Spawn and move BP_GooPod to socket
  (bind _returnvalue_2 (Game|SpawnActorfromClass "/Game/Blueprints/Mechanics/Actor/BP_GooPod.BP_GooPod_C" (Math|Transform|MakeTransform _location _rotation "0.250000,0.250000,0.250000") "Undefined" "OverrideRootScale" 0 0))
  (bind _output_get (Variables|Default|SetCurrentPod _returnvalue_2))
  ;[1 1 1] Attach
  (Variables|/Game/Blueprints/Mechanics/Actor/BP_GooPod.BP_GooPod_C|SetType _output_get Type%20of%20Pod)
  (Transformation|AttachComponentToComponent _output_get _mesh "PickupSocket" "SnapToTarget" "SnapToTarget" "SnapToTarget" true)
  (Variables|Default|SetHolding true))

(fn AttemptDrop
  (bind _currentpod (Variables|Default|GetCurrentPod))
  (Utilities|IsValid _currentpod
    (:Is%20Valid
      (Default|Detach _currentpod)
      (Variables|Default|SetHolding false))))

(fn RemoveArc
  (bind _currentvisualization (Variables|Default|GetCurrentVisualization))
  (bind _staticmesh (Variables|/Game/Blueprints/Player/Components/Spline.Spline_C|GetStaticMesh _currentvisualization))
  (Utilities|IsValid _currentvisualization
    (:Is%20Valid
      (if (Rendering|IsVisible _staticmesh)
        (Rendering|SetVisibility _staticmesh false false)
        (Utilities|Time|ClearandInvalidateTimerbyHandle (Variables|Default|GetUpdateVisualTimer))))))

(fn ActivateArc
  (Utilities|IsValid (Variables|Default|GetCurrentVisualization)
    (:Is%20Valid
      _)
    (:Is%20Not%20Valid
      (bind _returnvalue (Game|SpawnActorfromClass "/Game/Blueprints/Player/Components/Spline.Spline_C" (Math|Transform|MakeTransform "0, 0, 0" "0, 0, 0" "1.000000,1.000000,1.000000") "Undefined" "MultiplyWithRoot" 0 0))
      (Variables|Default|SetCurrentVisualization _returnvalue)))
  (Rendering|SetVisibility (Variables|/Game/Blueprints/Player/Components/Spline.Spline_C|GetStaticMesh (Variables|Default|GetCurrentVisualization)) true false)
  (bind _returnvalue_2 (Utilities|Time|SetTimerbyFunctionName 0 "UpdateVisualization" 0.02 true))
  (Variables|Default|SetUpdateVisualTimer _returnvalue_2))

(fn UpdateVisualization
  (bind _camera (Variables|Default|GetCamera))
  (bind _returnvalue (Math|Vector|GetForwardVector _camera))
  (bind (_x _y) (Math|Vector|BreakVector _returnvalue))
  (Transformation|SetActorLocationAndRotation (Variables|Default|GetCurrentVisualization) (Transformation|GetActorLocation (Variables|Default|GetCurrentPod)) (Pawn|GetControlRotation (Variables|Default|GetPlayerRef) :!class /Script/Engine.Pawn))
  (Collision|LineTraceByChannel (Transformation|GetWorldLocation _camera) (Math|Vector|MakeVector _x _y 0.0) "TraceTypeQuery1" false 0 "None"))

(fn IsHolding
  (return (Variables|Default|GetHolding)))