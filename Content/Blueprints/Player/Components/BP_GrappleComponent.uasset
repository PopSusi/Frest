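; Player component that finds the grapple point the camera faces and activates it on the player.
; Each tick, a sphere trace around the owner gathers candidates, keeping the one best aligned with camera forward by dot product above a threshold.
; A visibility line trace confirms the detected point is unobstructed, then a newly detected BP_GrapplePoint is stored on BP_Player and activated.
; The detected point and active reference are never cleared in live logic.
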(event EventBeginPlay
  (bind _returnvalue (Components|GetOwner))
  (Variables|Default|SetCamera (Actor|GetComponentbyClass _returnvalue "/Script/Engine.CameraComponent"))
  (bind _asbp_player (Utilities|Casting|CastToBP_Player _returnvalue))
  (Variables|Default|SetPlayerRef _asbp_player))

(event EventTick
  (params (DeltaSeconds :type Float%20%28single-precision%29))
  (CallFunction|CheckforGrapplePoints))

(fn ActivateGrapplePoint
  (Utilities|IsValid (Variables|Default|GetDetectedGrapplePoint)
    (:Is%20Valid
      (bind _outhit (Collision|LineTraceByChannel (Transformation|GetWorldLocation (Variables|Default|GetCamera)) (Transformation|GetActorLocation (Variables|Default|GetDetectedGrapplePoint)) "TraceTypeQuery1" false 0 "None"))
      (if (== (.hitactor _outhit) (Variables|Default|GetDetectedGrapplePoint))
        (if (!= (Variables|Default|GetDetectedGrapplePoint) (Variables|Default|GetGrapplePointRef))
          (bind _asbp_grapple_point (Utilities|Casting|CastToBP_GrapplePoint (Variables|Default|GetDetectedGrapplePoint)))
          (bind _output_get (Variables|Default|SetGrapplePointRef _asbp_grapple_point))
          (Variables|/Game/Blueprints/Player/BP_Player.BP_Player_C|SetGrapplePoint (Variables|Default|GetPlayerRef) _asbp_grapple_point)
          (Default|Activate _output_get (Variables|Default|GetPlayerRef)))))
    (:Is%20Not%20Valid
      (Variables|Default|SetGrapplePointAvailable false))))

(fn CheckforGrapplePoints
  (bind _returnvalue (Components|GetOwner))
  (bind _camera (Variables|Default|GetCamera))
  (bind _returnvalue_2 (Transformation|GetActorLocation _returnvalue))
  (bind _outhits (Collision|MultiSphereTraceForObjects _returnvalue_2 _returnvalue_2 (Variables|Default|GetGrappleDetectionRadius) (Utilities|Array|MakeArray "ObjectTypeQuery7") false 0 "None"))
  (Variables|Default|SetGrappleHighestDotProduct 0.7)
  (for _array_element _outhits
    (if (> (Math|Vector|DotProduct (Math|Vector|GetForwardVector _camera) (Math|Vector|GetUnitDirection(Vector) (Transformation|GetWorldLocation _camera) (Transformation|GetActorLocation (.hitactor _array_element)))) (Variables|Default|GetGrappleHighestDotProduct))
      (Variables|Default|SetGrapplePointAvailable true)
      (Variables|Default|SetGrappleHighestDotProduct (Math|Vector|DotProduct (Math|Vector|GetForwardVector _camera) (Math|Vector|GetUnitDirection(Vector) (Transformation|GetWorldLocation _camera) (Transformation|GetActorLocation (.hitactor _array_element)))))
      (Variables|Default|SetDetectedGrapplePoint (.hitactor _array_element))
      (else
        (Variables|Default|SetGrapplePointAvailable false))))
  (CallFunction|ActivateGrapplePoint))