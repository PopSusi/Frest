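; Player character that routes Enhanced Input through a MovementType state for walking, crouching, falling, climbing, wall sliding, rope swinging and teleporting.
; JumpCheck picks normal, charged crouch, air, wall or swing-release jumps by state.
; Tagged overlaps drive BP_WallClimbing, a capsule trace while falling starts wall slides, and grappling toggles capsule physics with a cable.
; Also handles pausing, NPC talk and laser rotation via overlaps, and checkpoint save data.
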(event OnComponentBeginOverlap(WallClimbChecker)
  (params (OverlappedComponent :type Primitive%20Component%20Object%20Reference) (OtherActor :type Actor%20Object%20Reference) (OtherComp :type Primitive%20Component%20Object%20Reference) (OtherBodyIndex :type Integer) (bFromSweep :type Boolean) (SweepResult :type Hit%20Result%20Structure%20%28by%20ref%29))
  (bind _returnvalue (Actor|GetComponentbyClass "/Game/Blueprints/Player/Components/BP_WallClimbing.BP_WallClimbing_C"))
  (if (Components|ComponentHasTag OtherComp "Climb")
    (if (AI|Components|NavMovement|IsFalling (Variables|Character|GetCharacterMovement))
      (Utilities|IsValid _returnvalue
        (:Is%20Valid
          (Default|InitiateWallClimb _returnvalue "0, 0, 0")
          (Variables|Default|SetMovementType "NewEnumerator1"))))))

(event OnComponentEndOverlap(WallClimbChecker)
  (params (OverlappedComponent :type Primitive%20Component%20Object%20Reference) (OtherActor :type Actor%20Object%20Reference) (OtherComp :type Primitive%20Component%20Object%20Reference) (OtherBodyIndex :type Integer))
  (bind _returnvalue (Actor|GetComponentbyClass "/Game/Blueprints/Player/Components/BP_WallClimbing.BP_WallClimbing_C"))
  (if (Components|ComponentHasTag OtherComp "Climb")
    (Utilities|IsValid _returnvalue
      (:Is%20Valid
        (Default|EndWallClimb _returnvalue)
        (Variables|Default|SetMovementType "NewEnumerator7")))))

(event Custom|ResetWallJumpDelay
  (Variables|Default|SetCanDJump true)
  (Variables|/Script/Engine.CharacterMovementComponent|SetAirControl (Variables|Character|GetCharacterMovement) 0.5))

(event Custom|StartCrouch
  (Variables|Default|SetIsCrouching true)
  (Variables|/Script/Engine.CharacterMovementComponent|SetMaxWalkSpeed (Variables|Character|GetCharacterMovement) 3e+02)
  (switch Utilities|FlowControl|Switch|SwitchonEnum_MovementMode (Variables|Default|GetMovementType)
    (:NewEnumerator0
      (Variables|Default|SetMovementType "NewEnumerator6")
      (Development|PrintString (Utilities|String|EnumtoString (Variables|Default|GetMovementType))))))

(event Custom|EndCrouch
  (Variables|Default|SetIsCrouching false)
  (Variables|/Script/Engine.CharacterMovementComponent|SetMaxWalkSpeed (Variables|Character|GetCharacterMovement) (Variables|Default|GetDefaultWalkSpeed))
  (Variables|Default|SetCrouchHoldTime 0.0)
  (Variables|Default|SetMovementType "NewEnumerator0")
  (Development|PrintString (Utilities|String|EnumtoString (Variables|Default|GetMovementType))))

(event Input|EnhancedActionEvents|EnhancedInputActionIA_Talk
  (params (ActionValue :type Boolean) (ElapsedSeconds :type Float%20%28double-precision%29) (TriggeredSeconds :type Float%20%28double-precision%29) (InputAction :type Input%20Action%20Object%20Reference :default "/Game/Inputs/InputActions/IA_Talk.IA_Talk"))
  (bind _overlappingactors (Collision|GetOverlappingActors 0 :!class /Script/Engine.Actor))
  ;[1 1 1] Press R to talk to NPCs when in range. Movement is disabled until NPC dialogue is over - Ryan
  (:Started
    (for _array_element _overlappingactors
      (if (Utilities|DoesObjectImplementInterface _array_element "/Game/Blueprints/NPCs/BPI_Dialogue.BPI_Dialogue_C")
        (Pawn|Components|CharacterMovement|DisableMovement (Variables|Character|GetCharacterMovement))
        (Class|BPIDialogue|Talk(Message) _array_element)))
    (bind _array_element_2 (Utilities|Array|ForEachLoopwithBreak _overlappingactors)
      (:LoopBody
        (if (Utilities|DoesObjectImplementInterface _array_element_2 "/Game/Blueprints/Level/Puzzles/BP_LaserInterface.BP_LaserInterface_C")
          (Utilities|FlowControl|DoOnce false :!label _label
            (:Completed
              (bind _asbp_laser_interface (Utilities|Casting|CastToBP_LaserInterface _array_element_2))
              (Default|Rotate _asbp_laser_interface)))))))
  (:Canceled
    (goto _label Reset))
  (:Completed
    (goto _label Reset)))

(event Input|EnhancedActionEvents|EnhancedInputActionIA_Pause
  (params (ActionValue :type Boolean) (ElapsedSeconds :type Float%20%28double-precision%29) (TriggeredSeconds :type Float%20%28double-precision%29) (InputAction :type Input%20Action%20Object%20Reference :default "/Game/Inputs/InputActions/IA_Pause.IA_Pause"))
  (bind _returnvalue (Game|GetPlayerController 0))
  ;[1 1 1] Pause Menu - Ryan
  (:Started
    (if (not (Variables|Default|GetIsPaused))
      (Variables|Default|SetIsPaused true)
      (Utilities|IsValid (Variables|Default|GetPauseMenu)
        (:Is%20Valid
          _)
        (:Is%20Not%20Valid
          (bind _returnvalue_2 (UserInterface|CreateWidget "/Game/UI/Widgets/Menus/WB_Pause.WB_Pause_C" _returnvalue))
          (bind _output_get (Variables|Default|SetPauseMenu _returnvalue_2))))
      (UserInterface|Viewport|AddtoViewport _output_get 0)
      (Input|SetInputModeGameandUI _returnvalue (Variables|Default|GetPauseMenu) "DoNotLock" true false)
      (Variables|/Script/Engine.PlayerController|SetbShowMouseCursor (Game|GetPlayerController 0) true)
      (Game|SetGamePaused true)
      (Utilities|FlowControl|Sequence
        (:then_0
          (Utilities|IsValid (Variables|Default|GetCodexMenu)
            (:Is%20Not%20Valid
              (bind _returnvalue_3 (UserInterface|CreateWidget "/Game/UI/Widgets/WB_Codex.WB_Codex_C"))
              (Variables|Default|SetCodexMenu _returnvalue_3))))
        (:then_1
          (Utilities|IsValid (Variables|Default|GetLevelSelectMenu)
            (:Is%20Not%20Valid
              (bind _returnvalue_4 (UserInterface|CreateWidget "/Game/UI/Widgets/Menus/WB_LevelSelect.WB_LevelSelect_C"))
              (Variables|Default|SetLevelSelectMenu _returnvalue_4)))))
      (else
        (Variables|Default|SetIsPaused false)
        (Widget|RemovefromParent (Variables|Default|GetPauseMenu))
        (Game|SetGamePaused false)
        (Input|SetInputModeGameOnly _returnvalue false)
        (Variables|/Script/Engine.PlayerController|SetbShowMouseCursor _returnvalue false)))))

(event Input|EnhancedActionEvents|EnhancedInputActionIA_Crouch
  (params (ActionValue :type Boolean) (ElapsedSeconds :type Float%20%28double-precision%29) (TriggeredSeconds :type Float%20%28double-precision%29) (InputAction :type Input%20Action%20Object%20Reference :default "/Game/Inputs/InputActions/IA_Crouch.IA_Crouch"))
  (:Triggered
    (Variables|Default|SetCrouchHoldTime ElapsedSeconds))
  (:Started
    (CallFunction|StartCrouch))
  (:Canceled
    (CallFunction|EndCrouch :!label _label))
  (:Completed
    (goto _label)))

(event Input|EnhancedActionEvents|EnhancedInputActionIA_LookH
  (params (ActionValue :type Float%20%28double-precision%29) (ElapsedSeconds :type Float%20%28double-precision%29) (TriggeredSeconds :type Float%20%28double-precision%29) (InputAction :type Input%20Action%20Object%20Reference :default "/Game/Inputs/InputActions/IA_LookH.IA_LookH"))
  ;[1 1 1] Movement
  (switch Utilities|FlowControl|Switch|SwitchonEnum_MovementMode (Variables|Default|GetMovementType)
    (:NewEnumerator0
      _)
    (:NewEnumerator1
      _)
    (:NewEnumerator2
      _)
    (:NewEnumerator5
      _)
    (:NewEnumerator6
      _)
    (:NewEnumerator7
      _))
  (Pawn|Input|AddControllerYawInput ActionValue))

(event Input|EnhancedActionEvents|EnhancedInputActionIA_LookV
  (params (ActionValue :type Float%20%28double-precision%29) (ElapsedSeconds :type Float%20%28double-precision%29) (TriggeredSeconds :type Float%20%28double-precision%29) (InputAction :type Input%20Action%20Object%20Reference :default "/Game/Inputs/InputActions/IA_LookV.IA_LookV"))
  ;[1 1 1] Movement
  (switch Utilities|FlowControl|Switch|SwitchonEnum_MovementMode (Variables|Default|GetMovementType)
    (:NewEnumerator0
      _)
    (:NewEnumerator1
      _)
    (:NewEnumerator2
      _)
    (:NewEnumerator5
      _)
    (:NewEnumerator6
      _)
    (:NewEnumerator7
      _))
  (Pawn|Input|AddControllerPitchInput ActionValue))

(event Input|EnhancedActionEvents|EnhancedInputActionIA_MoveForward
  (params (ActionValue :type Float%20%28double-precision%29) (ElapsedSeconds :type Float%20%28double-precision%29) (TriggeredSeconds :type Float%20%28double-precision%29) (InputAction :type Input%20Action%20Object%20Reference :default "/Game/Inputs/InputActions/IA_MoveForward.IA_MoveForward"))
  (bind _returnvalue (Pawn|GetControlRotation :!class /Script/Engine.Pawn))
  (bind _yaw (Math|Rotator|BreakRotator _returnvalue))
  (bind _returnvalue_2 (Math|Rotator|MakeRotator 0.0 0.0 _yaw))
  (bind _returnvalue_3 (Math|Vector|GetForwardVector _returnvalue_2))
  ;[1 1 1] Movement
  (switch Utilities|FlowControl|Switch|SwitchonEnum_MovementMode (Variables|Default|GetMovementType)
    (:NewEnumerator0
      (Pawn|Input|AddMovementInput _returnvalue_3 ActionValue false :!label _label))
    (:NewEnumerator1
      (Utilities|WallClimbUp ActionValue))
    (:NewEnumerator2
      (Physics|AddForce (Variables|Collision|GetCapsuleComponent) (* _returnvalue_3 (* ActionValue 2.5e+04)) "None" false))
    (:NewEnumerator4
      (CallFunction|TeleportMovement 0.0))
    (:NewEnumerator5
      (Pawn|Input|AddMovementInput (Math|Vector|GetUpVector _returnvalue_2) 1.0 false))
    (:NewEnumerator6
      (goto _label))
    (:NewEnumerator7
      (goto _label))))

(event Input|EnhancedActionEvents|EnhancedInputActionIA_MoveRight
  (params (ActionValue :type Float%20%28double-precision%29) (ElapsedSeconds :type Float%20%28double-precision%29) (TriggeredSeconds :type Float%20%28double-precision%29) (InputAction :type Input%20Action%20Object%20Reference :default "/Game/Inputs/InputActions/IA_MoveRight.IA_MoveRight"))
  (bind _returnvalue (Pawn|GetControlRotation :!class /Script/Engine.Pawn))
  (bind _yaw (Math|Rotator|BreakRotator _returnvalue))
  (bind _returnvalue_2 (Math|Rotator|MakeRotator 0.0 0.0 _yaw))
  (bind _returnvalue_3 (Math|Vector|GetRightVector _returnvalue_2))
  ;[1 1 1] Movement
  (switch Utilities|FlowControl|Switch|SwitchonEnum_MovementMode (Variables|Default|GetMovementType)
    (:NewEnumerator0
      (Pawn|Input|AddMovementInput _returnvalue_3 ActionValue false :!label _label))
    (:NewEnumerator1
      (goto _label))
    (:NewEnumerator2
      (Physics|AddForce (Variables|Collision|GetCapsuleComponent) (* _returnvalue_3 (* ActionValue 2.5e+04)) "None" false))
    (:NewEnumerator4
      (CallFunction|TeleportMovement ActionValue))
    (:NewEnumerator6
      (goto _label))
    (:NewEnumerator7
      (goto _label))))

(event Input|EnhancedActionEvents|EnhancedInputActionIA_Jump
  (params (ActionValue :type Boolean) (ElapsedSeconds :type Float%20%28double-precision%29) (TriggeredSeconds :type Float%20%28double-precision%29) (InputAction :type Input%20Action%20Object%20Reference :default "/Game/Inputs/InputActions/IA_Jump.IA_Jump"))
  ;[1 1 1] Movement
  (:Started
    (CallFunction|JumpCheck))
  (:Canceled
    (Character|StopJumping :!label _label))
  (:Completed
    (goto _label)))

(event Input|EnhancedActionEvents|EnhancedInputActionIA_Grapple
  (params (ActionValue :type Boolean) (ElapsedSeconds :type Float%20%28double-precision%29) (TriggeredSeconds :type Float%20%28double-precision%29) (InputAction :type Input%20Action%20Object%20Reference :default "/Game/Inputs/InputActions/IA_Grapple.IA_Grapple"))
  (bind _capsulecomponent (Variables|Collision|GetCapsuleComponent))
  (bind _cable (Variables|Default|GetCable))
  (:Started
    (Development|PrintString "Hello")
    (if (Variables|Default|GetIsSwinging)
      (Variables|Default|SetIsSwinging false)
      (Variables|Default|SetMovementType "NewEnumerator7")
      (Default|EndRopeSwing (Variables|Default|GetGrapplePoint))
      (Physics|SetSimulatePhysics _capsulecomponent false)
      (Class|CableComponent|SetAttachEndto (Variables|Default|GetCable) self "None" "None")
      (Variables|Default|SetGrapplePoint 0)
      (else
        (Utilities|IsValid (Variables|Default|GetGrapplePoint)
          (:Is%20Valid
            (Variables|Default|SetIsSwinging true)
            (Variables|Default|SetMovementType "NewEnumerator2")
            (Physics|SetSimulatePhysics _capsulecomponent true)
            (Default|StartRopeSwing (Variables|Default|GetGrapplePoint))
            (Development|SetHiddeninGame _cable false false)
            (Class|CableComponent|SetAttachEndto _cable (Variables|Default|GetGrapplePoint) "None" "None")))))))

(event EventBeginPlay
  (bind _charactermovement (Variables|Character|GetCharacterMovement))
  (Input|AddMappingContext (PlayerController|LocalPlayerSubsystems|GetEnhancedInputLocalPlayerSubsystem (Game|GetPlayerController 0)) "/Game/Inputs/InputActions/IMC_Player.IMC_Player" 0 "(bIgnoreAllPressedKeysUntilRelease=True,bForceImmediately=False,bNotifyUserSettings=False)")
  (Variables|Default|SetDefaultWalkSpeed (Variables|/Script/Engine.CharacterMovementComponent|GetMaxWalkSpeed _charactermovement))
  (Variables|Default|SetDefaultGravity (Variables|/Script/Engine.CharacterMovementComponent|GetGravityScale _charactermovement))
  (Variables|Default|SetCurrentCamera (Variables|Default|GetCamera))
  (Input|SetInputModeGameOnly (Game|GetPlayerController 0) false)
  (bind _playersave (CallFunction|GetPlayerSave))
  (Class|BPISaveGameInterface|SavePlayerData(Message) (Game|GetGameInstance) _playersave false))

(event Collision|EventActorBeginOverlap
  (params (OtherActor :type Actor%20Object%20Reference)))

(event EventTick
  (params (DeltaSeconds :type Float%20%28single-precision%29))
  (Development|PrintString (Utilities|String|ToString(Float) (Variables|Default|GetJumpKeyHoldTime)) true true "(R=0.000000,G=0.660000,B=1.000000,A=1.000000)" 0.0)
  (switch Utilities|FlowControl|Switch|SwitchonEnum_MovementMode (Variables|Default|GetMovementType)
    (:NewEnumerator7
      (if (Utilities|Enum|Equal(Enum) (Variables|Default|GetMovementType) "NewEnumerator7")
        (if (AI|Components|NavMovement|IsFalling (Variables|Character|GetCharacterMovement))
          _
          (else
            (Variables|Default|SetMovementType "NewEnumerator0")))
        (|WallJumpCheck_2)))))

(event EventOnLanded
  (params (Hit :type Hit%20Result%20Structure%20%28by%20ref%29))
  (bind _returnvalue (Actor|GetComponentbyClass "/Game/Blueprints/Player/Components/BP_WallClimbing.BP_WallClimbing_C"))
  ;[1 1 1] Movement
  (Variables|Default|SetMovementType "NewEnumerator0")
  (Variables|Default|SetJumpCount 0)
  (Variables|Default|SetIsWallSliding false)
  (CallFunction|WallSlideVelocityReset)
  (Variables|/Script/Engine.CharacterMovementComponent|SetGravityScale (Variables|Character|GetCharacterMovement) (Variables|Default|GetDefaultGravity))
  (CallFunction|EndCrouch)
  (Utilities|IsValid _returnvalue
    (:Is%20Valid
      (Default|EndWallClimb _returnvalue))))

(fn ConstructionScript)

(fn JumpCheck
  (bind _returnvalue (Transformation|GetVelocity))
  (bind _returnvalue_2 (Transformation|GetActorRotation))
  (bind _returnvalue_3 (Input|EnhancedActionValues|GetIA_MoveRight))
  (bind _returnvalue_4 (Input|EnhancedActionValues|GetIA_MoveForward))
  (bind _cable (Variables|Default|GetCable))
  (bind _camera (Variables|Default|GetCamera))
  (bind (_x _y) (Math|Vector|BreakVector _returnvalue))
  (bind _returnvalue_5 (Math|Float|Absolute(Float) _returnvalue_4))
  (bind _returnvalue_6 (Math|Float|Absolute(Float) _returnvalue_3))
  (switch Utilities|FlowControl|Switch|SwitchonEnum_MovementMode (Variables|Default|GetMovementType)
    (:NewEnumerator0
      ;[1 1 1] Normal
      (if (Variables|Default|GetIsCrouching)
        ;[1 1 1] Crouched
        (if (> (Variables|Default|GetCrouchHoldTime) 1.0) :!label _label
          (Character|LaunchCharacter (Math|Vector|MakeVector _x _y (Variables|Default|GetCrouchJumpHeight)) false false)
          (Math|Integer|IncrementInt (Variables|Default|GetJumpCount)
            (:%20%20
              (Variables|Default|SetMovementType "NewEnumerator7")
              (LocalVariables|SetFromState "From Super Jump")
              ;[1 1 1] Reports
              (Development|PrintString (Utilities|String|Append (LocalVariables|GetFromState) "  into  " (Utilities|String|EnumtoString (Variables|Default|GetMovementType))) :!label _label_2))))
        (else
          (Character|Jump :!label _label_3)
          (Math|Integer|IncrementInt (Variables|Default|GetJumpCount)
            (:%20%20
              (LocalVariables|SetFromState "From Normal Jump")
              (Variables|Default|SetMovementType "NewEnumerator7")
              (goto _label_2))))))
    (:NewEnumerator1
      ;[1 1 1] Wall Relation Check
      (Variables|Default|SetCanDJump false :!label _label_4)
      (Utilities|Time|SetTimerbyFunctionName 0 "ResetWallJumpDelay" 0.5)
      (Variables|/Script/Engine.CharacterMovementComponent|SetAirControl (Variables|Character|GetCharacterMovement) 0.0)
      ;[1 1 1] WallJump
      (Animation|PlayAnimMontage "/Game/Art/Spencer_Assets/Riley_Anim_Test/Actual_Anims/Anim_Raw/TestMontage.TestMontage" 1.0 "None")
      (Development|PrintString "Wall Jump")
      (CallFunction|ResetJumpVelocity)
      (Character|LaunchCharacter (+ (* (Transformation|GetActorForwardVector) (* (Variables|Default|GetWallJumpForwardForce) (Math|Float|SelectFloat -1.0 1.0 (Variables|Default|GetIsWallClimbing)))) (Math|Vector|MakeVector 0.0 0.0 (Variables|Default|GetWallJumpVertForce))) true true)
      (Variables|Default|SetJumpCount (- (Variables|Default|GetJumpMaxCount) 1))
      ;[1 1 1] Off Climb
      (if (Variables|Default|GetIsWallClimbing)
        (Transformation|SetActorRotation (Math|Rotator|MakeRotator (.roll _returnvalue_2) (.pitch _returnvalue_2) (+ (.yaw _returnvalue_2) 1.8e+02)))
        (Variables|Default|SetMovementType "NewEnumerator7")
        (LocalVariables|SetFromState "From Wall Jump")
        (Variables|Default|SetMovementType "NewEnumerator7")
        (goto _label_2)
        (else
          (goto _label_2))))
    (:NewEnumerator2
      ;[1 1 1] Swinging
      (Variables|Default|SetIsSwinging false)
      (Default|EndRopeSwing (Variables|Default|GetGrapplePoint))
      (Physics|SetSimulatePhysics (Variables|Collision|GetCapsuleComponent) false)
      (Class|CableComponent|SetAttachEndto _cable self "None" "None")
      (Development|SetHiddeninGame _cable true false)
      (CallFunction|ResetJumpVelocity)
      (Character|LaunchCharacter (Math|Vector|MakeVector 0.0 0.0 (+ (.z (Transformation|GetVelocity)) (Variables|Default|GetAirJumpForce))) false true)
      (Math|Integer|DecrementInt (Variables|Default|GetJumpCount)
        (:%20%20
          (LocalVariables|SetFromState "From Swinging into Jump")
          (Variables|Default|SetMovementType "NewEnumerator7")
          (goto _label_2))))
    (:NewEnumerator4
      (CallFunction|TeleportCancelAttempt)
      (goto _label_3))
    (:NewEnumerator5
      (goto _label_4))
    (:NewEnumerator6
      (goto _label))
    (:NewEnumerator7
      ;[1 1 1] AirJump
      (if (< (Variables|Default|GetJumpCount) (Variables|Default|GetJumpMaxCount))
        (if (Variables|Default|GetCanDJump)
          (Animation|PlayAnimMontage "/Game/Art/Spencer_Assets/Riley_Anim_Test/Actual_Anims/Anim_Raw/TestMontage.TestMontage" 1.0 "None")
          (CallFunction|ResetJumpVelocity)
          (if (or (!= _returnvalue_5 0.0) (!= _returnvalue_6 0.0))
            (Transformation|SetActorRotation (Math|Rotator|MakeRotator 0.0 0.0 (.Yaw (Math|Rotator|BreakRotator (Math|Rotator|MakeRotfromX (+ (* (Math|Vector|GetForwardVector _camera) _returnvalue_4) (* (Math|Vector|GetRightVector _camera) _returnvalue_3))))))))
          (Character|LaunchCharacter (+ (+ (Transformation|GetVelocity) (Math|Vector|MakeVector 0.0 0.0 (Variables|Default|GetAirJumpForce))) (* (Transformation|GetActorForwardVector) (* (Math|Float|Clamp(Float) (+ _returnvalue_5 _returnvalue_6)) (Variables|Default|GetDoubleJumpForwardSpeed)))) true true)
          (Math|Integer|IncrementInt (Variables|Default|GetJumpCount)
            (:%20%20
              (LocalVariables|SetFromState "From Double Jump")
              (Variables|Default|SetMovementType "NewEnumerator7")
              (goto _label_2))))))))

(fn ResetJumpVelocity
  (bind _returnvalue (Transformation|GetVelocity))
  (bind (_x _y) (Math|Vector|BreakVector _returnvalue))
  (Variables|/Script/Engine.MovementComponent|SetVelocity (Variables|Character|GetCharacterMovement) (Math|Vector|MakeVector (* _x 0.5) (* _y 0.5) 0.0)))

(fn BigJumpy
  (params (Force :type Float%20%28double-precision%29))
  (bind _charactermovement (Variables|Character|GetCharacterMovement))
  (bind _velocity (Variables|/Script/Engine.MovementComponent|GetVelocity _charactermovement))
  (Character|LaunchCharacter (Math|Vector|MakeVector (.x _velocity) (.y _velocity) Force) false true))

(fn TeleportMovement
  (params (SideMovement :type Float%20%28double-precision%29))
  (Pawn|Input|AddMovementInput (Math|Vector|GetRightVector (Variables|Default|GetCamera)) SideMovement false))

(fn TeleportCancelAttempt
  (bind _returnvalue (Actor|GetComponentbyClass "/Game/Blueprints/Player/Components/BPC_TeleportPickup.BPC_TeleportPickup_C"))
  (bind _returnvalue_2 (Utilities|IsValid _returnvalue))
  (if _returnvalue_2
    (Default|EndTeleport _returnvalue)
    (else
      (Development|PrintString "Non-existent Component: Teleport")))
  (Variables|Default|SetMovementType "NewEnumerator7")
  (return _returnvalue_2))

(fn GetPlayerSave
  ;[1 1 1] Gets Last Checkpoint - Ryan
  (return (Utilities|Struct|MakeS_PlayerData (Transformation|GetActorTransform) (Variables|Default|GetHealth) (Pawn|GetControlRotation :!class /Script/Engine.Pawn) (Variables|Default|GetGoldFlies))))

(fn UsePlayerSave
  (params (Player%20Save :type S%20Player%20Data%20Structure))
  ;[1 1 1] Updates the Player with the Information they had at the last Checkpoint - Ryan
  (if (not (== (.lastcheckpoint Player%20Save) (Math|Transform|MakeTransform "0, 0, 0")))
    (Transformation|SetActorTransform (.lastcheckpoint Player%20Save))
    (Pawn|SetControlRotation (Pawn|GetController) (.controllerrotation Player%20Save))
    (Variables|Default|SetHealth (.health Player%20Save))
    (Variables|Default|SetGoldFlies (.goldflies Player%20Save))))

(event Custom|WallSlideVelocityReset
  (bind _returnvalue (Transformation|GetVelocity))
  (Utilities|FlowControl|DoOnce false) ; enters at Reset
)