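; BP_OverworldPlayer is the player-controlled actor for the overworld, which moves around and interacts with nearby actors.
; BeginPlay adds the input mapping context, and movement input follows fixed world axes rather than the camera or actor facing.
; Talk sends Interact to every overlapping actor implementing InteractFix.
; A debug key activates all LevelSelect actors; leftover orthographic camera-spawning logic is disconnected, though BeginPlay still caches the camera transform.
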(event Input|EnhancedActionEvents|EnhancedInputActionIA_Talk
  (params (ActionValue :type Boolean) (ElapsedSeconds :type Float%20%28double-precision%29) (TriggeredSeconds :type Float%20%28double-precision%29) (InputAction :type Input%20Action%20Object%20Reference :default "/Game/Inputs/InputActions/IA_Talk.IA_Talk"))
  (:Started
    (for _array_element (Collision|GetOverlappingActors 0 :!class /Script/Engine.Actor)
      (if (Utilities|DoesObjectImplementInterface _array_element "/Game/Blueprints/Mechanics/Component/InteractFix.InteractFix_C")
        (Class|InteractFix|Interact(Message) _array_element)))))

(event Input|EnhancedActionEvents|EnhancedInputActionIA_MoveRight
  (params (ActionValue :type Float%20%28double-precision%29) (ElapsedSeconds :type Float%20%28double-precision%29) (TriggeredSeconds :type Float%20%28double-precision%29) (InputAction :type Input%20Action%20Object%20Reference :default "/Game/Inputs/InputActions/IA_MoveRight.IA_MoveRight"))
  (Pawn|Input|AddMovementInput "1.000000,0.000000,0.000000" ActionValue false))

(event Input|EnhancedActionEvents|EnhancedInputActionIA_MoveForward
  (params (ActionValue :type Float%20%28double-precision%29) (ElapsedSeconds :type Float%20%28double-precision%29) (TriggeredSeconds :type Float%20%28double-precision%29) (InputAction :type Input%20Action%20Object%20Reference :default "/Game/Inputs/InputActions/IA_MoveForward.IA_MoveForward"))
  (Pawn|Input|AddMovementInput "0.000000,-1.000000,0.000000" ActionValue false))

(event EventBeginPlay
  (Input|AddMappingContext (PlayerController|LocalPlayerSubsystems|GetEnhancedInputLocalPlayerSubsystem (Game|GetPlayerController 0)) "/Game/Inputs/InputActions/IMC_Player.IMC_Player" 0 "(bIgnoreAllPressedKeysUntilRelease=True,bForceImmediately=False,bNotifyUserSettings=False)")
  (Variables|Default|SetCameraTrans (Transformation|GetWorldTransform (Variables|Default|GetCamera))))

(event Collision|EventActorBeginOverlap
  (params (OtherActor :type Actor%20Object%20Reference)))

(event EventTick
  (params (DeltaSeconds :type Float%20%28single-precision%29)))

(event Input|KeyboardEvents|DebugKeyN
  (params (Key :type Key%20Structure :default "None") (ActionValue :type Input%20Action%20Value%20Structure))
  (:Pressed
    (bind _outactors (Actor|GetAllActorsOfClass "/Game/Blueprints/Hub/LevelSelect.LevelSelect_C"))
    (for _array_element _outactors
      (Variables|/Game/Blueprints/Hub/LevelSelect.LevelSelect_C|SetActive _array_element true)
      (Development|PrintString "Unlocked Temporarily"))))

(fn ConstructionScript)