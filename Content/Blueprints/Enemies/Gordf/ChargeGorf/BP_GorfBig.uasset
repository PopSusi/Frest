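; Big Gorf enemy that roams randomly, then charges the player once they enter its proximity radius.
; Looping timers turn it toward the player and puff dust during wind-up before an AI move to the player's snapshotted position, repeating on success.
; Body contact damages the player; falling head stomps in certain movement states bounce them and remove health.
; Death spawns a fly pickup and stashes the actor off-map for later reset instead of destroying it.
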(event OnComponentBeginOverlap(HeadCollision)
  (params (OverlappedComponent :type Primitive%20Component%20Object%20Reference) (OtherActor :type Actor%20Object%20Reference) (OtherComp :type Primitive%20Component%20Object%20Reference) (OtherBodyIndex :type Integer) (bFromSweep :type Boolean) (SweepResult :type Hit%20Result%20Structure%20%28by%20ref%29))
  ;[1 1 1] Jumping on the Enemy's Head destroys it and bounces the player upwards - Ryan
  (bind _asbp_player (Utilities|Casting|CastToBP_Player OtherActor))
  (if (and (or (Utilities|Enum|Equal(Enum) (Variables|/Game/Blueprints/Player/BP_Player.BP_Player_C|GetMovementType _asbp_player) "NewEnumerator12") (Utilities|Enum|Equal(Enum) (Variables|/Game/Blueprints/Player/BP_Player.BP_Player_C|GetMovementType _asbp_player) "NewEnumerator15")) (< (.z (Transformation|GetVelocity _asbp_player)) 0.0))
    (Utilities|FlowControl|DoOnce false
      (:Completed
        ;;[0 0.4666 1] Put Death Sound Here
        (Audio|PlaySound2D "/Game/Sounds/SFX/Gorf/gorftdeath.gorftdeath" 1.0 1.0 0.0 0 0)
        (Character|LaunchCharacter _asbp_player "0.000000,0.000000,1500.000000" false true)
        (bind _result (Math|Integer|DecrementInt (Variables|Default|GetHealth))
          (:%20%20
            (if (== _result 0)
              (Animation|PlayAnimMontage "/Game/Art/Spencer_Assets/Gorf/Animations/Gorf_Death_Montage.Gorf_Death_Montage" 0.5 "None")
              (Utilities|Time|ClearandInvalidateTimerbyHandle (Variables|Default|GetTimer%20Handle))
              (Utilities|FlowControl|Delay 0.5)
              (Game|SpawnActorfromClass "/Game/Blueprints/Enemies/Gordf/DeathFly.DeathFly_C" (Transformation|GetActorTransform self) "Undefined" "MultiplyWithRoot" 0 0)
              (Audio|PlaySound2D "/Game/Sounds/MetaSounds/MS_CollectibleStereo.MS_CollectibleStereo" 1.0 1.0 0.0 0 0)
              (UserInterface|Animation|PlayAnimation (Variables|/Game/Blueprints/Player/BP_Player.BP_Player_C|GetHUD _asbp_player) (Variables|/Game/UI/Widgets/HUD/WB_HUD.WB_HUD_C|GetGoldFlyUpdate (Variables|/Game/Blueprints/Player/BP_Player.BP_Player_C|GetHUD _asbp_player)) 0.0 1 "Forward" 1.0 true)
              (CallFunction|Stash)
              (else
                (Utilities|Time|SetTimerbyEvent (delegate Custom|ResetDamage) 0.5)
                (CallFunction|TookDamage)))))))))

(event OnComponentBeginOverlap(DetectionRadius)
  (params (OverlappedComponent :type Primitive%20Component%20Object%20Reference) (OtherActor :type Actor%20Object%20Reference) (OtherComp :type Primitive%20Component%20Object%20Reference) (OtherBodyIndex :type Integer) (bFromSweep :type Boolean) (SweepResult :type Hit%20Result%20Structure%20%28by%20ref%29))
  ;[1 1 1] Enemy rotates to face player when the player is in range - Ryan
)

(event OnSeePawn(PawnSensing)
  (params (Pawn :type Pawn%20Object%20Reference))
  ;[1 1 1] If the enemy sees the player, it will follow them until they exit their sensing range - Ryan
)

(event OnComponentHit(CapsuleComponent)
  (params (HitComponent :type Primitive%20Component%20Object%20Reference) (OtherActor :type Actor%20Object%20Reference) (OtherComp :type Primitive%20Component%20Object%20Reference) (NormalImpulse :type Vector :default "0, 0, 0") (Hit :type Hit%20Result%20Structure%20%28by%20ref%29))
  (bind _charactermovement (Variables|Character|GetCharacterMovement))
  ;[1 1 1] Deal Damage to Player on Contact - Ryan
  (bind _asbp_player (Utilities|Casting|CastToBP_Player OtherActor))
  (Default|TakeDamage _asbp_player false)
  (Pawn|Components|CharacterMovement|DisableMovement _charactermovement)
  (Utilities|FlowControl|Delay 1.0)
  (Pawn|Components|CharacterMovement|SetMovementMode _charactermovement "MOVE_Walking" 0))

(event OnComponentBeginOverlap(IsPlayerCloseRadius)
  (params (OverlappedComponent :type Primitive%20Component%20Object%20Reference) (OtherActor :type Actor%20Object%20Reference) (OtherComp :type Primitive%20Component%20Object%20Reference) (OtherBodyIndex :type Integer) (bFromSweep :type Boolean) (SweepResult :type Hit%20Result%20Structure%20%28by%20ref%29))
  ;[1 1 1] Enemy rotates to face player when the player is in range - Ryan
  (if (== (Utilities|GetClass OtherActor) "/Game/Blueprints/Player/BP_Player.BP_Player_C")
    (bind _asbp_player (Utilities|Casting|CastToBP_Player (Game|GetPlayerCharacter 0)))
    (Variables|Default|SetPlayer _asbp_player)
    (Utilities|FlowControl|DoOnce false
      (:Completed
        (Components|Animation|PlayAnimation (Variables|Character|GetMesh) "/Game/Art/Spencer_Assets/Gorf/Animations/Gorf_Alert.Gorf_Alert" false)
        (Utilities|Time|ClearandInvalidateTimerbyHandle (Variables|Default|GetRoamTimer))
        (if (not false)
          (Components|Movement|StopMovementImmediately (Variables|Character|GetCharacterMovement))
          (bind _returnvalue (Utilities|Time|SetTimerbyEvent (delegate Custom|Event%20RotateEnemy) 0.01 true))
          (Variables|Default|SetTimer%20Handle _returnvalue)
          (bind _returnvalue_2 (Utilities|Time|SetTimerbyEvent (delegate Custom|ChargeEvent) 2.0))
          (Variables|Default|SetStartChargeTimer _returnvalue_2))))))

(event Custom|RandomRoam
  ;[1 1 1] Enemies will randomly roam to a nearby spot and then sit for 2 seconds before moving again - Ryan
  (Variables|/Script/Engine.CharacterMovementComponent|SetMaxWalkSpeed (Variables|Character|GetCharacterMovement) 2e+02)
  (Components|Animation|PlayAnimation (Variables|Character|GetMesh) "/Game/Art/Spencer_Assets/Gorf/Animations/Gorf_Walk.Gorf_Walk" true)
  (AI|AIMoveTo self (.RandomLocation (AI|Navigation|GetRandomReachablePointinRadius (Transformation|GetActorLocation) 1.5e+03 0 0)) 0 5.0 false
    (:OnSuccess
      (bind _returnvalue (Utilities|Time|SetTimerbyEvent (delegate Custom|RandomRoam) 2.0))
      (Variables|Default|SetRoamTimer _returnvalue))))

(event Custom|SpawnDustCloud
  (Utilities|SpawnCloud))

(event Custom|DoCharge
  (bind _returnvalue (Game|Player|GetPlayerPawn 0))
  (bind _returnvalue_2 (Transformation|GetActorLocation _returnvalue))
  (Utilities|Time|ClearandInvalidateTimerbyHandle (Variables|Default|GetTimer%20Handle))
  (bind _output_get (Variables|Default|SetPlayerChargeLocation (Math|Vector|MakeVector (.x _returnvalue_2) (.y _returnvalue_2) (.z (Transformation|GetActorLocation)))))
  (Variables|/Script/Engine.CharacterMovementComponent|SetMaxWalkSpeed (Variables|Character|GetCharacterMovement) 8e+02)
  (AI|AIMoveTo self _output_get 0 5.0 false
    (:OnSuccess
      (Utilities|Time|ClearandInvalidateTimerbyHandle (Variables|Default|GetDustCloudTimer))
      (Components|Animation|PlayAnimation (Variables|Character|GetMesh) "/Game/Art/Spencer_Assets/Gorf/Animations/Gorf_Idle.Gorf_Idle" true)
      (Variables|/Script/Engine.CharacterMovementComponent|SetMaxWalkSpeed (Variables|Character|GetCharacterMovement) 2e+02)
      (CallFunction|StartRotate))
    (:OnFail
      (if (Utilities|Array|ContainsItem (Collision|GetOverlappingActors (Variables|Default|GetDetection%20Radius) 0 :!class /Script/Engine.PrimitiveComponent) (Game|Player|GetPlayerPawn 0))
        _
        (else
          _))
      (Utilities|Time|ClearandInvalidateTimerbyHandle (Variables|Default|GetDustCloudTimer))
      (CallFunction|ResetDetection)
      (CallFunction|RandomRoam))))

(event Custom|StartRotate
  (Components|Animation|PlayAnimation (Variables|Character|GetMesh) "/Game/Art/Spencer_Assets/Gorf/Animations/Gorf_Idle.Gorf_Idle" true)
  (Utilities|Time|ClearandInvalidateTimerbyHandle (Variables|Default|GetRoamTimer))
  ;[1 1 1] Enemy rotates to face player when the player is in range - Ryan
  (if (not false)
    (Components|Movement|StopMovementImmediately (Variables|Character|GetCharacterMovement))
    (bind _returnvalue (Utilities|Time|SetTimerbyEvent (delegate Custom|Event%20RotateEnemy) 0.01 true))
    (Variables|Default|SetTimer%20Handle _returnvalue)
    (bind _returnvalue_2 (Utilities|Time|SetTimerbyEvent (delegate Custom|ChargeEvent) 2.0))
    (Variables|Default|SetStartChargeTimer _returnvalue_2)))

(event Custom|ResetDamage
  ;[1 1 1] Jumping on the Enemy's Head destroys it and bounces the player upwards - Ryan
  (Utilities|FlowControl|DoOnce false) ; enters at Reset
)

(event Custom|TookDamage
  (Components|Movement|StopMovementImmediately (Variables|Character|GetCharacterMovement))
  (for _array_element (Utilities|Array|MakeArray (Variables|Default|GetTimer%20Handle) (Variables|Default|GetDustCloudTimer) (Variables|Default|GetChargeTimer) (Variables|Default|GetStartChargeTimer))
    (Utilities|Time|ClearandInvalidateTimerbyHandle _array_element))
  (Components|Animation|PlayAnimation (Variables|Character|GetMesh) "/Game/Art/Spencer_Assets/Gorf/Animations/Gorf_Alert.Gorf_Alert" false)
  (Utilities|FlowControl|Delay 1.0)
  (CallFunction|StartRotate))

(event Custom|Event%20RotateEnemy
  ;[1 1 1] Enemy rotates to face player when the player is in range - Ryan
  (Transformation|SetActorRotation (Math|Rotator|MakeRotator 0.0 0.0 (.yaw (Math|Interpolation|RInterpTo (Transformation|GetActorRotation) (Math|Rotator|FindLookatRotation (Transformation|GetActorLocation) (Transformation|GetActorLocation (Variables|Default|GetPlayer))) (Utilities|Time|GetWorldDeltaSeconds) 3.0)))))

(event Custom|ChargeEvent
  (Components|Animation|PlayAnimation (Variables|Character|GetMesh) "/Game/Art/Spencer_Assets/Gorf/Animations/Gorf_Run.Gorf_Run" true)
  (Utilities|SpawnCloud
    (:NewParam
      (bind _returnvalue (Utilities|Time|SetTimerbyEvent (delegate Custom|SpawnDustCloud) 0.5 true))
      (Variables|Default|SetDustCloudTimer _returnvalue)
      (bind _returnvalue_2 (Utilities|Time|SetTimerbyEvent (delegate Custom|DoCharge) 2.0))
      (Variables|Default|SetChargeTimer _returnvalue_2))))

(event Custom|Reset%20Detection
  (Utilities|FlowControl|DoOnce false) ; enters at Reset
)

(event Custom|ReplaceReset_1
  ;[1 1 1] Reset Gorfs - Susi
  (CallFunction|Unstash))

(event EventBeginPlay
  (bind _returnvalue (Transformation|GetActorTransform))
  ;[1 1 1] On Begin Play, enemies will randomly roam and their return location will be their initial location by default - Ryan
  (Variables|Default|SetSpawnTransform _returnvalue)
  (Variables|Default|SetReturnTransform _returnvalue)
  (CallFunction|RandomRoam)
  (bind _asbp_player (Utilities|Casting|CastToBP_Player (Game|GetPlayerCharacter 0)))
  (Variables|Default|SetPlayer _asbp_player))

(event Collision|EventActorBeginOverlap
  (params (OtherActor :type Actor%20Object%20Reference)))

(event EventTick
  (params (DeltaSeconds :type Float%20%28single-precision%29))
  (bind _returnvalue (Utilities|Time|GetWorldDeltaSeconds))
  (bind _chargedirection (Variables|Default|GetChargeDirection))
  (bind _player (Variables|Default|GetPlayer))
  (bind _returnvalue_2 (Transformation|GetWorldLocation _chargedirection))
  (bind _returnvalue_3 (Transformation|GetWorldRotation _chargedirection))
  (bind _returnvalue_4 (Transformation|GetActorLocation _player))
  (bind _returnvalue_5 (Math|Rotator|FindLookatRotation _returnvalue_2 _returnvalue_4))
  (bind _returnvalue_6 (Math|Interpolation|RInterpTo _returnvalue_3 _returnvalue_5 _returnvalue 3.0))
  ;[1 1 1] Enemy rotates to face player when the player is in range - Ryan
  (Transformation|SetWorldRotation (Variables|Default|GetChargeDirection) (Math|Rotator|MakeRotator 0.0 (.pitch _returnvalue_6) (.yaw _returnvalue_6)) false false))

(fn ConstructionScript)

(fn Stash
  (Physics|SetEnableGravity (Variables|Collision|GetCapsuleComponent) false)
  (Transformation|SetActorLocation "-10000.000000,-10000.000000,-10000.000000" false true)
  (Pawn|Components|CharacterMovement|SetMovementMode (Variables|Character|GetCharacterMovement) "MOVE_Walking" 0)
  (CallFunction|RandomRoam))

(fn Unstash
  (Physics|SetEnableGravity (Variables|Collision|GetCapsuleComponent) true)
  (Transformation|SetActorTransform (Variables|Default|GetSpawnTransform) false true)
  (Pawn|Components|CharacterMovement|SetMovementMode (Variables|Character|GetCharacterMovement) "MOVE_Walking" 0)
  (CallFunction|RandomRoam))