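; Flying Gorf enemy that roams at random unless stationary and can be killed by a player stomping on its head.
; When the player enters its close radius, it attaches a ScholarLaser to its crystal, then turns and follows on looping timers until the player leaves the detection radius.
; A stomp bounces the player, spawns a DeathFly and stashes the Gorf off-map rather than destroying it, so reset can restore its spawn transform.
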(event OnComponentBeginOverlap(HeadCollision)
  (params (OverlappedComponent :type Primitive%20Component%20Object%20Reference) (OtherActor :type Actor%20Object%20Reference) (OtherComp :type Primitive%20Component%20Object%20Reference) (OtherBodyIndex :type Integer) (bFromSweep :type Boolean) (SweepResult :type Hit%20Result%20Structure%20%28by%20ref%29))
  ;[1 1 1] Jumping on the Enemy's Head destroys it and bounces the player upwards - Ryan
  (bind _asbp_player (Utilities|Casting|CastToBP_Player OtherActor))
  (if (and (or (Utilities|Enum|Equal(Enum) (Variables|/Game/Blueprints/Player/BP_Player.BP_Player_C|GetMovementType _asbp_player) "NewEnumerator12") (Utilities|Enum|Equal(Enum) (Variables|/Game/Blueprints/Player/BP_Player.BP_Player_C|GetMovementType _asbp_player) "NewEnumerator15")) (< (.z (Transformation|GetVelocity _asbp_player)) 0.0))
    (Audio|PlaySound2D "/Game/Sounds/SFX/Gorf/gorftdeath.gorftdeath" 1.0 1.0 0.0 0 0)
    (Character|LaunchCharacter _asbp_player "0.000000,0.000000,1500.000000" false true)
    (Components|Animation|PlayAnimation (Variables|Character|GetMesh) "/Game/Art/Spencer_Assets/Gorf/Animations/Flying_Gorf/Flying_Gorf_Death.Flying_Gorf_Death" false)
    (CallFunction|TookDamage)
    (Utilities|FlowControl|Delay 0.5)
    (Game|SpawnActorfromClass "/Game/Blueprints/Enemies/Gordf/DeathFly.DeathFly_C" (Transformation|GetActorTransform self) "Undefined" "MultiplyWithRoot" 0 0)
    (Audio|PlaySound2D "/Game/Sounds/MetaSounds/MS_CollectibleStereo.MS_CollectibleStereo" 1.0 1.0 0.0 0 0)
    (UserInterface|Animation|PlayAnimation (Variables|/Game/Blueprints/Player/BP_Player.BP_Player_C|GetHUD _asbp_player) (Variables|/Game/UI/Widgets/HUD/WB_HUD.WB_HUD_C|GetGoldFlyUpdate (Variables|/Game/Blueprints/Player/BP_Player.BP_Player_C|GetHUD _asbp_player)) 0.0 1 "Forward" 1.0 true)
    (CallFunction|Stash)))

(event OnComponentBeginOverlap(DetectionRadius)
  (params (OverlappedComponent :type Primitive%20Component%20Object%20Reference) (OtherActor :type Actor%20Object%20Reference) (OtherComp :type Primitive%20Component%20Object%20Reference) (OtherBodyIndex :type Integer) (bFromSweep :type Boolean) (SweepResult :type Hit%20Result%20Structure%20%28by%20ref%29))
  ;[1 1 1] Enemy rotates to face player when the player is in range - Ryan
)

(event OnComponentEndOverlap(DetectionRadius)
  (params (OverlappedComponent :type Primitive%20Component%20Object%20Reference) (OtherActor :type Actor%20Object%20Reference) (OtherComp :type Primitive%20Component%20Object%20Reference) (OtherBodyIndex :type Integer))
  (if (== (Utilities|GetClass OtherActor) "/Game/Blueprints/Player/BP_Player.BP_Player_C")
    (CallFunction|TookDamage)
    (Utilities|FlowControl|Gate true) ; enters at Close
  ))

(event OnComponentHit(CapsuleComponent)
  (params (HitComponent :type Primitive%20Component%20Object%20Reference) (OtherActor :type Actor%20Object%20Reference) (OtherComp :type Primitive%20Component%20Object%20Reference) (NormalImpulse :type Vector :default "0, 0, 0") (Hit :type Hit%20Result%20Structure%20%28by%20ref%29))
  ;[1 1 1] Deal Damage to Player on Contact - Ryan
)

(event OnComponentBeginOverlap(IsPlayerCloseRadius)
  (params (OverlappedComponent :type Primitive%20Component%20Object%20Reference) (OtherActor :type Actor%20Object%20Reference) (OtherComp :type Primitive%20Component%20Object%20Reference) (OtherBodyIndex :type Integer) (bFromSweep :type Boolean) (SweepResult :type Hit%20Result%20Structure%20%28by%20ref%29))
  (if (not (Variables|Default|GetIsStationary))
    ;[1 1 1] Enemy rotates to face player when the player is in range - Ryan
    (if (== (Utilities|GetClass OtherActor) "/Game/Blueprints/Player/BP_Player.BP_Player_C")
      (Utilities|FlowControl|DoOnce false
        (:Completed
          (Utilities|SpawnLaser
            (:NewParam2
              (Utilities|Time|ClearandInvalidateTimerbyHandle (Variables|Default|GetRoamTimer))
              (if (not false)
                (Components|Movement|StopMovementImmediately (Variables|Character|GetCharacterMovement))
                (bind _returnvalue (Utilities|Time|SetTimerbyEvent (delegate Custom|Event%20RotateEnemy) 0.01 true))
                (Variables|Default|SetRotationTimer%20Handle _returnvalue)
                (bind _returnvalue_2 (Utilities|Time|SetTimerbyEvent (delegate Custom|FollowEvent) 0.1 true))
                (Variables|Default|SetFollowTimer _returnvalue_2)
                (Utilities|FlowControl|Gate true) ; enters at Open
              ))))))))

(event Custom|RandomRoam
  ;[1 1 1] Enemies will randomly roam to a nearby spot and then sit for 2 seconds before moving again - Ryan
  (Components|Animation|PlayAnimation (Variables|Character|GetMesh) "/Game/Art/Spencer_Assets/Gorf/Animations/Flying_Gorf/Flying_Gorf_Flap.Flying_Gorf_Flap" true)
  (AI|AIMoveTo self (.RandomLocation (AI|Navigation|GetRandomReachablePointinRadius (Transformation|GetActorLocation) 1.5e+03 0 0)) 0 5.0 false
    (:OnSuccess
      (bind _returnvalue (Utilities|Time|SetTimerbyEvent (delegate Custom|RandomRoam) 2.0))
      (Variables|Default|SetRoamTimer _returnvalue))))

(event Custom|ResetDamage
  ;[1 1 1] Jumping on the Enemy's Head destroys it and bounces the player upwards - Ryan
)

(event Custom|TookDamage
  (Components|Movement|StopMovementImmediately (Variables|Character|GetCharacterMovement))
  (for _array_element (Utilities|Array|MakeArray (Variables|Default|GetRotationTimer%20Handle) (Variables|Default|GetFollowTimer) (Variables|Default|GetRoamTimer) "")
    (Utilities|Time|ClearandInvalidateTimerbyHandle _array_element))
  (Components|Animation|PlayAnimation (Variables|Character|GetMesh) "/Game/Art/Spencer_Assets/Gorf/Animations/Flying_Gorf/Flying_Gorf_Flap.Flying_Gorf_Flap" true)
  (CallFunction|ResetDetection)
  (Utilities|FlowControl|Gate true) ; enters at Close
)

(event Custom|Event%20RotateEnemy
  ;[1 1 1] Enemy rotates to face player when the player is in range - Ryan
  (Variables|Default|SetDesiredRotation (.yaw (Math|Interpolation|RInterpTo (Transformation|GetActorRotation) (Math|Rotator|FindLookatRotation (Transformation|GetActorLocation) (Transformation|GetActorLocation (Variables|Default|GetPlayer))) (Utilities|Time|GetWorldDeltaSeconds) 8.0))))

(event Custom|FollowEvent
  (bind _returnvalue (Game|GetPlayerCharacter 0))
  (bind _returnvalue_2 (Transformation|GetActorLocation _returnvalue))
  (AI|AIMoveTo self (Math|Vector|MakeVector (.x _returnvalue_2) (.y _returnvalue_2) (.z (Transformation|GetActorLocation))) 0 5.0 false))

(event Custom|Reset%20Detection
  ;[1 1 1] Enemy rotates to face player when the player is in range - Ryan
  (Utilities|FlowControl|DoOnce false) ; enters at Reset
)

(event Custom|ReplaceReset_1
  ;[1 1 1] Reset Gorfs - Susi
  (CallFunction|Unstash))

(event EventBeginPlay
  (bind _returnvalue (Transformation|GetActorTransform))
  ;[1 1 1] On Begin Play, enemies will randomly roam and their return location will be their initial location by default - Ryan
  (Variables|Default|SetSpawnTransform _returnvalue)
  (Variables|Default|SetReturnTransform _returnvalue)
  (bind _asbp_player (Utilities|Casting|CastToBP_Player (Game|GetPlayerCharacter 0)))
  (Variables|Default|SetPlayer _asbp_player)
  (Transformation|AttachComponentToComponent (Variables|Default|GetCrystal) (Variables|Character|GetMesh) "RootSocket" "KeepWorld" "KeepWorld" "KeepWorld" true)
  (if (Variables|Default|GetIsStationary)
    (Pawn|Components|CharacterMovement|SetMovementMode (Variables|Character|GetCharacterMovement) "MOVE_Flying" 0)
    (else
      (CallFunction|RandomRoam))))

(event Collision|EventActorBeginOverlap
  (params (OtherActor :type Actor%20Object%20Reference)))

(event EventTick
  (params (DeltaSeconds :type Float%20%28single-precision%29))
  (Utilities|FlowControl|Gate true
    (:Exit
      (Transformation|SetActorRotation (Math|Rotator|MakeRotator 0.0 0.0 (Variables|Default|GetDesiredRotation))))))

(fn ConstructionScript)

(fn Stash
  (Physics|SetEnableGravity (Variables|Collision|GetCapsuleComponent) false)
  (Transformation|SetActorLocation "-10000.000000,-10000.000000,-10000.000000" false true)
  (Pawn|Components|CharacterMovement|SetMovementMode (Variables|Character|GetCharacterMovement) "MOVE_Walking" 0)
  (CallFunction|RandomRoam))

(fn Unstash
  (Physics|SetEnableGravity (Variables|Collision|GetCapsuleComponent) true)
  (Transformation|SetActorTransform (Variables|Default|GetSpawnTransform) false true)
  (Pawn|Components|CharacterMovement|SetMovementMode (Variables|Character|GetCharacterMovement) "MOVE_Walking" 0)
  (CallFunction|RandomRoam))