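; Gorf enemy that roams, chases the player on sight, damages them on contact and dies when stomped.
; AIMoveTo loops random roaming, while a detection overlap starts a looping timer that turns it toward the player.
; PawnSensing drives the chase, and a retriggerable delay detects lost sight, sending it back to where it spotted the player.
; A falling player hitting the head collision is launched upward as the enemy spawns DeathFly and destroys itself.
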(event OnComponentBeginOverlap(HeadCollision)
  (params (OverlappedComponent :type Primitive%20Component%20Object%20Reference) (OtherActor :type Actor%20Object%20Reference) (OtherComp :type Primitive%20Component%20Object%20Reference) (OtherBodyIndex :type Integer) (bFromSweep :type Boolean) (SweepResult :type Hit%20Result%20Structure%20%28by%20ref%29))
  ;[1 1 1] Jumping on the Enemy's Head destroys it and bounces the player upwards - Ryan
  (bind _asbp_player (Utilities|Casting|CastToBP_Player (Game|GetPlayerCharacter 0)))
  (if (and (< (.z (Transformation|GetVelocity _asbp_player)) 0.0) (== (Utilities|GetClass OtherActor) "/Game/Blueprints/Player/BP_Player.BP_Player_C"))
    (Character|LaunchCharacter _asbp_player "0.000000,0.000000,2500.000000" false false)
    (Game|SpawnActorfromClass "/Game/Blueprints/Enemies/Gordf/DeathFly.DeathFly_C" (Transformation|GetActorTransform self) "Undefined" "MultiplyWithRoot" 0 0)
    (Audio|PlaySound2D "/Game/Sounds/SFX/Movement/DoubleJump.DoubleJump" 1.0 1.0 0.0 0 0)
    (Actor|DestroyActor)))

(event OnComponentBeginOverlap(DetectionRadius)
  (params (OverlappedComponent :type Primitive%20Component%20Object%20Reference) (OtherActor :type Actor%20Object%20Reference) (OtherComp :type Primitive%20Component%20Object%20Reference) (OtherBodyIndex :type Integer) (bFromSweep :type Boolean) (SweepResult :type Hit%20Result%20Structure%20%28by%20ref%29))
  ;[1 1 1] Enemy rotates to face player when the player is in range - Ryan
  (bind _asbp_player (Utilities|Casting|CastToBP_Player (Game|GetPlayerCharacter 0)))
  (Variables|Default|SetPlayer _asbp_player)
  (if (== (Utilities|GetClass OtherActor) "/Game/Blueprints/Player/BP_Player.BP_Player_C")
    (if (not (Variables|Default|GetIn%20Chase))
      (Components|Movement|StopMovementImmediately (Variables|Character|GetCharacterMovement))
      (bind _returnvalue (Utilities|Time|SetTimerbyEvent (delegate Custom|Event%20RotateEnemy) 0.01 true))
      (Variables|Default|SetTimer%20Handle _returnvalue))))

(event OnSeePawn(PawnSensing)
  (params (Pawn :type Pawn%20Object%20Reference))
  ;[1 1 1] If the enemy sees the player, it will follow them until they exit their sensing range - Ryan
  (Utilities|FlowControl|Sequence
    (:then_0
      (if (not (Variables|Default|GetIn%20Chase))
        (Variables|Default|SetReturn%20Location (Transformation|GetActorLocation))))
    (:then_1
      (Variables|Default|SetIn%20Chase true)
      (Utilities|FlowControl|Sequence
        (:then_0
          (AI|AIMoveTo self "0, 0, 0" Pawn 5.0 false))
        (:then_1
          ;[1 1 1] If the enemy loses the player, they will move back to the spot they initially saw the player, and then continue to randomly roam - Ryan
          (Utilities|FlowControl|RetriggerableDelay 1.0)
          (Variables|Default|SetIn%20Chase false)
          (Components|Movement|StopMovementImmediately (Variables|Character|GetCharacterMovement))
          (Utilities|Time|ClearandInvalidateTimerbyHandle (Variables|Default|GetTimer%20Handle))
          (Utilities|FlowControl|Delay 2.0)
          (AI|AIMoveTo self (Variables|Default|GetReturn%20Location) 0 5.0 false
            (:OnSuccess
              (Utilities|FlowControl|Delay 2.0)
              (CallFunction|EventRandomRoam))))))))

(event OnComponentBeginOverlap(CapsuleComponent)
  (params (OverlappedComponent :type Primitive%20Component%20Object%20Reference) (OtherActor :type Actor%20Object%20Reference) (OtherComp :type Primitive%20Component%20Object%20Reference) (OtherBodyIndex :type Integer) (bFromSweep :type Boolean) (SweepResult :type Hit%20Result%20Structure%20%28by%20ref%29))
  ;[1 1 1] Respawn Player on Contact with Enemy - Ryan (this should eventually get changed to just dealing damage)
  (if (== (Utilities|GetClass OtherActor) "/Game/Blueprints/Player/BP_Player.BP_Player_C")
    (Utilities|Time|ClearandInvalidateTimerbyHandle (Variables|Default|GetTimer%20Handle))
    (bind _asbp_player (Utilities|Casting|CastToBP_Player OtherActor))
    (Game|Damage|ApplyDamage _asbp_player 1.0 0 self)))

(event Custom|Event%20RandomRoam
  ;[1 1 1] Enemies will randomly roam to a nearby spot and then sit for 2 seconds before moving again - Ryan
  (AI|AIMoveTo self (.RandomLocation (AI|Navigation|GetRandomReachablePointinRadius (Transformation|GetActorLocation) 1.5e+03 0 0)) 0 5.0 false
    (:OnSuccess
      (Utilities|FlowControl|Delay 2.0)
      (CallFunction|EventRandomRoam))))

(event Custom|Event%20RotateEnemy
  ;[1 1 1] Enemy rotates to face player when the player is in range - Ryan
  (Transformation|SetActorRotation (Math|Rotator|MakeRotator 0.0 0.0 (.yaw (Math|Interpolation|RInterpTo (Transformation|GetActorRotation) (Math|Rotator|FindLookatRotation (Transformation|GetActorLocation) (Transformation|GetActorLocation (Variables|Default|GetPlayer))) (Utilities|Time|GetWorldDeltaSeconds) 3.0)))))

(event EventBeginPlay
  ;[1 1 1] On Begin Play, enemies will randomly roam and their return location will be their initial location by default - Ryan
  (Variables|Default|SetReturn%20Location (Transformation|GetActorLocation))
  (CallFunction|EventRandomRoam))

(event Collision|EventActorBeginOverlap
  (params (OtherActor :type Actor%20Object%20Reference)))

(event EventTick
  (params (DeltaSeconds :type Float%20%28single-precision%29)))

(fn ConstructionScript)