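; Ranged Gorf enemy that roams randomly, shoots projectiles at the player and damages them on contact.
; A player entering the close radius starts timer-driven tracking and, if CanDig is set, a Timeline burrow to a random point near the player.
; After surfacing, radius checks choose digging again, shooting on a repeat timer or roaming.
; Stomp kills bounce the player, spawn DeathFly and stash the Gorf off-map for later reset.
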(event OnComponentBeginOverlap(HeadCollision)
  (params (OverlappedComponent :type Primitive%20Component%20Object%20Reference) (OtherActor :type Actor%20Object%20Reference) (OtherComp :type Primitive%20Component%20Object%20Reference) (OtherBodyIndex :type Integer) (bFromSweep :type Boolean) (SweepResult :type Hit%20Result%20Structure%20%28by%20ref%29))
  ;[1 1 1] Jumping on the Enemy's Head destroys it and bounces the player upwards - Ryan
  (bind _asbp_player (Utilities|Casting|CastToBP_Player OtherActor))
  (Default|GorfReplaceDoubleJump _asbp_player)
  (if (and (or (Utilities|Enum|Equal(Enum) (Variables|/Game/Blueprints/Player/BP_Player.BP_Player_C|GetMovementType _asbp_player) "NewEnumerator12") (Utilities|Enum|Equal(Enum) (Variables|/Game/Blueprints/Player/BP_Player.BP_Player_C|GetMovementType _asbp_player) "NewEnumerator15")) (< (.z (Transformation|GetVelocity _asbp_player)) 0.0))
    ;;[0 0.4666 1] Put Death Sound Here
    (Audio|PlaySound2D "/Game/Sounds/SFX/Gorf/gorftdeath.gorftdeath" 1.0 1.0 0.0 0 0)
    (Default|CallGorfDied)
    (Pawn|Components|CharacterMovement|DisableMovement (Variables|Character|GetCharacterMovement))
    (Character|LaunchCharacter _asbp_player "0.000000,0.000000,1500.000000" false true)
    (Animation|PlayAnimMontage "/Game/Art/Spencer_Assets/Gorf/Animations/Basic_Gorf/Gorf_Death_Montage.Gorf_Death_Montage" 0.5 "None")
    (Utilities|Time|ClearandInvalidateTimerbyHandle (Variables|Default|GetTimer%20Handle))
    (Utilities|FlowControl|Delay 0.5)
    (Game|SpawnActorfromClass "/Game/Blueprints/Enemies/Gordf/DeathFly.DeathFly_C" (Transformation|GetActorTransform self) "Undefined" "MultiplyWithRoot" 0 0)
    (Audio|PlaySound2D "/Game/Sounds/MetaSounds/MS_CollectibleStereo.MS_CollectibleStereo" 1.0 1.0 0.0 0 0)
    (UserInterface|Animation|PlayAnimation (Variables|/Game/Blueprints/Player/BP_Player.BP_Player_C|GetHUD _asbp_player) (Variables|/Game/UI/Widgets/HUD/WB_HUD.WB_HUD_C|GetGoldFlyUpdate (Variables|/Game/Blueprints/Player/BP_Player.BP_Player_C|GetHUD _asbp_player)) 0.0 1 "Forward" 1.0 true)
    (CallFunction|ResetDetection)
    (CallFunction|Stash)))

(event OnComponentBeginOverlap(DetectionRadius)
  (params (OverlappedComponent :type Primitive%20Component%20Object%20Reference) (OtherActor :type Actor%20Object%20Reference) (OtherComp :type Primitive%20Component%20Object%20Reference) (OtherBodyIndex :type Integer) (bFromSweep :type Boolean) (SweepResult :type Hit%20Result%20Structure%20%28by%20ref%29))
  ;[1 1 1] Enemy rotates to face player when the player is in range - Ryan
)

(event OnSeePawn(PawnSensing)
  (params (Pawn :type Pawn%20Object%20Reference))
  ;[1 1 1] If the enemy sees the player, it will follow them until they exit their sensing range - Ryan
)

(event OnComponentHit(CapsuleComponent)
  (params (HitComponent :type Primitive%20Component%20Object%20Reference) (OtherActor :type Actor%20Object%20Reference) (OtherComp :type Primitive%20Component%20Object%20Reference) (NormalImpulse :type Vector :default "0, 0, 0") (Hit :type Hit%20Result%20Structure%20%28by%20ref%29))
  (bind _charactermovement (Variables|Character|GetCharacterMovement))
  ;[1 1 1] Deal Damage to Player on Contact - Ryan
  (bind _asbp_player (Utilities|Casting|CastToBP_Player OtherActor))
  (Default|TakeDamage _asbp_player false)
  (Pawn|Components|CharacterMovement|DisableMovement _charactermovement)
  (Utilities|FlowControl|Delay 1.0)
  (Pawn|Components|CharacterMovement|SetMovementMode _charactermovement "MOVE_Walking" 0))

(event OnComponentBeginOverlap(IsPlayerCloseRadius)
  (params (OverlappedComponent :type Primitive%20Component%20Object%20Reference) (OtherActor :type Actor%20Object%20Reference) (OtherComp :type Primitive%20Component%20Object%20Reference) (OtherBodyIndex :type Integer) (bFromSweep :type Boolean) (SweepResult :type Hit%20Result%20Structure%20%28by%20ref%29))
  ;[1 1 1] Enemy rotates to face player when the player is in range - Ryan
  (if (== (Utilities|GetClass OtherActor) "/Game/Blueprints/Player/BP_Player.BP_Player_C")
    (bind _asbp_player (Utilities|Casting|CastToBP_Player (Game|GetPlayerCharacter 0)))
    (Variables|Default|SetPlayer _asbp_player)
    (Utilities|FlowControl|DoOnce false
      (:Completed
        (Utilities|Time|ClearandInvalidateTimerbyHandle (Variables|Default|GetRoamTimer))
        (if (not false)
          (Components|Movement|StopMovementImmediately (Variables|Character|GetCharacterMovement))
          (Animation|PlayAnimMontage "/Game/Art/Spencer_Assets/Gorf/Animations/Basic_Gorf/Gorf_Alert_Montage.Gorf_Alert_Montage" 1.0 "None")
          (bind _returnvalue (Utilities|Time|SetTimerbyEvent (delegate Custom|Event%20RotateEnemy) 0.01 true))
          (Variables|Default|SetTimer%20Handle _returnvalue)
          (CallFunction|DigEvent))))))

(event Custom|RandomRoam
  ;[1 1 1] Enemies will randomly roam to a nearby spot and then sit for 2 seconds before moving again - Ryan
  (AI|AIMoveTo self (.RandomLocation (AI|Navigation|GetRandomReachablePointinRadius (Transformation|GetActorLocation) 1.5e+03 0 0)) 0 5.0 false
    (:OnSuccess
      _)
    (:OnFail
      _))
  (bind _returnvalue (Utilities|Time|SetTimerbyEvent (delegate Custom|RandomRoam) 2.0))
  (Variables|Default|SetRoamTimer _returnvalue))

(event Custom|Event%20RotateEnemy
  (bind _returnvalue (Utilities|Time|GetWorldDeltaSeconds))
  (bind _arrow1 (Variables|Default|GetArrow1))
  (bind _player (Variables|Default|GetPlayer))
  (bind _returnvalue_2 (Transformation|GetWorldLocation _arrow1))
  (bind _returnvalue_3 (Transformation|GetWorldRotation _arrow1))
  (bind _returnvalue_4 (Transformation|GetActorLocation _player))
  (bind _returnvalue_5 (Math|Rotator|FindLookatRotation _returnvalue_2 _returnvalue_4))
  (bind _returnvalue_6 (Math|Interpolation|RInterpTo _returnvalue_3 _returnvalue_5 _returnvalue 3.0))
  ;[1 1 1] Enemy rotates to face player when the player is in range - Ryan
  (Transformation|SetActorRotation (Math|Rotator|MakeRotator 0.0 0.0 (.yaw (Math|Interpolation|RInterpTo (Transformation|GetActorRotation) (Math|Rotator|FindLookatRotation (Transformation|GetActorLocation) (Transformation|GetActorLocation (Variables|Default|GetPlayer))) (Utilities|Time|GetWorldDeltaSeconds) 3.0))))
  (Transformation|SetWorldRotation (Variables|Default|GetArrow1) (Math|Rotator|MakeRotator 0.0 (.pitch _returnvalue_6) (.yaw _returnvalue_6)) false false))

(event Custom|DigEvent
  (bind _mesh (Variables|Character|GetMesh))
  (bind _niagara (Variables|Default|GetNiagara))
  (if (Variables|Default|GetCanDig)
    (Variables|Default|SetBeforeDig (Variables|/Script/Engine.SceneComponent|GetRelativeLocation _mesh))
    (Utilities|Time|ClearandInvalidateTimerbyHandle (Variables|Default|GetCheckifPlayerCloserTimer))
    (CallFunction|ResetMove)
    (bind _newtrack_0 (Timeline|Timeline_0 PlayFromStart)
      (:Update
        (Transformation|SetRelativeLocation _mesh (Math|Vector|MakeVector 0.0 0.0 _newtrack_0) false true))
      (:Finished
        (Components|Activation|Activate _niagara false)
        (Development|SetHiddeninGame _niagara false false)
        (Collision|SetCollisionResponsetoChannel (Variables|Default|GetCapsuleComponent) "ECC_Pawn" "ECR_Ignore")
        (CallFunction|MoveAway)))))

(event Custom|UndigEvent
  (bind _niagara (Variables|Default|GetNiagara))
  (bind _newtrack_0 (Timeline|Timeline ReverseFromEnd)
    (:Update
      (Transformation|SetRelativeLocation (Variables|Character|GetMesh) (Math|Vector|MakeVector 0.0 0.0 _newtrack_0) false true))
    (:Finished
      (Components|Activation|Deactivate _niagara)
      (Development|SetHiddeninGame _niagara true false)
      (Collision|SetCollisionResponsetoChannel (Variables|Default|GetCapsuleComponent) "ECC_Pawn" "ECR_Block")
      (CallFunction|CheckifPlayerIsClose))))

(event Custom|MoveAway
  (AI|AIMoveTo (Variables|Character|GetCharacterMovement) self (.RandomLocation (AI|Navigation|GetRandomReachablePointinRadius (Transformation|GetActorLocation (Game|GetPlayerCharacter 0)) 1.5e+03 0 0)) 0 5.0 false
    (:OnSuccess
      (Utilities|FlowControl|DoOnce false
        (:Completed
          (Utilities|Time|SetTimerbyEvent (delegate Custom|UndigEvent) 2.0))))
    (:OnFail
      (CallFunction|MoveAway))))

(event Custom|Reset%20Detection
  (Utilities|FlowControl|DoOnce false) ; enters at Reset
)

(event Custom|Check%20if%20player%20is%20close
  (if (Utilities|Array|IsNotEmpty (Collision|GetOverlappingActors (Variables|Default|GetIsPlayerCloseRadius) "/Game/Blueprints/Player/BP_Player.BP_Player_C" :!class /Script/Engine.PrimitiveComponent))
    (if (Variables|Default|GetCanDig)
      (CallFunction|ResetMove)
      (CallFunction|DigEvent)
      (else
        (CallFunction|ShootProjectile :!label _label)))
    (elif (Utilities|Array|IsNotEmpty (Collision|GetOverlappingActors (Variables|Default|GetDetection%20Radius) "/Game/Blueprints/Player/BP_Player.BP_Player_C" :!class /Script/Engine.PrimitiveComponent))
      (goto _label)
      (else
        (Utilities|Time|ClearandInvalidateTimerbyHandle (Variables|Default|GetTimer%20Handle))
        (CallFunction|ResetDetection)
        (CallFunction|RandomRoam)))))

(event Custom|ShootProjectile
  (Game|SpawnActorfromClass "/Game/Blueprints/Enemies/Gordf/RangedGorf/BP_GorfProjectile.BP_GorfProjectile_C" (Transformation|GetWorldTransform (Variables|Default|GetArrow1)) "Undefined" "MultiplyWithRoot" 0 self 0)
  (bind _returnvalue (Utilities|Time|SetTimerbyEvent (delegate Custom|Check%20if%20player%20is%20close) 3.0))
  (Variables|Default|SetCheckifPlayerCloserTimer _returnvalue))

(event Custom|ResetMove
  (Utilities|FlowControl|DoOnce false) ; enters at Reset
)

(event Custom|ReplaceReset_1
  ;[1 1 1] Reset Gorfs - Susi
  (CallFunction|Unstash))

(event EventBeginPlay
  ;[1 1 1] On Begin Play, enemies will randomly roam and their return location will be their initial location by default - Ryan
  (CallFunction|SetDefaults)
  (Variables|Default|SetReturnTransform (Transformation|GetActorTransform))
  (CallFunction|RandomRoam))

(event Collision|EventActorBeginOverlap
  (params (OtherActor :type Actor%20Object%20Reference)))

(event EventTick
  (params (DeltaSeconds :type Float%20%28single-precision%29)))

(fn ConstructionScript)

(fn Stash
  (Physics|SetEnableGravity (Variables|Default|GetCapsuleComponent) false)
  (Transformation|SetActorLocation "-10000.000000,-10000.000000,-10000.000000" false true)
  (Pawn|Components|CharacterMovement|SetMovementMode (Variables|Character|GetCharacterMovement) "MOVE_Walking" 0)
  (CallFunction|RandomRoam))

(fn Unstash
  (Physics|SetEnableGravity (Variables|Default|GetCapsuleComponent) true)
  (Transformation|SetActorTransform (Variables|Default|GetSpawnTransform_0) false true)
  (Pawn|Components|CharacterMovement|SetMovementMode (Variables|Character|GetCharacterMovement) "MOVE_Walking" 0)
  (CallFunction|RandomRoam))