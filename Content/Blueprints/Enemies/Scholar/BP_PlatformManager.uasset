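; Platform manager for the Scholar encounter that moves one of three platform meshes vertically after each of the Scholar's first three attacks.
; It binds to BP_Scholar's attack-ended callback, picks the mesh by attack count and adds reversed timeline values to its Z with sweep.
; After the third move, a DoOnce spawns a teleport pickup and resets the Scholar's state.
; ResetPlatforms moves the meshes through three chained timelines, then zeroes the count.
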(event Custom|RaisePlatform
  (bind _staticmesh2 (Variables|Default|GetStaticMesh2))
  (bind _staticmesh1 (Variables|Default|GetStaticMesh1))
  (bind _staticmesh (Variables|Default|GetStaticMesh))
  (bind _number_of_attacks (Variables|Default|GetNumber%20Of%20Attacks))
  (bind _returnvalue (- _number_of_attacks 1))
  (bind _returnvalue_2 (Math|Integer|Clamp(Integer) _returnvalue 0 2))
  (bind _returnvalue_3 (Utilities|Select :Index _returnvalue_2 :Option%200 _staticmesh2 :Option%201 _staticmesh1 :Option%202 _staticmesh))
  (bind _returnvalue_4 (Transformation|GetWorldLocation _returnvalue_3))
  (bind _result (Math|Integer|IncrementInt (Variables|Default|GetNumber%20Of%20Attacks))
    (:%20%20
      (if (not (> _result 3))
        (bind _newtrack_0 (Timeline|Raise ReverseFromEnd)
          (:Update
            (Transformation|SetWorldLocation _returnvalue_3 (Math|Vector|MakeVector (.x _returnvalue_4) (.y _returnvalue_4) (+ (.z _returnvalue_4) _newtrack_0)) true false))
          (:Finished
            (if (== (- (Variables|Default|GetNumber%20Of%20Attacks) 1) 2)
              (Utilities|FlowControl|DoOnce false :!label _label
                (:Completed
                  (Game|SpawnActorfromClass "/Game/Blueprints/Mechanics/Actor/BP_TeleportPickupScholar.BP_TeleportPickupScholar_C" (Transformation|GetWorldTransform (Variables|Default|GetSphere)) "Undefined" "MultiplyWithRoot" 0 "/Game/Art/ACharacters/Models/Ben/SM_BenBase.SM_BenBase" "/Game/Blueprints/Player/Components/BPC_TeleportPickupScholar.BPC_TeleportPickupScholar_C" 0)
                  (bind _returnvalue_5 (Actor|GetActorOfClass "/Game/Blueprints/Enemies/Scholar/BP_Scholar.BP_Scholar_C"))
                  (Default|ResetState _returnvalue_5)))
              (else
                (goto _label Reset)))))))))

(event Custom|ResetPlatforms
  (bind _staticmesh (Variables|Default|GetStaticMesh))
  (bind _staticmesh1 (Variables|Default|GetStaticMesh1))
  (bind _staticmesh2 (Variables|Default|GetStaticMesh2))
  (bind _returnvalue (Transformation|GetWorldLocation _staticmesh2))
  (bind _returnvalue_2 (Transformation|GetWorldLocation _staticmesh))
  (bind _returnvalue_3 (Transformation|GetWorldLocation _staticmesh1))
  (bind _newtrack_0 (Timeline|Timeline PlayFromStart)
    (:Update
      (Transformation|SetWorldLocation _staticmesh (Math|Vector|MakeVector (.x _returnvalue_2) (.y _returnvalue_2) (+ (.z _returnvalue_2) _newtrack_0)) true false))
    (:Finished
      (bind _newtrack_0_2 (Timeline|Timeline_0 PlayFromStart)
        (:Update
          (Transformation|SetWorldLocation _staticmesh1 (Math|Vector|MakeVector (.x _returnvalue_3) (.y _returnvalue_3) (+ (.z _returnvalue_3) _newtrack_0_2)) true false))
        (:Finished
          (bind _newtrack_0_3 (Timeline|Timeline_1 PlayFromStart)
            (:Update
              (Transformation|SetWorldLocation _staticmesh2 (Math|Vector|MakeVector (.x _returnvalue) (.y _returnvalue) (+ (.z _returnvalue) _newtrack_0_3)) true false))
            (:Finished
              (Variables|Default|SetNumber%20Of%20Attacks 0))))))))

(event EventBeginPlay
  (bind _returnvalue (Actor|GetActorOfClass "/Game/Blueprints/Enemies/Scholar/BP_Scholar.BP_Scholar_C"))
  (bind _output_get (Variables|Default|SetScholar _returnvalue))
  (EventDispatchers|BindEventtoAttackEnded _output_get (delegate Custom|RaisePlatform)))

(event Collision|EventActorBeginOverlap
  (params (OtherActor :type Actor%20Object%20Reference)))

(event EventTick
  (params (DeltaSeconds :type Float%20%28single-precision%29)))

(fn ConstructionScript)