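; Scholar boss that bobs, turns toward the player while active, and fights with animated hands.
; It queues random slam and laser attacks per phase, chaining them through timers and end callbacks; the punch attack is unwired.
; Slams track the player before dropping to a traced floor point, while lasers spawn moving walls and a blocker.
; Taking damage repositions the player and resets platforms and attacks, and death shows a thanks-for-playing screen and unlocks a codex.
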(event OnComponentBeginOverlap(Sphere1)
  (params (OverlappedComponent :type Primitive%20Component%20Object%20Reference) (OtherActor :type Actor%20Object%20Reference) (OtherComp :type Primitive%20Component%20Object%20Reference) (OtherBodyIndex :type Integer) (bFromSweep :type Boolean) (SweepResult :type Hit%20Result%20Structure%20%28by%20ref%29))
  (if (== OtherActor (Variables|Default|GetPlayer))
    (Variables|Default|SetIsActive (Variables|Default|GetIsActive))))

(event OnComponentBeginOverlap(Box)
  (params (OverlappedComponent :type Primitive%20Component%20Object%20Reference) (OtherActor :type Actor%20Object%20Reference) (OtherComp :type Primitive%20Component%20Object%20Reference) (OtherBodyIndex :type Integer) (bFromSweep :type Boolean) (SweepResult :type Hit%20Result%20Structure%20%28by%20ref%29))
  ;[1 1 1] HandHitBox
  (if (Variables|Default|GetIsLeftHitboxActive)
    (Utilities|FlowControl|DoOnce false
      (:Completed
        (for _array_element (Collision|GetOverlappingActors (Variables|Default|GetBox) 0 :!class /Script/Engine.PrimitiveComponent)
          (Game|Damage|ApplyDamage _array_element (Variables|Default|GetDamageAmount) 0 self)
          (Development|PrintString (Utilities|GetDisplayName _array_element)))))))

(event OnComponentEndOverlap(Box)
  (params (OverlappedComponent :type Primitive%20Component%20Object%20Reference) (OtherActor :type Actor%20Object%20Reference) (OtherComp :type Primitive%20Component%20Object%20Reference) (OtherBodyIndex :type Integer))
  ;[1 1 1] HandHitBox
  (Utilities|FlowControl|DoOnce false) ; enters at Reset
)

(event Custom|BodyBob
  (bind _body (Variables|Default|GetBody))
  (bind _returnvalue (Transformation|GetWorldLocation _body))
  (Utilities|FlowControl|FlipFlop
    (:A
      (bind _newtrack_0 (Timeline|BobTimeLine PlayFromStart)
        (:Update
          (Transformation|SetWorldLocation _body (Math|Vector|MakeVector (.x _returnvalue) (.y _returnvalue) (+ (* _newtrack_0 2.5) (.z _returnvalue))) true false))
        (:Finished
          (CallFunction|BodyBob))))
    (:B
      (Timeline|BobTimeLine ReverseFromEnd))))

(event Custom|LookAt
  (Transformation|SetWorldRotation (Variables|Default|GetSphere) (Math|Rotator|MakeRotator 0.0 0.0 (.yaw (Math|Rotator|FindLookatRotation (Transformation|GetActorLocation) (Transformation|GetActorLocation (Variables|Default|GetPlayer))))) false false))

(event Custom|SelectAttacksForPhase
  (for _index (range 0 (Variables|Default|GetNumberOfAttacksForPhase))
    (Utilities|Array|Add (Variables|Default|GetAttacksForPhase) (Utilities|Select :Index (Math|Random|RandomIntegerinRange 0 1) :Option%200 "NewEnumerator0" :Option%201 "NewEnumerator2")))
  (Variables|Default|SetNumberOfAttacksForPhase 2)
  (CallFunction|DotheAttack))

(event Custom|ResetState
  (Utilities|Time|ClearandInvalidateTimerbyHandle (stale Custom|SlamAttackStart _returnvalue))
  (Utilities|Time|ClearandInvalidateTimerbyHandle (stale Custom|SlamAttack _returnvalue_2))
  (Utilities|Time|ClearandInvalidateTimerbyHandle (stale Custom|DoTheAttack _returnvalue_2))
  (Variables|Default|SetIsIdle true))

(event Custom|Death
  (bind _returnvalue (Transformation|GetActorTransform))
  (bind _returnvalue_2 (Game|GetPlayerController 0))
  (Utilities|FlowControl|Sequence
    (:then_0
      (Utilities|FlowControl|Delay 0.2)
      (Audio|PlaySound2D "/Game/Sounds/SFX/BossFunnyDeath.BossFunnyDeath" 1.0 1.0 0.0 0 0))
    (:then_1
      (bind _height (Timeline|RISE%20MY%20SON PlayFromStart)
        (:Update
          (Transformation|SetActorTransform (Math|Transform|MakeTransform (Math|Vector|MakeVector (.x (.location _returnvalue)) (.y (.location _returnvalue)) (+ (.z (.location _returnvalue)) (* _height 1e+01))) (.rotation _returnvalue) "1.000000,1.000000,1.000000") true))
        (:Finished
          (Utilities|FlowControl|Delay 2.0)
          (bind _returnvalue_3 (UserInterface|CreateWidget "/Game/UI/Widgets/Menus/CUIWB_ThanksForPlaying.CUIWB_ThanksForPlaying_C" (Game|GetPlayerController 0)))
          (UserInterface|Viewport|AddtoViewport _returnvalue_3 0)
          (Input|SetInputModeGameandUI _returnvalue_2 _returnvalue_3 "DoNotLock" true false)
          (Variables|/Script/Engine.PlayerController|SetbShowMouseCursor _returnvalue_2 true)
          (Default|Unlock (Variables|Default|GetCodexToUnlock)))))))

(event Custom|PunchAttackStart
  (Variables|Default|SetHandRightLocation (Transformation|GetWorldLocation (Variables|Default|GetSphere)))
  (Utilities|Time|SetTimerbyEvent (delegate Custom|InitiatePunchAttack) 2.0))

(event Custom|InitiatePunchAttack
  (Variables|Default|SetHandRightLocation (* (Math|Vector|GetForwardVector (Variables|Default|GetRightHand)) 5e+01))
  (Variables|Default|SetIsRightHitboxActive true)
  (Utilities|Time|SetTimerbyEvent (delegate Custom|EndPunchAttack) 2.0))

(event Custom|EndPunchAttack
  (Variables|Default|SetHandRightLocation (Transformation|GetWorldLocation (Variables|Default|GetRightHandIdle)))
  (Variables|Default|SetIsRightHitboxActive false)
  (Default|CallAttackEnded)
  (CallFunction|DotheAttack))

(event Custom|SlamAttackStart
  ;[1 1 1] SlamAttack///Swaps between animation states and attack steps
  (Components|Animation|PlayAnimation (Variables|Default|GetLeftHand) "/Game/Art/ScholarHandsTemp/HANDSLAMATTACKSTARTTEST.HANDSLAMATTACKSTARTTEST" false)
  (bind _returnvalue (Utilities|Time|SetTimerbyEvent (delegate Custom|SlamAttack) 0.01 true)))

(event Custom|TakeDamage
  (bind _player (Variables|Default|GetPlayer))
  (Math|Integer|DecrementInt (Variables|Default|GetHealth)
    (:%20%20
      (Input|DisableInput _player 0)
      (bind _newtrack_0 (Timeline|Timeline Play)
        (:Update
          (Transformation|SetActorLocationAndRotation _player (Math|Interpolation|VInterpTo (Transformation|GetActorLocation _player) "800.000000,420.000000,230.000000" _newtrack_0 5.0) (Math|Interpolation|RInterpTo (Transformation|GetActorRotation _player) "0.000000,270.000000,0.000000" _newtrack_0 5.0) false true))
        (:Finished
          (Input|EnableInput _player 0)
          (Default|ResetPlatforms (Variables|Default|GetPlatformManager))
          (CallFunction|ResetState)
          (if (<= (Variables|Default|GetHealth) 0)
            (CallFunction|Death)
            (Development|PrintString "MAN IM DEAD 
")
            (else
              (Utilities|FlowControl|Delay 1.0)
              (CallFunction|DotheAttack))))))))

(event Custom|SlamAttack
  (bind _player (Variables|Default|GetPlayer))
  (bind _lefthand (Variables|Default|GetLeftHand))
  (bind _returnvalue (Transformation|GetWorldLocation _lefthand))
  ;[1 1 1] SlamAttack///Swaps between animation states and attack steps
  (Variables|Default|SetIsIdle false)
  (Variables|Default|SetHandLeftLocation (+ (* (Transformation|GetActorUpVector _player) (Variables|Default|GetHandHoverHeight)) (Transformation|GetActorLocation _player)))
  (if (not (Audio|Components|Audio|IsPlaying (Variables|Default|GetLeftHand)))
    (Utilities|Time|ClearandInvalidateTimerbyHandle (stale Custom|SlamAttackStart _returnvalue))
    (Utilities|FlowControl|Delay (Variables|Default|GetAttackHoldTime))
    (Variables|Default|SetIsLeftHitboxActive true)
    (bind _outhit (Collision|LineTraceByChannel _returnvalue (+ _returnvalue (* (Math|Vector|VectorUp) -5e+03)) "TraceTypeQuery1" false (Utilities|Array|MakeArray (Variables|Default|GetPlayer)) "None"))
    (Variables|Default|SetHandLeftLocation (.impactpoint _outhit))
    (Components|Animation|PlayAnimation (Variables|Default|GetLeftHand) "/Game/Art/ScholarHandsTemp/Hand_Anim_Armature_SlamAttackTest.Hand_Anim_Armature_SlamAttackTest" false)
    (bind _returnvalue_2 (Utilities|Time|SetTimerbyEvent (delegate Custom|EndSlamAttack) 1.0 false false 2.0))))

(event Custom|EndSlamAttack
  ;[1 1 1] SlamAttack///Swaps between animation states and attack steps
  (Variables|Default|SetIsIdle true)
  (Variables|Default|SetIsLeftHitboxActive false)
  (Variables|Default|SetHandLeftLocation (Transformation|GetWorldLocation (Variables|Default|GetLeftHandIdle)))
  (Components|Animation|PlayAnimation (Variables|Default|GetLeftHand) "/Game/Art/ScholarHandsTemp/Hand_Anim_Armature_Idle.Hand_Anim_Armature_Idle" false)
  (Default|CallAttackEnded)
  (CallFunction|DotheAttack))

(event Custom|LaserAttackStart
  (bind _redirectorcubespawn (Variables|Default|GetRedirectorCubeSpawn))
  (bind _returnvalue (Transformation|GetWorldTransform _redirectorcubespawn))
  ;[1 1 1] LaserAttack
  (for _array_element (Utilities|Array|MakeArray (Variables|Default|GetLaserWallStart) (Variables|Default|GetLaserWallStart1) (Variables|Default|GetLaserWallStart2) (Variables|Default|GetLaserWallStart3) (Variables|Default|GetLaserWallStart4))
    (bind _returnvalue_2 (Game|SpawnActorfromClass "/Game/Blueprints/Level/Environment/Lazers/LaserWall.LaserWall_C" (Transformation|GetWorldTransform _array_element) "Undefined" "MultiplyWithRoot" 0 -4e+03 (Variables|Default|GetTime%20to%20FinishLaserAttack) 0))
    (EventDispatchers|BindEventtoReachedEndPoint _returnvalue_2 (delegate Custom|LaserAttackEnd)))
  (Game|SpawnActorfromClass "/Game/Art/Environment/Architecture/World_2/W2Level1/section9/blockerwall.blockerwall_C" (Math|Transform|MakeTransform (.location _returnvalue) (.rotation _returnvalue) "2.000000,2.000000,2.000000") "Undefined" "MultiplyWithRoot" 0 0))

(event Custom|DoTheAttack
  (bind _attacksforphase (Variables|Default|GetAttacksForPhase))
  (bind _returnvalue (Utilities|Array|Length _attacksforphase))
  (Development|PrintString (Utilities|String|ToString(Integer) _returnvalue))
  (if (== _returnvalue 0)
    (Default|CallPhaseEnded)
    (CallFunction|SelectAttacksforPhase)
    (else
      (Variables|Default|SetSelectedAttack (Utilities|Array|Get(acopy) _attacksforphase))
      (Utilities|Array|RemoveIndex _attacksforphase)
      (bind _returnvalue_2 (Utilities|Time|SetTimerbyEvent (delegate Custom|InitializeAttack) (Variables|Default|GetTimeTillNextAttack))))))

(event Custom|InitializeAttack
  (switch Utilities|FlowControl|Switch|SwitchonAttacks (Variables|Default|GetSelectedAttack)
    (:NewEnumerator0
      (CallFunction|SlamAttackStart))
    (:NewEnumerator2
      (CallFunction|LaserAttackStart))))

(event Custom|LaserAttackEnd
  ;[1 1 1] LaserAttack
  (EventDispatchers|UnbindallEventsfromReachedEndPoint (stale Custom|LaserAttackStart _returnvalue_2))
  (bind _outactors (Actor|GetAllActorsOfClass "/Game/Blueprints/Level/Environment/Lazers/LaserWall.LaserWall_C"))
  (for _array_element _outactors
    (Actor|DestroyActor _array_element))
  (bind _outactors_2 (Actor|GetAllActorsOfClass "/Game/Art/Environment/Architecture/World_2/W2Level1/section9/blockerwall.blockerwall_C"))
  (for _array_element_2 _outactors_2
    (Actor|DestroyActor _array_element_2))
  (Default|CallAttackEnded)
  (CallFunction|DotheAttack))

(event EventBeginPlay
  (CallFunction|BodyBob)
  (Variables|Default|SetPlayer (Game|Player|GetPlayerPawn 0))
  (bind _returnvalue (Actor|GetActorOfClass "/Game/Blueprints/Enemies/Scholar/BP_PlatformManager.BP_PlatformManager_C"))
  (Variables|Default|SetPlatformManager _returnvalue)
  (Components|Animation|PlayAnimation (Variables|Default|GetRightHand) "/Game/Art/ScholarHandsTemp/Hand_Anim_Armature_Idle.Hand_Anim_Armature_Idle" false)
  (Components|Animation|PlayAnimation (Variables|Default|GetLeftHand) "/Game/Art/ScholarHandsTemp/Hand_Anim_Armature_Idle.Hand_Anim_Armature_Idle" false)
  (CallFunction|SelectAttacksforPhase))

(event Collision|EventActorBeginOverlap
  (params (OtherActor :type Actor%20Object%20Reference)))

(event EventTick
  (params (DeltaSeconds :type Float%20%28single-precision%29))
  (bind _lefthand (Variables|Default|GetLeftHand))
  (if (Variables|Default|GetIsActive)
    (CallFunction|Lookat)
    (Transformation|SetWorldLocation _lefthand (Math|Interpolation|VInterpTo (Transformation|GetWorldLocation _lefthand) (Math|Vector|SelectVector (Transformation|GetWorldLocation (Variables|Default|GetLeftHandIdle)) (Variables|Default|GetHandLeftLocation) (Variables|Default|GetIsIdle)) DeltaSeconds (Math|Float|SelectFloat 3.0 5.0 (Variables|Default|GetIsIdle))) true false)))

(fn ConstructionScript)