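; Boss key pickup that marks the end of a level and sends the player back to a hub.
; On pickup it starts a camera fade and saves any level codex entries through the game instance, calling the parent pickup and exit logic inside that loop.
; It saves gold flies, then opens the hub matching the save's PreviousHubLevel, defaulting to HubWorld.
; The delay and thanks-for-playing screen are disconnected.
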(event EventBeginPlay
  (|CallParentFunction) ; This node is disabled and will not be called.\nDrag off pins to build functionality.
)

(event Collision|EventActorBeginOverlap
  (params (OtherActor :type Actor%20Object%20Reference))
  (|CallParentFunction OtherActor) ; This node is disabled and will not be called.\nDrag off pins to build functionality.
)

(event EventTick
  (params (DeltaSeconds :type Float%20%28single-precision%29))
  (|CallParentFunction DeltaSeconds) ; This node is disabled and will not be called.\nDrag off pins to build functionality.
)

(event EventOnPickup
  (params (Player :type BP%20Player%20Object%20Reference))
  (bind _returnvalue (Game|GetGameInstance))
  (bind _codexes (Variables|Default|GetCodexes))
  (bind _codexes_2 (Variables|/Game/Maps/CodexUnlocks/CodexsToUnlock.CodexsToUnlock_C|GetCodexes _codexes))
  ;[1 1 1] Boss Key marks the end of the level, so it will unlock the story entry if it wasn't unlocked already and then bring you back to the hub with the currency persisting - Ryan
  (CameraFades|StartCameraFade :self (Game|GetPlayerCameraManager 0) :ToAlpha 2.0 :Duration 2.0 :bHoldWhenFinished true)
  (if (Utilities|Array|IsNotEmpty _codexes_2)
    (for _array_element _codexes_2
      (Class|BPISaveGameInterface|SaveLevelCodexes(Message) (Game|GetGameInstance) _array_element)
      (|CallParentFunction 0)
      (Class|BPISaveGameInterface|SavePlayerData(Message) _returnvalue (Utilities|Struct|MakeS_PlayerData "0.000000,0.000000,0.000000|0.000000,0.000000,0.000000|1.000000,1.000000,1.000000" 3 (Variables|/Game/Blueprints/Player/BP_Player.BP_Player_C|GetGoldFlies Player)) false)
      (bind _asbp_game_instance (Utilities|Casting|CastToBP_GameInstance _returnvalue))
      (switch int (Variables|/Game/Blueprints/Saving/BP_SaveGame.BP_SaveGame_C|GetPreviousHubLevel (Variables|/Game/Blueprints/Saving/BP_GameInstance.BP_GameInstance_C|GetSaveGame _asbp_game_instance))
        (:Default
          (Game|OpenLevel(byObjectReference) "/Game/Maps/HubWorld/HubWorld.HubWorld" true "Default"))
        (:0
          (Game|OpenLevel(byObjectReference) "/Game/Maps/HubWorld/world1entrance/1-Hub.1-Hub"))
        (:1
          (Game|OpenLevel(byObjectReference) "/Game/Maps/HubWorld/world2entrance/2-Hub.2-Hub"))
        (:2
          (Game|OpenLevel(byObjectReference) "/Game/Maps/HubWorld/world3entrance/3-Hub.3-Hub"))))
    (else
      (|CallParentFunction 0)
      (Class|BPISaveGameInterface|SavePlayerData(Message) _returnvalue (Utilities|Struct|MakeS_PlayerData "0.000000,0.000000,0.000000|0.000000,0.000000,0.000000|1.000000,1.000000,1.000000" 3 (Variables|/Game/Blueprints/Player/BP_Player.BP_Player_C|GetGoldFlies Player)) false)
      (bind _asbp_game_instance_2 (Utilities|Casting|CastToBP_GameInstance _returnvalue))
      (switch int (Variables|/Game/Blueprints/Saving/BP_SaveGame.BP_SaveGame_C|GetPreviousHubLevel (Variables|/Game/Blueprints/Saving/BP_GameInstance.BP_GameInstance_C|GetSaveGame _asbp_game_instance_2))
        (:Default
          (Game|OpenLevel(byObjectReference) "/Game/Maps/HubWorld/HubWorld.HubWorld" true "Default"))
        (:0
          (Game|OpenLevel(byObjectReference) "/Game/Maps/HubWorld/world1entrance/1-Hub.1-Hub"))
        (:1
          (Game|OpenLevel(byObjectReference) "/Game/Maps/HubWorld/world2entrance/2-Hub.2-Hub"))
        (:2
          (Game|OpenLevel(byObjectReference) "/Game/Maps/HubWorld/world3entrance/3-Hub.3-Hub"))))))

(fn ConstructionScript
  (|CallParentFunction))