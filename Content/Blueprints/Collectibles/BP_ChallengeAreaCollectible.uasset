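; BP_ChallengeAreaCollectible is the pickup that ends a challenge area (time trial) and sends the player back to the hub.
; On pickup it saves its collectible unlock to the game instance and the player's gold flies, then plays a level sequence.
; After a fixed delay it async-loads the hub level behind a loading-image widget with UI-only input, notifying the widget when loading completes.
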(event Custom|LoadHub
  (bind _level_to_load (Variables|Default|GetLevel%20to%20Load))
  (bind _worldasset (Utilities|Struct|BreakSoftWorldReference _level_to_load))
  (Utilities|AsyncLoadAsset _worldasset
    (:then
      (bind _returnvalue (UserInterface|CreateWidget "/Game/UI/Widgets/LevelLoad/LoadWithImage.LoadWithImage_C" (Game|GetPlayerController 0) "/Game/Art/LevelScreens/HubHigh.HubHigh" (Utilities|Struct|MakeSoftWorldReference _worldasset) "Hub"))
      (UserInterface|Viewport|AddtoViewport _returnvalue 0)
      (Input|SetInputModeUIOnly (Game|GetPlayerController 0) _returnvalue "DoNotLock" true))
    (:Completed
      (Default|LoadDone _returnvalue))))

(event EventOnPickup
  (params (Player :type BP%20Player%20Object%20Reference))
  ;[1 1 1] If the player completes the time trial, this fact gets saved, and they get sent back to the hub - Ryan
  (|CallParentFunction Player)
  (bind _asbp_game_instance (Utilities|Casting|CastToBP_GameInstance (Game|GetGameInstance)))
  (Default|SaveChallengeAreaCollectibles _asbp_game_instance (Variables|Default|GetCollectibleUnlock))
  (Class|BPISaveGameInterface|SavePlayerData(Message) Player (Utilities|Struct|MakeS_PlayerData "0.000000,0.000000,0.000000|0.000000,0.000000,0.000000|1.000000,1.000000,1.000000" 3 (Variables|/Game/Blueprints/Player/BP_Player.BP_Player_C|GetGoldFlies Player)) false)
  (Sequencer|Player|Play (Variables|/Script/LevelSequence.LevelSequenceActor|GetSequencePlayer (Variables|Default|GetLevelSequence)) :!class /Script/MovieScene.MovieSceneSequencePlayer)
  (Utilities|FlowControl|Delay 5.5)
  (CallFunction|LoadHub))

(fn ConstructionScript
  (|CallParentFunction))