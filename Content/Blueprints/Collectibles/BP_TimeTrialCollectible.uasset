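; Time trial side-quest collectible that starts hidden without collision and, when picked up, completes the trial and returns the player to the hub.
; Pickup saves the unlock and gold flies through the game instance, clears the NPC's timer and widgets, and destroys EmptyGorf actors.
; It then plays an end sequence and, after a delay, async-loads the level behind a loading-screen widget.
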(event Custom|LoadHub
  (Utilities|AsyncLoadAsset (Utilities|Struct|BreakSoftWorldReference (Variables|Default|GetLevel%20to%20Load))
    (:then
      (bind _returnvalue (UserInterface|CreateWidget "/Game/UI/Widgets/LevelLoad/LoadWithImage.LoadWithImage_C" (Game|GetPlayerController 0) "/Game/Art/LevelScreens/HubHigh.HubHigh" (Utilities|Struct|MakeSoftWorldReference "/Game/Maps/HubWorld/HubWorld.HubWorld") "Hub"))
      (UserInterface|Viewport|AddtoViewport _returnvalue 0)
      (Input|SetInputModeUIOnly (Game|GetPlayerController 0) _returnvalue "DoNotLock" true))
    (:Completed
      (Default|LoadDone _returnvalue))))

(event EventBeginPlay
  ;[1 1 1] Side quest collectible starts hidden - Ryan
  (Collision|SetCollisionEnabled (Variables|Default|GetSphere) "NoCollision")
  (Components|Activation|SetActive (Variables|Character|GetMesh) false false)
  (Development|SetHiddeninGame (Variables|Character|GetMesh) true false)
  (|CallParentFunction))

(event Collision|EventActorBeginOverlap
  (params (OtherActor :type Actor%20Object%20Reference))
  (|CallParentFunction OtherActor) ; This node is disabled and will not be called.\nDrag off pins to build functionality.
)

(event EventTick
  (params (DeltaSeconds :type Float%20%28single-precision%29))
  (|CallParentFunction DeltaSeconds) ; This node is disabled and will not be called.\nDrag off pins to build functionality.
)

(event EventOnPickup
  (params (Player :type BP%20Player%20Object%20Reference))
  ;[1 1 1] If the player completes the time trial, this fact gets saved, and they get sent back to the hub - Ryan
  (bind _foundwidgets (Widget|GetAllWidgetsOfClass "/Game/UI/Widgets/HUD/WB_Timer.WB_Timer_C" true))
  (for _array_element _foundwidgets
    (Widget|RemovefromParent _array_element)
    (|CallParentFunction Player)
    (bind _asbp_game_instance (Utilities|Casting|CastToBP_GameInstance (Game|GetGameInstance)))
    (Default|SaveTimeTrialCollectibles _asbp_game_instance (Variables|Default|GetCollectibleUnlock))
    (bind _playersave (Default|GetPlayerData Player))
    (Class|BPISaveGameInterface|SavePlayerData(Message) (Game|GetGameInstance) (Utilities|Struct|MakeS_PlayerData "0.000000,0.000000,0.000000|0.000000,0.000000,0.000000|1.000000,1.000000,1.000000" 3 (.goldflies _playersave)) false)
    (bind _returnvalue (Actor|GetActorOfClass "/Game/Blueprints/NPCs/BP_TimeTrialNPC.BP_TimeTrialNPC_C"))
    (Utilities|Time|ClearandInvalidateTimerbyHandle (Variables|/Game/UI/Widgets/HUD/WB_Timer.WB_Timer_C|GetTimeTrialTimer (Variables|/Game/Blueprints/NPCs/BP_TimeTrialNPC.BP_TimeTrialNPC_C|GetTimer%20Widget _returnvalue)))
    (Widget|RemovefromParent (Variables|/Game/Blueprints/NPCs/BP_TimeTrialNPC.BP_TimeTrialNPC_C|GetTimer%20Widget _returnvalue))
    (Default|CallPickedUp)
    (bind _outactors (Actor|GetAllActorsOfClass "/Game/Blueprints/Enemies/Gordf/EmptyGorf.EmptyGorf_C"))
    (for _array_element_2 _outactors
      (Actor|DestroyActor _array_element_2))
    (Sequencer|Player|Play (Variables|/Script/LevelSequence.LevelSequenceActor|GetSequencePlayer (Variables|Default|GetEndSequence)) :!class /Script/MovieScene.MovieSceneSequencePlayer)
    (Utilities|FlowControl|Delay 5.5)
    (CallFunction|LoadHub)))

(fn ConstructionScript
  (|CallParentFunction))