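; BP_SidequestCollectible is a side quest collectible, a child Blueprint that extends inherited pickup behavior.
; On BeginPlay it starts hidden, with sphere collision disabled and its mesh deactivated; nothing in this file re-enables it.
; On pickup it removes every top-level WB_Timer widget from the screen.
; The parent pickup call sits inside that loop, so it runs once per timer found and not at all without one.
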(event EventBeginPlay
  ;[1 1 1] Side quest collectible starts hidden - Ryan
  (Collision|SetCollisionEnabled (Variables|Default|GetSphere) "NoCollision")
  (Components|Activation|SetActive (Variables|Character|GetMesh) false false)
  (Development|SetHiddeninGame (Variables|Character|GetMesh) true false)
  (|CallParentFunction))

(event Collision|EventActorBeginOverlap
  (params (OtherActor :type Actor%20Object%20Reference))
  (|CallParentFunction OtherActor) ; This node is disabled and will not be called.\nDrag off pins to build functionality.
)

(event EventTick
  (params (DeltaSeconds :type Float%20%28single-precision%29))
  (|CallParentFunction DeltaSeconds) ; This node is disabled and will not be called.\nDrag off pins to build functionality.
)

(event EventOnPickup
  (params (Player :type BP%20Player%20Object%20Reference))
  ;[1 1 1] If the collectible is picked up, removes timer from screen - Ryan
  (bind _foundwidgets (Widget|GetAllWidgetsOfClass "/Game/UI/Widgets/HUD/WB_Timer.WB_Timer_C" true))
  (for _array_element _foundwidgets
    (Widget|RemovefromParent _array_element)
    (|CallParentFunction 0)))

(fn ConstructionScript
  (|CallParentFunction))