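; Refugee Cate collectible that unlocks a linked Codex entry and counts toward the level's rescue progress when picked up.
; On BeginPlay it destroys itself after a brief delay if that entry is already unlocked, so found Cates do not reappear.
; On pickup it increments the collected count in PlatformingGameMode, refreshes and animates the player's HUD tracker, then runs the parent pickup logic.
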(event EventBeginPlay
  (bind _codextounlock (Variables|Default|GetCodexToUnlock))
  ;[1 1 1] If this collectible has been found already, destroy it - Ryan
  (Utilities|IsValid _codextounlock
    (:Is%20Valid
      (if (Variables|/Game/UI/Blueprints/BP_CodexEntry.BP_CodexEntry_C|GetUnlocked _codextounlock)
        (Utilities|FlowControl|Delay 0.1)
        (Actor|DestroyActor)))))

(event Collision|EventActorBeginOverlap
  (params (OtherActor :type Actor%20Object%20Reference))
  (|CallParentFunction OtherActor) ; This node is disabled and will not be called.\nDrag off pins to build functionality.
)

(event EventTick
  (params (DeltaSeconds :type Float%20%28single-precision%29))
  (|CallParentFunction DeltaSeconds) ; This node is disabled and will not be called.\nDrag off pins to build functionality.
)

(event EventOnPickup
  (params (Player :type BP%20Player%20Object%20Reference))
  (bind _collectibleshud (Variables|/Game/Blueprints/Player/BP_Player.BP_Player_C|GetCollectiblesHUD Player))
  ;[1 1 1] Unlocks Codex Entry on Pickup, and updates the current level's progress of collected Refugee Cates - Ryan
  (Default|Unlock (Variables|Default|GetCodexToUnlock))
  (bind _asplatforming_game_mode (Utilities|Casting|CastToPlatformingGameMode (Game|GetGameMode)))
  (bind _result (Math|Integer|IncrementInt (Variables|/Game/GameModes/PlatformingGameMode.PlatformingGameMode_C|GetCollectedRefugeeCates _asplatforming_game_mode))
    (:%20%20
      (bind _output_get (Variables|/Game/GameModes/PlatformingGameMode.PlatformingGameMode_C|SetCollectedRefugeeCates _asplatforming_game_mode _result))
      (Variables|/Script/UMG.TextBlock|SetText (Variables|/Game/UI/Widgets/HUD/WB_CollectiblesHUD.WB_CollectiblesHUD_C|GetRefugeeCateTracker _collectibleshud) (Utilities|Text|FormatText "Refugee Cates: {X}/{Y}" _output_get (Variables|/Game/GameModes/PlatformingGameMode.PlatformingGameMode_C|GetTotalRefugeeCates _asplatforming_game_mode)))
      (UserInterface|Animation|PlayAnimation _collectibleshud (Variables|/Game/UI/Widgets/HUD/WB_CollectiblesHUD.WB_CollectiblesHUD_C|GetRefugeeCateUpdate _collectibleshud) 0.0 1 "Forward" 1.0 true)
      (|CallParentFunction 0))))

(fn ConstructionScript
  (|CallParentFunction))