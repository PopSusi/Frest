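; BP_BaseCollectible is the base collectible actor, picked up when the player overlaps it.
; Sphere overlap casts the other actor to BP_Player and passes it to the OnPickup event.
; OnPickup hides the mesh, disables sphere collision and plays one of two random pop sounds, without destroying the actor or saving.
; The construction script creates and stores a dynamic material instance for the mesh.
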(event OnComponentBeginOverlap(Sphere)
  (params (OverlappedComponent :type Primitive%20Component%20Object%20Reference) (OtherActor :type Actor%20Object%20Reference) (OtherComp :type Primitive%20Component%20Object%20Reference) (OtherBodyIndex :type Integer) (bFromSweep :type Boolean) (SweepResult :type Hit%20Result%20Structure%20%28by%20ref%29))
  ;[1 1 1] Base Collectible Functionality: Check for Player overlap and destroy the collectible - Ryan
  (bind _asbp_player (Utilities|Casting|CastToBP_Player OtherActor))
  (CallFunction|OnPickup _asbp_player))

(event Custom|On%20Pickup
  (params (Player :type BP%20Player%20Object%20Reference))
  ;[1 1 1] When a collectible is picked up, it is destroyed, and the save file is updated - Ryan
  (Rendering|SetVisibility (Variables|Default|GetMesh) false false)
  (Collision|SetCollisionEnabled (Variables|Default|GetSphere) "NoCollision")
  (Audio|PlaySound2D (select (Math|Random|RandomBool) "/Game/Sounds/SFX/Pickup/Pop2.Pop2" "/Game/Sounds/SFX/Pickup/Pop.Pop") 1.0 1.0 0.0 0 0))

(event EventBeginPlay)

(event Collision|EventActorBeginOverlap
  (params (OtherActor :type Actor%20Object%20Reference)))

(event EventTick
  (params (DeltaSeconds :type Float%20%28single-precision%29)))

(fn ConstructionScript
  (bind _returnvalue (Rendering|Material|CreateDynamicMaterialInstance (Variables|Default|GetMesh) 0 0 "None" :!class /Script/Engine.PrimitiveComponent))
  (Variables|Default|SetMaterial _returnvalue))