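; BP_KeyCodexEntryCollectible is a collectible that unlocks an associated codex entry when picked up.
; On BeginPlay it destroys itself if CodexToUnlock is already unlocked, so an obtained entry's pickup does not remain in the level.
; OnPickup calls Unlock on CodexToUnlock before handing off to the parent pickup logic.
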(event EventBeginPlay
  (if (Variables|/Game/UI/Blueprints/BP_CodexEntry.BP_CodexEntry_C|GetUnlocked (Variables|Default|GetCodexToUnlock))
    (Actor|DestroyActor)))

(event Collision|EventActorBeginOverlap
  (params (OtherActor :type Actor%20Object%20Reference))
  (|CallParentFunction OtherActor) ; This node is disabled and will not be called.\nDrag off pins to build functionality.
)

(event EventTick
  (params (DeltaSeconds :type Float%20%28single-precision%29))
  (|CallParentFunction DeltaSeconds) ; This node is disabled and will not be called.\nDrag off pins to build functionality.
)

(event EventOnPickup
  (params (Player :type BP%20Player%20Object%20Reference))
  ;[1 1 1] Unlock Associated Codex Entry On Pickup Before Getting Destroyed - Ryan
  (Default|Unlock (Variables|Default|GetCodexToUnlock))
  (|CallParentFunction 0))

(fn ConstructionScript
  (|CallParentFunction))