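; Gold Fly collectible that adds one to the player's GoldFlies currency on pickup and updates the HUD count.
; Pickup plays an effect and a mono/stereo 2D sound, then disables collision and hides the mesh rather than destroying the actor; FuckReset restores it.
; The HUD GoldFlyUpdate animation restarts according to its current time, mirroring the time during its outro so rapid pickups blend smoothly.
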(event Custom|FuckReset
  (bind _mesh (Variables|Character|GetMesh))
  ;[1 1 1] Everytime a Gold Fly is picked up, it gets added to the Player's total currency, and saved to the Save File. This value will persist between loading levels - Ryan
  (Collision|SetCollisionEnabled (Variables|Default|GetSphere) "QueryAndPhysics")
  (Components|Activation|SetActive _mesh true false)
  (Development|SetHiddeninGame _mesh false false))

(event EventBeginPlay)

(event EventOnPickup
  (params (Player :type BP%20Player%20Object%20Reference))
  (bind _hud (Variables|/Game/Blueprints/Player/BP_Player.BP_Player_C|GetHUD Player))
  (bind _mesh (Variables|Character|GetMesh))
  (bind _goldflyupdate (Variables|/Game/UI/Widgets/HUD/WB_HUD.WB_HUD_C|GetGoldFlyUpdate _hud))
  (bind _returnvalue (Class|UserWidget|GetAnimationCurrentTime _hud _goldflyupdate))
  ;[1 1 1] Everytime a Gold Fly is picked up, it gets added to the Player's total currency, and saved to the Save File. This value will persist between loading levels - Ryan
  (Components|Activation|Activate (Variables|Default|GetCollectFX) false)
  (bind _result (Math|Integer|IncrementInt (Variables|/Game/Blueprints/Player/BP_Player.BP_Player_C|GetGoldFlies Player))
    (:%20%20
      (bind _output_get (Variables|/Game/Blueprints/Player/BP_Player.BP_Player_C|SetGoldFlies Player _result))
      (Variables|/Script/UMG.TextBlock|SetText (Variables|/Game/UI/Widgets/HUD/WB_HUD.WB_HUD_C|GetGoldFlyCount _hud) (Utilities|Text|ToText(Integer) _output_get))
      (Collision|SetCollisionEnabled (Variables|Default|GetSphere) "NoCollision")
      (Components|Activation|SetActive _mesh false false)
      (CallFunction|PlayFrestSound2D "/Game/Sounds/MetaSounds/MS_CollectibleMono.MS_CollectibleMono" "/Game/Sounds/MetaSounds/MS_CollectibleStereo.MS_CollectibleStereo")
      (Development|SetHiddeninGame _mesh true false)
      (if (or (<= _returnvalue 0.0) (>= _returnvalue 4.0))
        (UserInterface|Animation|PlayAnimation _hud _goldflyupdate 0.0 1 "Forward" 1.0 true)
        (elif (not (and (> _returnvalue 0.0) (< _returnvalue 0.5)))
          (if (and (> _returnvalue 3.5) (< _returnvalue 4.0))
            (UserInterface|Animation|PlayAnimation _hud _goldflyupdate (* (- _returnvalue 4.0) -1.0) 1 "Forward" 1.0 true)
            (else
              (UserInterface|Animation|PlayAnimation _hud _goldflyupdate 0.5 1 "Forward" 1.0 true))))))))

(fn ConstructionScript
  (|CallParentFunction))