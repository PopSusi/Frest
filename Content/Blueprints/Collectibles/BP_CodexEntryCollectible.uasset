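; Collectible codex page pickup that unlocks its assigned codex entry in the platforming game.
; On BeginPlay it destroys itself after a short delay if that entry is already unlocked.
; On pickup it unlocks the entry, increments the game mode's collected page count, updates the player's codex page tracker text, runs the parent pickup logic and plays one of two random pop sounds.
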(event EventBeginPlay
  (bind _codextounlock (Variables|Default|GetCodexToUnlock))
  ;[1 1 1] Destroy this collectible if it has already been collected - Ryan
  (Utilities|IsValid _codextounlock
    (:Is%20Valid
      (if (Variables|/Game/UI/Blueprints/BP_CodexEntry.BP_CodexEntry_C|GetUnlocked _codextounlock)
        (Utilities|FlowControl|Delay 0.1)
        (Actor|DestroyActor)))))

(event Collision|EventActorBeginOverlap
  (params (OtherActor :type Actor%20Object%20Reference))
  (|CallParentFunction OtherActor) ; This node is disabled and will not be called.\nDrag off pins to build functionality.
)

(event EventTick
  (params (DeltaSeconds :type Float%20%28single-precision%29))
  (|CallParentFunction DeltaSeconds) ; This node is disabled and will not be called.\nDrag off pins to build functionality.
)

(event EventOnPickup
  (params (Player :type BP%20Player%20Object%20Reference))
  (bind _codextounlock (Variables|Default|GetCodexToUnlock))
  ;[1 1 1] Unlock Associated Codex Entry On Pickup Before Getting Destroyed - Ryan
  (Utilities|IsValid _codextounlock
    (:Is%20Valid
      (Default|Unlock _codextounlock)
      (bind _asplatforming_game_mode (Utilities|Casting|CastToPlatformingGameMode (Game|GetGameMode)))
      (bind _result (Math|Integer|IncrementInt (Variables|/Game/GameModes/PlatformingGameMode.PlatformingGameMode_C|GetCollectedCodexPages _asplatforming_game_mode))
        (:%20%20
          (bind _output_get (Variables|/Game/GameModes/PlatformingGameMode.PlatformingGameMode_C|SetCollectedCodexPages _asplatforming_game_mode _result))
          (Variables|/Script/UMG.TextBlock|SetText (Variables|/Game/UI/Widgets/HUD/WB_CollectiblesHUD.WB_CollectiblesHUD_C|GetCodexPageTracker (Variables|/Game/Blueprints/Player/BP_Player.BP_Player_C|GetCollectibleTracking Player)) (Utilities|Text|FormatText "Codex Pages: {X}/{Y}" _output_get (Variables|/Game/GameModes/PlatformingGameMode.PlatformingGameMode_C|GetTotalCodexPages _asplatforming_game_mode)))
          (|CallParentFunction 0)
          (Audio|PlaySoundatLocation (select (Math|Random|RandomBool) "/Game/Sounds/SFX/Pickup/Pop2.Pop2" "/Game/Sounds/SFX/Pickup/Pop.Pop") (Transformation|GetActorLocation) "0, 0, 0" 1.0 1.0 0.0 0 0 0 0))))))

(fn ConstructionScript
  (|CallParentFunction))