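; Teleport pickup actor that launches the player along its facing direction, then opens the Finale level shortly afterwards.
; On player overlap, it replaces any existing BPC_TeleportPickup component with a new one given flight settings, disables player damage and plays a sound.
; It then hides itself and stops its audio; a short timer re-enables the pickup and triggers the level change.
; The construction script applies the configurable mesh.
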(event OnComponentBeginOverlap(Sphere)
  (params (OverlappedComponent :type Primitive%20Component%20Object%20Reference) (OtherActor :type Actor%20Object%20Reference) (OtherComp :type Primitive%20Component%20Object%20Reference) (OtherBodyIndex :type Integer) (bFromSweep :type Boolean) (SweepResult :type Hit%20Result%20Structure%20%28by%20ref%29))
  (bind _returnvalue (Actor|GetComponentbyClass OtherActor "/Game/Blueprints/Player/Components/BPC_TeleportPickup.BPC_TeleportPickup_C"))
  (bind _as_bp_player (Variables|Default|GetAs%20BP%20Player))
  (if (== OtherActor _as_bp_player)
    (Utilities|FlowControl|DoOnce false
      (:Completed
        (if (Utilities|IsValid _returnvalue)
          (Utilities|IsValid _returnvalue
            (:Is%20Valid
              (Default|DestroyThis _returnvalue))))
        (Variables|/Script/Engine.Actor|SetbCanBeDamaged _as_bp_player false)
        (Game|AddComponentbyClass OtherActor "/Game/Blueprints/Player/Components/BPC_TeleportPickup.BPC_TeleportPickup_C" (Variables|Default|GetFlying%20Time) 2.5e+03 (Transformation|GetActorRotation) (Variables|Default|GetSetFlyingTime))
        (Audio|PlaySound2D "/Game/Sounds/SFX/Pickup/yarn02.yarn02" 0.8 1.0 0.0 0 0)
        (CallFunction|Deactivate)
        (bind _returnvalue_2 (Utilities|Time|SetTimerbyEvent (delegate EventReplaceReset) 1.5))
        (Variables|Default|SetCooldownTimer _returnvalue_2)))))

(event Custom|Deactivate
  (Rendering|SetActorHiddenInGame true)
  (Collision|SetCollisionEnabled (Variables|Default|GetSphere) "NoCollision")
  (Audio|Components|Audio|Stop (Variables|Default|GetAudio)))

(event EventBeginPlay
  (bind _asbp_player (Utilities|Casting|CastToBP_Player (Game|Player|GetPlayerPawn 0)))
  (Variables|Default|SetAs%20BP%20Player _asbp_player)
  (Audio|Components|Audio|Play (Variables|Default|GetAudio) 0.0))

(event Collision|EventActorBeginOverlap
  (params (OtherActor :type Actor%20Object%20Reference)))

(event EventTick
  (params (DeltaSeconds :type Float%20%28single-precision%29)))

(event EventReplaceReset
  (Utilities|FlowControl|Sequence
    (:then_0
      (Rendering|SetActorHiddenInGame false)
      (Collision|SetCollisionEnabled (Variables|Default|GetSphere) "QueryAndPhysics")
      (Audio|Components|Audio|Play (Variables|Default|GetAudio) 0.0)
      (Utilities|Time|ClearandInvalidateTimerbyHandle (Variables|Default|GetCooldownTimer))
      (Utilities|FlowControl|DoOnce false) ; enters at Reset
    )
    (:then_1
      (Game|OpenLevel(byObjectReference) "/Game/Maps/Finale.Finale"))))

(fn ConstructionScript
  (Components|StaticMesh|SetStaticMesh (Variables|Default|GetStaticMesh) (Variables|Default|GetMesh)))