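; WallJumpAppear is a level action block, apparently for wall jumping, whose two cube walls become solid temporarily when triggered.
; Both cubes start with collision disabled, and any overlap with the Box enables it for a configurable duration before disabling it again.
; Only collision is toggled, not visibility.
; BeginPlay also makes the player character emit a short-range noise.
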(event OnComponentBeginOverlap(Box)
  (params (OverlappedComponent :type Primitive%20Component%20Object%20Reference) (OtherActor :type Actor%20Object%20Reference) (OtherComp :type Primitive%20Component%20Object%20Reference) (OtherBodyIndex :type Integer) (bFromSweep :type Boolean) (SweepResult :type Hit%20Result%20Structure%20%28by%20ref%29))
  (Collision|SetCollisionEnabled (Variables|Default|GetCube) "QueryAndPhysics")
  (Collision|SetCollisionEnabled (Variables|Default|GetCube1) "QueryAndPhysics")
  (Utilities|FlowControl|Delay (Variables|Default|GetWallAppearDurration))
  (Collision|SetCollisionEnabled (Variables|Default|GetCube) "NoCollision")
  (Collision|SetCollisionEnabled (Variables|Default|GetCube1) "NoCollision"))

(event EventBeginPlay
  (Collision|SetCollisionEnabled (Variables|Default|GetCube) "NoCollision")
  (Collision|SetCollisionEnabled (Variables|Default|GetCube1) "NoCollision")
  (Class|Actor|MakeNoise (Game|GetPlayerCharacter 0) 1.0 0 "0, 0, 0" 1e+01 "None"))

(fn ConstructionScript)